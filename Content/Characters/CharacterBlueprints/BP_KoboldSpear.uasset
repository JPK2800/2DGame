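; BP_KoboldSpear is a child character Blueprint for a spear-wielding kobold that supplies its own action and billboard data.
; Its LoadActionData override assigns kobold spear basic attack and dodge data to BPC CharacterActionData, and idle and walk data to BPC BillboardDataControl.
; It then calls the parent LoadActionData.
; The event graph holds only disabled stubs, and the construction script just calls its parent.
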(fn `LoadActionData`
  (bind _bpc_characteractiondata (`self.BPC_CharacterActionData`))
  (bind _bpc_billboarddatacontrol (`self.BPC_BillboardDataControl`))
  (bind _data (`/Game/ActionData/BPFL_ActionDataLoad.Kobold_Spear_BasicAttack`))
  (set `/Game/ActionData/BPC_CharacterActionData.BasicAttackData` _data _bpc_characteractiondata)
  (bind _data_2 (`/Game/ActionData/BPFL_ActionDataLoad.Kobold_Spear_Dodge`))
  (set `/Game/ActionData/BPC_CharacterActionData.DodgeActionData` _data_2 _bpc_characteractiondata)
  (bind _data_3 (`/Game/ActionData/BPFL_ActionDataLoad.Kobold_Spear_Idle`))
  (set `/Game/CharacterComponents/Billboard_Limbs/BPC_BillboardDataControl.IdleData` _data_3 _bpc_billboarddatacontrol)
  (bind _data_4 (`/Game/ActionData/BPFL_ActionDataLoad.Kobold_Spear_Walk`))
  (set `/Game/CharacterComponents/Billboard_Limbs/BPC_BillboardDataControl.WalkData` _data_4 _bpc_billboarddatacontrol)
  (`parent.LoadActionData`))

(fn `UserConstructionScript`
  (`parent.UserConstructionScript`))