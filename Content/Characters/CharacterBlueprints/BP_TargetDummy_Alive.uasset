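; BP_TargetDummy_Alive is a character Blueprint for the "alive" target dummy, supplying its spin attack and idle data.
; On BeginPlay it assigns the spin attack to the character action data component's basic attack and the idle data to the billboard data control component.
; It then calls the parent BeginPlay, so both are set before inherited startup logic runs.
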(event `self.ReceiveBeginPlay`
  (bind _data (`/Game/ActionData/BPFL_ActionDataLoad.TargetDummy_Alive_SpinAttack`))
  (set `/Game/ActionData/BPC_CharacterActionData.BasicAttackData` _data (`self.BPC_CharacterActionData`))
  (bind _data_2 (`/Game/ActionData/BPFL_ActionDataLoad.TargetDummy_Alive_Idle`))
  (set `/Game/CharacterComponents/Billboard_Limbs/BPC_BillboardDataControl.IdleData` _data_2 (`self.BPC_BillboardDataControl`))
  (`parent.ReceiveBeginPlay`))

(fn `UserConstructionScript`
  (`parent.UserConstructionScript`))