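; BP_Wolf is a wolf character Blueprint that supplies wolf-specific animation and attack data.
; LoadActionData assigns wolf idle and run data to the billboard data component's idle and walk slots, and wolf bite data to the action data component's basic attack.
; The event graph holds only disabled default events, and the construction script just calls its parent.
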(fn `LoadActionData`
  (bind _bpc_billboarddatacontrol (`self.BPC_BillboardDataControl`))
  (bind _data (`/Game/ActionData/BPFL_ActionDataLoad.Wolf_Idle`))
  (set `/Game/CharacterComponents/Billboard_Limbs/BPC_BillboardDataControl.IdleData` _data _bpc_billboarddatacontrol)
  (bind _data_2 (`/Game/ActionData/BPFL_ActionDataLoad.Wolf_Run`))
  (set `/Game/CharacterComponents/Billboard_Limbs/BPC_BillboardDataControl.WalkData` _data_2 _bpc_billboarddatacontrol)
  (bind _data_3 (`/Game/ActionData/BPFL_ActionDataLoad.Wolf_Bite`))
  (set `/Game/ActionData/BPC_CharacterActionData.BasicAttackData` _data_3 (`self.BPC_CharacterActionData`)))

(fn `UserConstructionScript`
  (`parent.UserConstructionScript`))