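; BP_Chest is a chest actor that bursts out coins when it is defeated.
; The defeating-hit event from its BPC_StatTracking component starts a short one-shot delay timer.
; A looping timer runs SpawnCoin, spawning BP_Coin at the chest's location with randomized pitch and yaw, and clears itself once the CoinsToSpawn count is reached.
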(event `self.BPC_StatTracking.OnDefeatingHit`
  (`self.DefeatedChestStartCoinSpawnTImer`))

(fn `CoinSpawnStart`
  (bind _returnvalue (`KismetSystemLibrary.K2_SetTimer` null "SpawnCoin" 0.0625 true))
  (set `self.Timer` _returnvalue))

(fn `DefeatedChestStartCoinSpawnTImer`
  (`KismetSystemLibrary.K2_SetTimerDelegate` (`|CreateDelegate` :!event `CoinSpawnStart`) 0.375))

(fn `SpawnCoin`
  (bind (_returnvalue_roll _returnvalue_pitch _returnvalue_yaw) (`KismetMathLibrary.BreakRotator` (`self.K2_GetActorRotation`)))
  (`|SpawnActorFromClass` "/Game/Objects/BP_Coin.BP_Coin_C" (`KismetMathLibrary.MakeTransform` (`self.K2_GetActorLocation`) (`KismetMathLibrary.MakeRotator` _returnvalue_roll (+ _returnvalue_pitch (`KismetMathLibrary.RandomFloatInRange` -5.0 5.0)) (+ _returnvalue_yaw (`KismetMathLibrary.RandomFloatInRange` -50.0 50.0)))) "Undefined" "MultiplyWithRoot" self self)
  (`/Engine/EditorBlueprintResources/StandardMacros.IncrementInt` (`self.CoinsSpawned`)
    (:`  `
      (if (>= (`self.CoinsSpawned`) (`self.CoinsToSpawn`))
        (`KismetSystemLibrary.K2_ClearAndInvalidateTimerHandle` (`self.Timer`))))))

(fn `UserConstructionScript`
  (`parent.UserConstructionScript`))