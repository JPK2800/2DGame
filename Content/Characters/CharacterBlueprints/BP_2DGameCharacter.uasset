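; Base game character that manages a networked action state, movement control and enemy detection.
; The owning client applies state changes locally, then relays them via server and multicast to non-locally-controlled copies.
; Tick raises start/stop movement events from velocity and drives optional forced forward movement.
; It spawns an attached detection decal that reports enemies, flags defeat, and can hide and attach itself to an incapacitation target.
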(event `self.ReceiveBeginPlay`
  (set `CharacterMovementComponent.MaxWalkSpeed` (`self.DefaultSpeed`) (`self.CharacterMovement`))
  (`self.SpawnDetectionComponent`))

(event `self.ReceiveTick`
  (params (DeltaSeconds :type "Float (single-precision)"))
  (`self.Track Movement Events Step` DeltaSeconds)
  (`self.ForceMovementForwardStep` DeltaSeconds))

(event `ServerUpdateState`
  (params (State :type Name) (Clear :type Boolean))
  (`self.MulticastUpdateState` State Clear))

(event `MulticastUpdateState`
  (params (State :type Name) (Clear :type Boolean))
  (if (not (`self.IsLocallyControlled`))
    (`self.Trigger Update State` State Clear)))

(event `self.BPC_StatTracking.OnDefeatingHit`
  (set `self.IsDefeated` true))

(fn `EnemyDetected`
  (params (Enemy :type "/Game/Characters/CharacterBlueprints/BP_2DGameCharacter Object Reference"))
  (`self.LocalEnemyDetected` Enemy))

(fn `ForceMovementForwardStep`
  (params (DeltaTime :type "Float (double-precision)"))
  (if (`self.ForceMovementForward`)
    (`self.AddMovementInput` (`KismetMathLibrary.GetForwardVector` (`self.ForceMovementRotation`)))))

(fn `HideActorWhenIncapacitating`
  (params (HideAndAttach :type Boolean) (IncapTarget :type "/Game/Characters/CharacterBlueprints/BP_2DGameCharacter Object Reference"))
  (bind _mesh (`self.Mesh`))
  (bind _capsulecomponent (`self.CapsuleComponent`))
  (bind _incaptarget (`self.IncapTarget`))
  (bind _output_get (set `self.IncapTarget` IncapTarget))
  (`/Engine/EditorBlueprintResources/StandardMacros.IsValid` _output_get
    (:`Is Valid`
      (if HideAndAttach
        (`SceneComponent.SetVisibility` _mesh false true)
        (`PrimitiveComponent.SetCollisionEnabled` _capsulecomponent "NoCollision")
        (`self.K2_AttachToActor` _incaptarget "None" "SnapToTarget" "SnapToTarget" "KeepWorld")
        (`KismetSystemLibrary.PrintString` "Incap")
        (else
          (`SceneComponent.SetVisibility` _mesh true true)
          (`PrimitiveComponent.SetCollisionEnabled` _capsulecomponent "QueryAndPhysics")
          (`self.K2_DetachFromActor` _incaptarget "KeepRelative" "KeepRelative" "KeepWorld")
          (`KismetSystemLibrary.PrintString` "End Incap"))))))

(fn `In No Action State`
  (returns (Valid :type Boolean))
  (return (== (`self.CharacterState`) "None")))

(fn `Owner Update State`
  (params (State :type Name) (Clear :type Boolean))
  (if (`self.IsLocallyControlled`)
    (`self.ServerUpdateState` State Clear)
    (`self.Trigger Update State` State Clear)))

(fn `SetForceForwardState`
  (params (Enable :type Boolean) (InputRotationWorld :type "Rotator Structure"))
  (bind _charactermovement (`self.CharacterMovement`))
  (bind _output_get (set `self.ForceMovementForward` Enable))
  (if _output_get
    (`self.K2_SetActorRotation` InputRotationWorld)
    (bind _output_get_2 (set `self.ForceMovementRotation` InputRotationWorld))
    (set `MovementComponent.Velocity` (* (`KismetMathLibrary.GetForwardVector` _output_get_2) (`CharacterMovementComponent.MaxWalkSpeed` _charactermovement)) _charactermovement)
    (else
      (set `CharacterMovementComponent.bUseControllerDesiredRotation` true (`self.CharacterMovement`)))))

(fn `SignalAllowMovement`
  (params (AllowMovement :type Boolean))
  (`self.InMovementControl` AllowMovement))

(fn `SpawnDetectionComponent`
  (bind _returnvalue (`self.K2_GetActorRotation` self))
  (bind _returnvalue_2 (`|SpawnActorFromClass` "/Game/EnemyController/DetectionOverlapObject/BP_DetectionDecal.BP_DetectionDecal_C" (`KismetMathLibrary.MakeTransform` (+ (`self.K2_GetActorLocation` self) (* (`KismetMathLibrary.GetForwardVector` _returnvalue) 550.0)) _returnvalue (-1.0 -1.0 -1.0)) "Undefined" "MultiplyWithRoot" null false false self self))
  (`self.K2_AttachToActor` _returnvalue_2 self "None" "KeepWorld" "KeepWorld" "KeepWorld" true)
  (add `/Game/EnemyController/DetectionOverlapObject/BP_DetectionDecal.EnemyDetected` _returnvalue_2 (`|CreateDelegate` :!event `EnemyDetected`)))

(fn `Track Movement Events Step`
  (params (DeltaTime :type "Float (double-precision)"))
  (bind _returnvalue (`KismetMathLibrary.VSize` (`self.GetVelocity`)))
  (if (and (> _returnvalue 10.0) (not (`self.IsMoving`)))
    (set `self.IsMoving` true)
    (`self.StartMovement`)
    (elif (and (<= _returnvalue 10.0) (`self.IsMoving`))
      (set `self.IsMoving` false)
      (`self.StopMovement`))))

(fn `Trigger Update State`
  (params (State :type Name) (Clear :type Boolean))
  (if Clear
    (bind _output_get (set `self.CharacterState` "None"))
    (`self.UpdateState` _output_get)
    (else
      (bind _output_get_2 (set `self.CharacterState` State))
      (`self.UpdateState` _output_get_2))))

(fn `UpdateMovementSpeed`
  (params (Speed :type "Float (double-precision)") (Reset :type Boolean))
  (if Reset
    (set `CharacterMovementComponent.MaxWalkSpeed` (`self.DefaultSpeed`) (`self.CharacterMovement`))
    (else
      (set `CharacterMovementComponent.MaxWalkSpeed` Speed (`self.CharacterMovement`)))))

(fn `UserConstructionScript`)