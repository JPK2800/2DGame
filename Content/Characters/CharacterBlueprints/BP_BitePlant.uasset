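; BP_BitePlant is the Bite Plant character Blueprint, which equips the character with its bite and spit attacks.
; On BeginPlay it runs the parent logic, then assigns a bite as the basic attack and a spit as the special attack on its character action data component.
; Tick, overlap and construction add no logic of their own.
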(event `self.ReceiveBeginPlay`
  (bind _bpc_characteractiondata (`self.BPC_CharacterActionData`))
  (`parent.ReceiveBeginPlay`)
  (bind _action (`/Game/ActionData/BPFL_ActionDataLoad.BitePlant_Bite`))
  (set `/Game/ActionData/BPC_CharacterActionData.BasicAttackData` _action _bpc_characteractiondata)
  (bind _action_2 (`/Game/ActionData/BPFL_ActionDataLoad.BitePlant_Spit`))
  (set `/Game/ActionData/BPC_CharacterActionData.SpecialAttackData` _action_2 _bpc_characteractiondata))

(fn `UserConstructionScript`
  (`parent.UserConstructionScript`))