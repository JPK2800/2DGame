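; Sequence controller actor that steps through an array of gameplay events on the authority, starting at BeginPlay unless manual triggering is required.
; Each step spawns dialogue and scripted-event actors, then adds a BP_StratGameMode objective or starts a fallback duration timer.
; Optional completion bindings on dialogue, script and objectives allow early endings; force-ending drops actor references, clears the objective and advances.
; The actor destroys itself when the sequence runs out.
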(event `self.ReceiveBeginPlay`
  (bind _asbp_strat_game_mode (cast `/Game/SequenceControl/Objectives/BP_StratGameMode` (`GameplayStatics.GetGameMode`)))
  (set `self.GameMode` _asbp_strat_game_mode)
  (if (not (`self.RequireManualTrigger`))
    (`self.BeginNextSequenceEvent`)))

(fn `BeginNextSequenceEvent`
  (bind _eventsequence (`self.EventSequence`))
  (bind _currenteventindex (`self.CurrentEventIndex`))
  (if (`KismetArrayLibrary.Array_IsValidIndex` _eventsequence _currenteventindex)
    (`|ExecutionSequence`
      (:`then_0`
        (`self.BeginSequenceNodeIfAuthority` (`|GetArrayItem` _eventsequence _currenteventindex)))
      (:`then_1`
        (`/Engine/EditorBlueprintResources/StandardMacros.IncrementInt` (`self.CurrentEventIndex`))))
    (else
      (`self.K2_DestroyActor`))))

(fn `BeginSequenceNodeIfAuthority`
  (params (SequenceEvent :type "/Game/SequenceControl/Struct_SequenceEvent Structure"))
  (bind (_durationifnoobjective _dialogue _scriptedevent _objective _hasobjective _forceendondialogueend _forceendonobjectivecomplete _forceendonscriptcomplete) (break `/Game/SequenceControl/Struct_SequenceEvent` SequenceEvent))
  (bind _returnvalue (`GameplayStatics.GetPlayerController` 0))
  (bind _gamemode (`self.GameMode`))
  (if (`self.HasAuthority`)
    (`/Engine/EditorBlueprintResources/StandardMacros.IsValid` _gamemode
      (:`Is Valid`
        (`|ExecutionSequence`
          (:`then_0`
            (bind _returnvalue_2 (`|SpawnActorFromClass` _dialogue (`KismetMathLibrary.MakeTransform` (0.0 0.0 0.0)) "Undefined" "MultiplyWithRoot" _returnvalue null))
            (`/Engine/EditorBlueprintResources/StandardMacros.IsValid` _returnvalue_2
              (:`Is Valid`
                (bind _output_get (set `self.DialogueActor` _returnvalue_2))
                (if _forceendondialogueend
                  (add `/Game/SequenceControl/Dialogue/BP_DialogueActor.OnDialogueComplete` _output_get (`|CreateDelegate` :!event `ForceEndSequenceNodeIfAuthority`))))))
          (:`then_1`
            (bind _returnvalue_3 (`|SpawnActorFromClass` _scriptedevent (`KismetMathLibrary.MakeTransform` (0.0 0.0 0.0)) "Undefined" "MultiplyWithRoot" _returnvalue null))
            (`/Engine/EditorBlueprintResources/StandardMacros.IsValid` _returnvalue_3
              (:`Is Valid`
                (bind _output_get_2 (set `self.ScriptEventActor` _returnvalue_3))
                (if _forceendonscriptcomplete
                  (add `/Game/SequenceControl/ScriptedEvent/BP_ScriptedEvent.OnEventEnd` _output_get_2 (`|CreateDelegate` :!event `ForceEndSequenceNodeIfAuthority`))))))
          (:`then_2`
            (if _hasobjective
              (`/Game/SequenceControl/Objectives/BP_StratGameMode.ServerAddNewObjective` _gamemode _objective)
              (if _forceendonobjectivecomplete
                (add `/Game/SequenceControl/Objectives/BP_StratGameMode.OnObjectivesComplete` _gamemode (`|CreateDelegate` :!event `ForceEndSequenceNodeIfAuthority`)))
              (else
                (`KismetSystemLibrary.K2_SetTimer` null "EndSequenceNodeIfAuthority" _durationifnoobjective)))))))))

(fn `EndSequenceNodeIfAuthority`
  (if (`self.HasAuthority`)
    (`self.BeginNextSequenceEvent`)))

(fn `ForceEndSequenceNodeIfAuthority`
  (bind _gamemode (`self.GameMode`))
  (if (`self.HasAuthority`)
    (`|ExecutionSequence`
      (:`then_0`
        (`/Engine/EditorBlueprintResources/StandardMacros.IsValid` (`self.DialogueActor`)
          (:`Is Valid`
            (set `self.DialogueActor` null))))
      (:`then_1`
        (`/Engine/EditorBlueprintResources/StandardMacros.IsValid` (`self.ScriptEventActor`)
          (:`Is Valid`
            (set `self.ScriptEventActor` null))))
      (:`then_2`
        (`/Engine/EditorBlueprintResources/StandardMacros.IsValid` _gamemode
          (:`Is Valid`
            (`/Game/SequenceControl/Objectives/BP_StratGameMode.ClearObjective` _gamemode))))
      (:`then_3`
        (`self.EndSequenceNodeIfAuthority`)))))

(fn `UserConstructionScript`)