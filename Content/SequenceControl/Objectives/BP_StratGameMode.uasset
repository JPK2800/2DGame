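; Game mode that tracks a replicated objective with up to three trigger-driven counters and shows it in WBP_ObjectiveUI.
; Server events set objectives, spawn scripted event actors and multicast completion; OnRep refreshes the widget.
; ReceiveObjectiveUpdate increments matching counters, although the third writes to Progress2, and reassigns the struct.
; When every goal is met or -1, it removes the widget and calls OnObjectivesComplete.
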(event `ServerAddNewObjective`
  (params (NewObjective :type "/Game/SequenceControl/Objectives/Struct_Objective Structure"))
  (set `self.Objectives` NewObjective)
  (`self.UpdateObjectiveList`))

(event `ServerObjectivesComplete`
  (`self.MulticastObjectivesComplete`)
  (`self.ObjectiveComplete`))

(event `MulticastObjectivesComplete`
  (`self.ObjectiveComplete`))

(event `ServerSpawnScriptedEvent`
  (params (ScriptedEvent :type "/Game/SequenceControl/ScriptedEvent/BP_ScriptedEvent Class Reference"))
  (`|SpawnActorFromClass` ScriptedEvent (`KismetMathLibrary.MakeTransform` (0.0 0.0 0.0)) "Undefined" "MultiplyWithRoot" (`GameplayStatics.GetPlayerController` 0) null))

(fn `ClearObjective`
  (bind _objectiveui (`self.ObjectiveUI`))
  (`/Engine/EditorBlueprintResources/StandardMacros.IsValid` _objectiveui
    (:`Is Valid`
      (`Widget.RemoveFromParent` _objectiveui)
      (set `self.ObjectiveUI` null))))

(fn `IsObjectiveComplete`
  (returns (IsComplete :type Boolean))
  (bind (_objectives_objectivedisplaytext _objectives_progress1 _objectives_goal1 _objectives_trigger1 _objectives_progress2 _objectives_goal2 _objectives_trigger2 _objectives_progress3 _objectives_goal3) (break `/Game/SequenceControl/Objectives/Struct_Objective` (`self.Objectives`)))
  (return (and (or (>= _objectives_progress1 _objectives_goal1) (== _objectives_goal1 -1)) (or (>= _objectives_progress2 _objectives_goal2) (== _objectives_goal2 -1)) (or (>= _objectives_progress3 _objectives_goal3) (== _objectives_goal3 -1)))))

(fn `ObjectiveComplete`
  (`self.ClearObjective`)
  (`self.OnObjectivesComplete`))

(fn `OnRep_Objectives`
  (`self.UpdateObjectiveList`))

(fn `ReceiveObjectiveUpdate`
  (params (Trigger :type Byte))
  (locals (ValueUpdated :type Boolean))
  (bind (_objectives_objectivedisplaytext _objectives_progress1 _objectives_goal1 _objectives_trigger1 _objectives_progress2 _objectives_goal2 _objectives_trigger2 _objectives_progress3 _objectives_goal3 _objectives_trigger3) (break `/Game/SequenceControl/Objectives/Struct_Objective` (`self.Objectives`)))
  (bind _objectives (`self.Objectives`))
  (`|ExecutionSequence`
    (:`then_0`
      (if (== _objectives_trigger1 Trigger)
        (if (< _objectives_progress1 _objectives_goal1)
          (setmembers `/Game/SequenceControl/Objectives/Struct_Objective` :`StructRef` _objectives :`Progress1` (+ _objectives_progress1 1))
          (set `local.ValueUpdated` true :!label _label))))
    (:`then_1`
      (if (== _objectives_trigger2 Trigger)
        (if (< _objectives_progress2 _objectives_goal2)
          (setmembers `/Game/SequenceControl/Objectives/Struct_Objective` :`StructRef` _objectives :`Progress2` (+ _objectives_progress2 1))
          (goto _label))))
    (:`then_2`
      (if (== _objectives_trigger3 Trigger)
        (if (< _objectives_progress3 _objectives_goal3)
          (setmembers `/Game/SequenceControl/Objectives/Struct_Objective` :`StructRef` _objectives :`Progress2` (+ _objectives_progress3 1))
          (goto _label))))
    (:`then_3`
      (if (`local.ValueUpdated`)
        (set `self.Objectives` (`self.Objectives`))))
    (:`then_4`
      (if (`local.ValueUpdated`)
        (bind _iscomplete (`self.IsObjectiveComplete`))
        (if _iscomplete
          (`self.ObjectiveComplete`))))))

(fn `UpdateObjectiveList`
  (`|ExecutionSequence`
    (:`then_0`
      (`/Engine/EditorBlueprintResources/StandardMacros.IsValid` (`self.ObjectiveUI`)
        (:`Is Not Valid`
          (bind _returnvalue (`|CreateWidget` "/Game/SequenceControl/Objectives/WBP_ObjectiveUI.WBP_ObjectiveUI_C" (`GameplayStatics.GetPlayerController` 0)))
          (set `self.ObjectiveUI` _returnvalue)
          (`UserWidget.AddToPlayerScreen` _returnvalue 0))))
    (:`then_1`
      (`/Engine/EditorBlueprintResources/StandardMacros.IsValid` (`self.ObjectiveUI`)
        (:`Is Valid`
          (`/Game/SequenceControl/Objectives/WBP_ObjectiveUI.UpdateData` (`self.ObjectiveUI`) (`self.Objectives`)))))))

(fn `UserConstructionScript`)