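; Dialogue actor for the green wizard kobold tutorial, showing the "Evil Wizard Kobold" coaching the player to get close to a dummy and dodge just before it hits.
; BeginPlay runs the parent's logic, then calls StartScript to begin the conversation.
; InitDialogue fills DialogueScript with three entries, each holding two portrait frames, speaker names, colors and text lines.
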(event `self.ReceiveBeginPlay`
  (`parent.ReceiveBeginPlay`)
  (`self.StartScript`))

(fn `InitDialogue`
  (bind _array (`|MakeArray` "/Game/SequenceControl/Dialogue/DialogueIcons/GreenTutKobold/green_kob_dialogue0000.green_kob_dialogue0000" "/Game/SequenceControl/Dialogue/DialogueIcons/GreenTutKobold/green_kob_dialogue0001.green_kob_dialogue0001" :!type "Texture2D Object Reference"))
  (bind _dialoguescript (`self.DialogueScript`))
  (`KismetArrayLibrary.Array_Add` _dialoguescript (make `/Game/SequenceControl/Dialogue/Struct_DialogueData` _array "Kobold" "Evil Wizard Kobold" (struct :`R` 1.0 :`G` 1.0 :`B` 1.0 :`A` 1.0) (struct :`R` 0.623961 :`B` 0.412543 :`A` 1.0) "I think it worked?"))
  (`KismetArrayLibrary.Array_Add` _dialoguescript (make `/Game/SequenceControl/Dialogue/Struct_DialogueData` _array "Kobold" "Evil Wizard Kobold" (struct :`R` 1.0 :`G` 1.0 :`B` 1.0 :`A` 1.0) (struct :`R` 0.623961 :`B` 0.412543 :`A` 1.0) "The dummy cant move so" "try to get real close to it!"))
  (`KismetArrayLibrary.Array_Add` _dialoguescript (make `/Game/SequenceControl/Dialogue/Struct_DialogueData` _array "Kobold" "Evil Wizard Kobold" (struct :`R` 1.0 :`G` 1.0 :`B` 1.0 :`A` 1.0) (struct :`R` 0.623961 :`B` 0.412543 :`A` 1.0) "Then dodge right before" "it hits you.")))

(fn `UserConstructionScript`
  (`parent.UserConstructionScript`))