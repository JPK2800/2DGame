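; Dialogue actor for the Lich Lair in which the Dragon warns of a skeleton enemy and advises dodging, then counterattacking.
; InitDialogue adds that single entry to DialogueScript, with speaker name, colors and three lines of text.
; BeginPlay calls the parent, then StartScript, so the dialogue starts as soon as the actor begins play.
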(event `self.ReceiveBeginPlay`
  (`parent.ReceiveBeginPlay`)
  (`self.StartScript`))

(fn `InitDialogue`
  (`KismetArrayLibrary.Array_Add` (`self.DialogueScript`) (make `/Game/SequenceControl/Dialogue/Struct_DialogueData` _ "Dragon" "Dragon" (struct :`R` 1.0 :`G` 1.0 :`B` 1.0 :`A` 1.0) (struct :`R` 1.0 :`B` 0.096302 :`A` 1.0) "An enemy! That is a skeleton!" "Dodge its attacks and" "and try to counterattack!")))

(fn `UserConstructionScript`
  (`parent.UserConstructionScript`))