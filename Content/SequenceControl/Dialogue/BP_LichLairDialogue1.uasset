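; BP_LichLairDialogue1 is a dialogue sequence for the Lich Lair in which a Dragon welcomes the player to their first dungeon as a tutorial guide.
; InitDialogue fills the inherited DialogueScript array with the Dragon's lines, each carrying speaker, color and text-row data.
; BeginPlay runs the parent logic, then calls StartScript, so the dialogue starts as soon as the actor begins play.
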(event `self.ReceiveBeginPlay`
  (`parent.ReceiveBeginPlay`)
  (`self.StartScript`))

(fn `InitDialogue`
  (bind _dialoguescript (`self.DialogueScript`))
  (`KismetArrayLibrary.Array_Add` _dialoguescript (make `/Game/SequenceControl/Dialogue/Struct_DialogueData` _ "Dragon" "Dragon" (struct :`R` 1.0 :`G` 1.0 :`B` 1.0 :`A` 1.0) (struct :`R` 1.0 :`B` 0.096302 :`A` 1.0) "Hi, Little One! Welcome to your " "first dungeon!"))
  (`KismetArrayLibrary.Array_Add` _dialoguescript (make `/Game/SequenceControl/Dialogue/Struct_DialogueData` _ "Dragon" "Dragon" (struct :`R` 1.0 :`G` 1.0 :`B` 1.0 :`A` 1.0) (struct :`R` 1.0 :`B` 0.096302 :`A` 1.0) "I am here to help you learn" "the basics to dungeoneering!"))
  (`KismetArrayLibrary.Array_Add` _dialoguescript (make `/Game/SequenceControl/Dialogue/Struct_DialogueData` _ "Dragon" "Dragon" (struct :`R` 1.0 :`G` 1.0 :`B` 1.0 :`A` 1.0) (struct :`R` 1.0 :`B` 0.096302 :`A` 1.0) "Dungeons are full of monsters and" "traps, so you will need to be" "careful!"))
  (`KismetArrayLibrary.Array_Add` _dialoguescript (make `/Game/SequenceControl/Dialogue/Struct_DialogueData` _ "Dragon" "Dragon" (struct :`R` 1.0 :`G` 1.0 :`B` 1.0 :`A` 1.0) (struct :`R` 1.0 :`B` 0.096302 :`A` 1.0) "Head inside when you are ready!")))

(fn `UserConstructionScript`
  (`parent.UserConstructionScript`))