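; BP_SequenceTriggerBox is a one-shot trigger volume that spawns a configured sequence actor when the locally controlled player character enters it.
; It checks overlaps already present on BeginPlay and also listens for begin-overlap events on its collision component, filtering for a player-controlled, locally controlled BP_2DGameCharacter.
; SpawnSequence runs only with authority, spawning SequenceClass at the box's transform, setting PlayedAlready and destroying the trigger.
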(event `self.ReceiveBeginPlay`
  (`self.InitCheckForOverlap`))

(event `self.CollisionComponent.OnComponentBeginOverlap`
  (params (OverlappedComponent :type "PrimitiveComponent Object Reference") (OtherActor :type "Actor Object Reference") (OtherComp :type "PrimitiveComponent Object Reference") (OtherBodyIndex :type Integer) (bFromSweep :type Boolean) (SweepResult :type "HitResult Structure (by ref)"))
  (bind _asbp_2dgame_character (cast `/Game/Characters/CharacterBlueprints/BP_2DGameCharacter` OtherActor))
  (if (and (`Pawn.IsPlayerControlled` _asbp_2dgame_character) (`Pawn.IsLocallyControlled` _asbp_2dgame_character) (not (`self.PlayedAlready`)))
    (`self.SpawnSequence`)))

(fn `InitCheckForOverlap`
  (for _array_element (`PrimitiveComponent.GetOverlappingActors` (`self.CollisionComponent`) "/Game/Characters/CharacterBlueprints/BP_2DGameCharacter.BP_2DGameCharacter_C")
    (bind _asbp_2dgame_character (cast `/Game/Characters/CharacterBlueprints/BP_2DGameCharacter` _array_element))
    (if (and (`Pawn.IsPlayerControlled` _asbp_2dgame_character) (`Pawn.IsLocallyControlled` _asbp_2dgame_character))
      (`self.SpawnSequence`))))

(fn `SpawnSequence`
  (if (`self.HasAuthority`)
    (`|SpawnActorFromClass` (`self.SequenceClass`) (`self.GetTransform`) "Undefined" "MultiplyWithRoot" self null)
    (set `self.PlayedAlready` true)
    (`self.K2_DestroyActor`)))

(fn `UserConstructionScript`)