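; Tutorial scripted event in which the kobold wizard NPC powers up a passive target dummy, turning it into a hostile one.
; On BeginPlay it triggers the wizard's timed spellcast-channel billboard action and starts a matching timer.
; When the timer fires, it replaces the passive dummy with a living dodge-objective dummy at the same transform, possessed by a new enemy AI.
; It then ends the scripted event.
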(event `self.ReceiveBeginPlay`
  (`parent.ReceiveBeginPlay`)
  (`|ExecutionSequence`
    (:`then_0`
      (bind _returnvalue (`GameplayStatics.GetActorOfClass` "/Game/Characters/CharacterBlueprints/NPC_Idle/BP_Kobold_Wizard_NPC_Tutorial.BP_Kobold_Wizard_NPC_Tutorial_C"))
      (`/Engine/EditorBlueprintResources/StandardMacros.IsValid` _returnvalue
        (:`Is Valid`
          (bind _bpc_characteractiondata (`/Game/Characters/CharacterBlueprints/BP_2DGameCharacter.BPC_CharacterActionData` _returnvalue))
          (`/Engine/EditorBlueprintResources/StandardMacros.IsValid` _bpc_characteractiondata
            (:`Is Valid`
              (`/Game/ActionData/BPC_CharacterActionData.ServerTriggerSpecialAction` :`self` _bpc_characteractiondata :`Action` (make `/Game/ActionData/Struct_Action1` "PoweringUpDummy" (struct) _ false "Default" null) :`Duration` 5.0 :`Action_BillboardData_0_FrameCount` 2 :`Action_BillboardData_OneSide` true :`Action_BillboardData_SkipDiags` true :`Action_BillboardData_PlayRate` 2.0 :`Action_BillboardData_UseZ` true :`Action_BillboardData_OrientToCam` true :`Action_BillboardData_-135_Frames` "/Game/empty.empty" :`Action_BillboardData_-90_Frames` "/Game/empty.empty" :`Action_BillboardData_-45_Frames` "/Game/empty.empty" :`Action_BillboardData_180_Frames` "/Game/empty.empty" :`Action_BillboardData_135_Frames` "/Game/empty.empty" :`Action_BillboardData_90_Frames` "/Game/empty.empty" :`Action_BillboardData_45_Frames` "/Game/empty.empty" :`Action_BillboardData_0_Frames` "/Game/Characters/CharacterArt/kobold_wizard_tut_npc1/kobold_wizard_spellcastchannel_NPC1.kobold_wizard_spellcastchannel_NPC1"))))))
    (:`then_1`
      (`KismetSystemLibrary.K2_SetTimer` null "SwapDummyWithHostileDummy" 5.0))))

(fn `SwapDummyWithHostileDummy`
  (locals (TF :type "Transform Structure"))
  (`|ExecutionSequence`
    (:`then_0`
      (bind _returnvalue (`GameplayStatics.GetActorOfClass` "/Game/Characters/CharacterBlueprints/BP_TargetDummy_Passive.BP_TargetDummy_Passive_C"))
      (`/Engine/EditorBlueprintResources/StandardMacros.IsValid` _returnvalue
        (:`Is Valid`
          (bind _output_get (set `local.TF` (`self.GetTransform` _returnvalue)))
          (`self.K2_DestroyActor` _returnvalue)
          (bind _returnvalue_2 (`|SpawnActorFromClass` "/Game/EnemyController/BP_GameEnemyAi_LivingDummy.BP_GameEnemyAi_LivingDummy_C" (`KismetMathLibrary.MakeTransform` (0.0 0.0 0.0)) "Undefined" "MultiplyWithRoot" null 50.0 null))
          (bind _returnvalue_3 (`|SpawnActorFromClass` "/Game/Characters/CharacterBlueprints/BP_TargetDummy_Alive_DodgeObjective.BP_TargetDummy_Alive_DodgeObjective_C" _output_get "AlwaysSpawn" "MultiplyWithRoot" _returnvalue_2 null))
          (`Controller.Possess` _returnvalue_2 _returnvalue_3))))
    (:`then_1`
      (`self.EndScriptedEvent`))))

(fn `UserConstructionScript`
  (`parent.UserConstructionScript`))