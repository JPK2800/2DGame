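; BP_Breakable3D is a breakable 3D prop that gives material feedback when hit or overlapped by attack telegraphs, and exposes a server event to destroy itself.
; It creates a dynamic material on its static mesh at BeginPlay.
; Hits from BPC_StatTracking briefly set a HitFlash parameter, cleared by a timer.
; Overlapping telegraphs are tracked in a list, tinting the mesh green while any remain and firing overlap dispatchers.
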(event `self.ReceiveBeginPlay`
  (bind _returnvalue (`PrimitiveComponent.CreateDynamicMaterialInstance` (`self.StaticMesh`) 0 null "None"))
  (bind _output_get (set `self.DynMat` _returnvalue))
  (`PrimitiveComponent.SetMaterial` (`self.StaticMesh`) 0 _output_get))

(event `self.BPC_StatTracking.OnTakeHit`
  (params (Damage :type "Float (double-precision)") (DotTick :type Boolean) (Attacker :type "/Game/Characters/CharacterBlueprints/BP_2DGameCharacter Object Reference"))
  (bind _returnvalue (`KismetSystemLibrary.K2_SetTimerDelegate` (delegate `OnEndHitFlash`) 0.15))
  (set `self.Timer` _returnvalue)
  (`MaterialInstanceDynamic.SetScalarParameterValue` (`self.DynMat`) "HitFlash" 1.0))

(event `OnEndHitFlash`
  (`MaterialInstanceDynamic.SetScalarParameterValue` (`self.DynMat`) "HitFlash" 0.0))

(event `ServerDestroyActor`
  (`self.K2_DestroyActor`))

(fn `Overlapped Telegraph`
  (params (Telegraph :type "/Game/AttackDecals/BP_HitTelegraphActor Object Reference") (StartOverlap :type Boolean))
  (bind _hittelegraph (`self.HitTelegraph`))
  (bind _dynmat (`self.DynMat`))
  (bind _returnvalue (`KismetArrayLibrary.Array_Length` _hittelegraph))
  (if StartOverlap
    (`self.OnTelegraphOverlap` Telegraph)
    (`KismetArrayLibrary.Array_Add` _hittelegraph Telegraph)
    (if (== _returnvalue 1)
      (`MaterialInstanceDynamic.SetScalarParameterValue` _dynmat "UseColorShiftForTelegraph" 1.0)
      (`MaterialInstanceDynamic.SetVectorParameterValue` _dynmat "ColorShiftTelegraph" (struct :`G` 1.0 :`B` 0.234551 :`A` 1.0)))
    (else
      (`self.OnTelegraphOverlapEnd` Telegraph)
      (`KismetArrayLibrary.Array_RemoveItem` _hittelegraph Telegraph)
      (if (== _returnvalue 0)
        (`MaterialInstanceDynamic.SetScalarParameterValue` _dynmat "UseColorShiftForTelegraph" 0.0)))))

(fn `UserConstructionScript`)