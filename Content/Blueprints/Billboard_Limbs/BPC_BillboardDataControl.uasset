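; Character component that switches flipbook data on the owning BP_2DGameCharacter's tagged billboard limbs to match its state.
; Movement and stat-tracking events select idle, walk, stomped, defeated or small-slime incapacitation data.
; Actions override movement visuals until cleared, with defeat using a timer from frame count and play rate to reach its idle.
; Non-DoT hits briefly flash the limb materials, and incapacitation also listens for hits on the attacker.
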(event `self.ReceiveBeginPlay`
  (bind _returnvalue (`self.GetOwner`))
  (bind _asbp_2dgame_character (cast `/Game/Characters/CharacterBlueprints/BP_2DGameCharacter` _returnvalue))
  (add `/Game/Characters/CharacterBlueprints/BP_2DGameCharacter.StartMovement` _asbp_2dgame_character (delegate `BeginSetMoving`))
  (add `/Game/Characters/CharacterBlueprints/BP_2DGameCharacter.StopMovement` _asbp_2dgame_character (delegate `BeginSetIdle`))
  (add `/Game/Characters/CharacterBlueprints/BP_2DGameCharacter.UpdateState` _asbp_2dgame_character (delegate `BeginUpdateState`))
  (bind _bpc_stattracking (`/Game/Characters/CharacterBlueprints/BP_2DGameCharacter.BPC_StatTracking` _asbp_2dgame_character))
  (add `/Game/Blueprints/StatTracking/BPC_StatTracking.OnDefeatingHit` _bpc_stattracking (delegate `OnDefeatingHit`))
  (add `/Game/Blueprints/StatTracking/BPC_StatTracking.OnReceiveIncapacitation` _bpc_stattracking (delegate `OnBeginIncapacitation`))
  (add `/Game/Blueprints/StatTracking/BPC_StatTracking.OnEndIncapacitation` _bpc_stattracking (delegate `OnEndIncapacitation`))
  (add `/Game/Blueprints/StatTracking/BPC_StatTracking.OnTakeHit` _bpc_stattracking (delegate `OnTakeHit`))
  (for _array_element (`Actor.K2_GetComponentsByClass` _returnvalue "/Game/Blueprints/Billboard_Limbs/BPC_BillboardLimb.BPC_BillboardLimb_C")
    (bind _componenttags (`ActorComponent.ComponentTags` _array_element))
    (if (`KismetArrayLibrary.Array_IsNotEmpty` _componenttags)
      (if (`KismetArrayLibrary.Array_Contains` _componenttags (`self.TagName`))
        (`KismetArrayLibrary.Array_Add` (`self.RelevantBillboards`) _array_element))))
  (`self.SetIdle`))

(event `BeginSetMoving`
  (`self.SetMoving`))

(event `OnBeginIncapacitation`
  (params (Type :type Name) (Attacker :type "/Game/Characters/CharacterBlueprints/BP_2DGameCharacter Object Reference") (HideAndAttachAttacker :type Boolean))
  (`self.SetIncap` Attacker Type HideAndAttachAttacker))

(event `OnEndIncapacitation`
  (`self.Clear Incap`))

(event `OnTakeHit`
  (params (Damage :type "Float (double-precision)") (DotTick :type Boolean) (Attacker :type "/Game/Characters/CharacterBlueprints/BP_2DGameCharacter Object Reference"))
  (if (not DotTick)
    (`self.SetHitFlash`)))

(event `BeginSetIdle`
  (`self.SetIdle`))

(event `BeginUpdateState`
  (params (State :type Name))
  (`self.UpdateState` State))

(event `OnDefeatingHit`
  (`self.SetDefeated`))

(fn `Clear Action`
  (if (`self.IsDefeated`)
    (for _array_element (`self.RelevantBillboards`)
      (`/Game/Blueprints/Billboard_Limbs/BPC_BillboardLimb.UpdateData` _array_element (`self.DefeatedIdleData`)))
    (elif (not (`self.IsIncapacitated`))
      (set `self.InActionState` false)
      (`|ExecutionSequence`
        (:`then_0`
          (if (== (`self.CurrentMovementState`) "Idle")
            (`self.SetIdle`)
            (elif (== (`self.CurrentMovementState`) "Moving")
              (`self.SetMoving`))))
        (:`then_1`
          (for _array_element_2 (`self.RelevantBillboards`)
            (`/Game/Blueprints/Billboard_Limbs/BPC_BillboardLimb.ResyncFlipbooks` _array_element_2)))))))

(fn `Clear Incap`
  (bind _incapattacker (`self.IncapAttacker`))
  (if (`self.IsIncapacitated`)
    (`|ExecutionSequence`
      (:`then_0`
        (`/Engine/EditorBlueprintResources/StandardMacros.IsValid` _incapattacker
          (:`Is Valid`
            (clear `/Game/Blueprints/StatTracking/BPC_StatTracking.OnTakeHit` (`/Game/Characters/CharacterBlueprints/BP_2DGameCharacter.BPC_StatTracking` _incapattacker)))))
      (:`then_1`
        (set `self.IncapAttacker` null)
        (set `self.IsIncapacitated` false)
        (`self.Clear Action`)))))

(fn `EndHitFlash`
  (for _array_element (`self.RelevantBillboards`)
    (bind _dynamicmaterial (`/Game/Blueprints/Billboard_Limbs/BPC_BillboardLimb.DynamicMaterial` _array_element))
    (`/Engine/EditorBlueprintResources/StandardMacros.IsValid` _dynamicmaterial
      (:`Is Valid`
        (`MaterialInstanceDynamic.SetScalarParameterValue` _dynamicmaterial "HitFlash" 0.0)))))

(fn `IncapAttackerTakeHit`
  (params (Damage :type "Float (double-precision)") (DotTick :type Boolean) (Attacker :type "/Game/Characters/CharacterBlueprints/BP_2DGameCharacter Object Reference"))
  (if (not DotTick)
    (`self.SetHitFlash`)))

(fn `SetAction`
  (params (Data :type "/Game/Blueprints/Billboard_Limbs/Struct_BillboardData Structure (by ref)"))
  (set `self.InActionState` true)
  (for _array_element (`self.RelevantBillboards`)
    (`/Game/Blueprints/Billboard_Limbs/BPC_BillboardLimb.UpdateData` _array_element Data)
    (`/Game/Blueprints/Billboard_Limbs/BPC_BillboardLimb.StartFlipbookFromStart` _array_element)))

(fn `SetDefeated`
  (bind _defeateddata (`self.DefeatedData`))
  (bind (_0_frames _45_frames _90_frames _135_frames _180_frames __45_frames __90_frames __135_frames _usenegativeframes _flipsideframes _orienttocam _usez _playrate) (break `/Game/Blueprints/Billboard_Limbs/Struct_BillboardData` _defeateddata))
  (`self.SetAction` _defeateddata)
  (set `self.IsDefeated` true)
  (`KismetSystemLibrary.K2_SetTimer` null "Clear Action" (/ (`KismetArrayLibrary.Array_Length` _0_frames) _playrate)))

(fn `SetHitFlash`
  (for _array_element (`self.RelevantBillboards`)
    (bind _dynamicmaterial (`/Game/Blueprints/Billboard_Limbs/BPC_BillboardLimb.DynamicMaterial` _array_element))
    (`/Engine/EditorBlueprintResources/StandardMacros.IsValid` _dynamicmaterial
      (:`Is Valid`
        (`MaterialInstanceDynamic.SetScalarParameterValue` _dynamicmaterial "HitFlash" 1.0))))
  (bind _returnvalue (`KismetSystemLibrary.K2_SetTimer` null "EndHitFlash" 0.15))
  (set `self.HitFlashTimer` _returnvalue))

(fn `SetIdle`
  (set `self.CurrentMovementState` "Idle")
  (if (not (`self.InActionState`))
    (for _array_element (`self.RelevantBillboards`)
      (if (`self.IsStomped`)
        (`/Game/Blueprints/Billboard_Limbs/BPC_BillboardLimb.UpdateData` _array_element (`self.StompedIdleData`))
        (else
          (`/Game/Blueprints/Billboard_Limbs/BPC_BillboardLimb.UpdateData` _array_element (`self.IdleData`)))))))

(fn `SetIncap`
  (params (Attacker :type "/Game/Characters/CharacterBlueprints/BP_2DGameCharacter Object Reference") (IncapType :type Name) (HideAndAttachAttacker :type Boolean))
  (`|ExecutionSequence`
    (:`then_0`
      (bind _output_get (set `self.IncapAttacker` Attacker))
      (bind _bpc_stattracking (`/Game/Characters/CharacterBlueprints/BP_2DGameCharacter.BPC_StatTracking` _output_get))
      (`/Engine/EditorBlueprintResources/StandardMacros.IsValid` _bpc_stattracking
        (:`Is Valid`
          (add `/Game/Blueprints/StatTracking/BPC_StatTracking.OnTakeHit` _bpc_stattracking (`|CreateDelegate` :!event `IncapAttackerTakeHit`))
          (switch `name` IncapType
            (:`SmallSlime`
              (`self.SetSmallSlimeIncap`))))))))

(fn `SetMoving`
  (set `self.CurrentMovementState` "Moving")
  (if (not (`self.InActionState`))
    (for _array_element (`self.RelevantBillboards`)
      (if (`self.IsStomped`)
        (`/Game/Blueprints/Billboard_Limbs/BPC_BillboardLimb.UpdateData` _array_element (`self.StompedWalkData`))
        (else
          (`/Game/Blueprints/Billboard_Limbs/BPC_BillboardLimb.UpdateData` _array_element (`self.WalkData`)))))))

(fn `SetSmallSlimeIncap`
  (`self.SetAction` (`self.SmallSlimeIncap`))
  (set `self.IsIncapacitated` true))

(fn `SetStomped`
  (params (Enable :type Boolean))
  (if (!= (`self.IsStomped`) Enable)
    (set `self.IsStomped` Enable)
    (`self.Clear Action`)))

(fn `UpdateState`
  (params (State :type Name))
  (`|ExecutionSequence`
    (:`then_0`
      (set `self.IsDefeated` false)
      (set `self.IsStomped` false)
      (`self.Clear Action`)
      (switch `name` State
        (:`Stomped`
          (`self.SetStomped` true))
        (:`Defeated`
          (`self.SetDefeated`))))))