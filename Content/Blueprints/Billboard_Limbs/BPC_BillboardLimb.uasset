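; Billboard limb component that renders a camera-facing, directional flipbook sprite, configured from a data struct through UpdateData.
; Each tick it rotates toward the player camera and picks a frame set from the owner's yaw relative to the view, with optional diagonal-skip or single-side modes.
; Sets are pushed to a dynamic material only when angle or flip changes, mirroring side views via XScale.
; The material handles playback, with rate and restart/resync set by parameters.
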(event `self.ReceiveBeginPlay`
  (`self.InitDynamicMat`))

(event `self.ReceiveTick`
  (params (DeltaSeconds :type "Float (single-precision)"))
  (`self.OrientLimbStep` DeltaSeconds)
  (`self.UpdateMaterialAngleStep` DeltaSeconds))

(fn `InitDynamicMat`
  (bind _returnvalue (`self.CreateDynamicMaterialInstance` 0 "/Game/Characters/Mat_FlipbookMaterial.Mat_FlipbookMaterial"))
  (bind _output_get (set `self.DynamicMaterial` _returnvalue))
  (`self.SetMaterial` 0 _output_get))

(fn `OrientLimbStep`
  (params (DeltaTime :type "Float (double-precision)"))
  (bind _returnvalue (`self.GetOwner`))
  (bind _returnvalue_2 (`KismetMathLibrary.FindLookAtRotation` (`PlayerCameraManager.GetCameraLocation` (`self.CameraManager`)) (`Actor.K2_GetActorLocation` _returnvalue)))
  (`/Engine/EditorBlueprintResources/StandardMacros.IsValid` _returnvalue
    (:`Is Valid`
      (if (`self.OrientToCamera`)
        (`/Engine/EditorBlueprintResources/StandardMacros.IsValid` (`self.CameraManager`)
          (:`Is Valid`
            _)
          (:`Is Not Valid`
            (set `self.CameraManager` (`GameplayStatics.GetPlayerCameraManager` 0))))
        (if (`self.OrientUseZAxis`)
          (`self.K2_SetWorldRotation` (`KismetMathLibrary.MakeRotator` (+ (.roll _returnvalue_2) 180.0) (+ (* (.pitch _returnvalue_2) 1.0) -90.0) (.yaw _returnvalue_2)))
          (else
            (`self.K2_SetWorldRotation` (`KismetMathLibrary.MakeRotator` (+ (.roll _returnvalue_2) 90.0) -90.0 (+ (.yaw _returnvalue_2) 90.0)))))))))

(fn `ResyncFlipbooks`
  (`MaterialInstanceDynamic.SetScalarParameterValue` (`self.DynamicMaterial`) "ResetTime" 0.0))

(fn `StartFlipbookFromStart`
  (`MaterialInstanceDynamic.SetScalarParameterValue` (`self.DynamicMaterial`) "ResetTime" (`GameplayStatics.GetRealTimeSeconds`)))

(fn `UpdateData`
  (params (Data :type "/Game/Blueprints/Billboard_Limbs/Struct_BillboardData Structure"))
  (`|ExecutionSequence`
    (:`then_0`
      (set `self.0_Frames` Data_0_Frames_3_028B00B844E292C899EAA3A562E33BC7)
      (set `self.45_Frames` Data_45_Frames_5_D43F149A41B15205A3BD69BFAC2626BD)
      (set `self.90_Frames` Data_90_Frames_7_2C10A25D46B000AF50AF9380333B5691)
      (set `self.135_Frames` Data_135_Frames_9_EAE025994E0F982539F0B0B0258B70D2)
      (set `self.180_Frames` Data_180_Frames_11_4361621A4E3E796D0B313991F5BE7024)
      (set `self.-45_Frames` `Data_-45_Frames_13_47607E2C4583212D3429C5BEBF9CFF3E`)
      (set `self.-90_Frames` `Data_-90_Frames_15_13FD55394E6D04DD40DFF4A9236FF428`)
      (set `self.-135_Frames` `Data_-135_Frames_17_A081635E41B6D7F80F483CA85319E615`)
      (set `self.FlipSideSprites` Data_FlipSideFrames_23_46BEC0E6407D43F253E0D89891E0A2C7)
      (set `self.OrientToCamera` Data_OrientToCam_26_E6EC66584897E752B1333CB8CEA23B08)
      (set `self.OrientUseZAxis` Data_UseZ_28_B9A6E912426A7685F0A97BA2E089B545)
      (bind _output_get (set `self.PlayRate` Data_PlayRate_31_5653BD6F41767AC25D56449EE85EFC95))
      (set `self.SkipDiagnonals` Data_SkipDiags_35_E3CFCE73445F8EC35DC49DA96E907E5E)
      (set `self.OnlyOneSide` Data_OneSide_37_DFB7FADD4B2856697C8D78A3DF659838)
      (`MaterialInstanceDynamic.SetScalarParameterValue` (`self.DynamicMaterial`) "Rate" _output_get))
    (:`then_1`
      (set `self.CurrentAngle` -1)
      (`self.UpdateMaterialAngleStep` (`GameplayStatics.GetWorldDeltaSeconds`)))))

(fn `UpdateMatByAngle`
  (params (NewAngle :type Integer) (Textures :type "Array of Texture2D Object Reference") (XFlip :type Boolean))
  (bind _returnvalue (`KismetArrayLibrary.Array_Length` Textures))
  (bind _dynamicmaterial (`self.DynamicMaterial`))
  (bind _dynamicmaterial_2 (`self.DynamicMaterial`))
  (`|ExecutionSequence`
    (:`then_0`
      (`MaterialInstanceDynamic.SetScalarParameterValue` _dynamicmaterial "TexCount" (`KismetMathLibrary.Conv_IntToDouble` _returnvalue))
      (if (== _returnvalue 5)
        _))
    (:`then_1`
      (set `self.CurrentAngle` NewAngle)
      (for (_array_element _array_index) Textures
        (switch `int` _array_index
          (:`0`
            (`MaterialInstanceDynamic.SetTextureParameterValue` _dynamicmaterial_2 "Tex1" _array_element))
          (:`1`
            (`MaterialInstanceDynamic.SetTextureParameterValue` _dynamicmaterial_2 "Tex2" _array_element))
          (:`2`
            (`MaterialInstanceDynamic.SetTextureParameterValue` _dynamicmaterial_2 "Tex3" _array_element))
          (:`3`
            (`MaterialInstanceDynamic.SetTextureParameterValue` _dynamicmaterial_2 "Tex4" _array_element))
          (:`4`
            (`MaterialInstanceDynamic.SetTextureParameterValue` _dynamicmaterial_2 "Tex5" _array_element))
          (:`5`
            (`MaterialInstanceDynamic.SetTextureParameterValue` _dynamicmaterial_2 "Tex6" _array_element))
          (:`6`
            (`MaterialInstanceDynamic.SetTextureParameterValue` _dynamicmaterial_2 "Tex7" _array_element))
          (:`7`
            (`MaterialInstanceDynamic.SetTextureParameterValue` _dynamicmaterial_2 "Tex8" _array_element))
          (:`8`
            (`MaterialInstanceDynamic.SetTextureParameterValue` _dynamicmaterial_2 "Tex9" _array_element))
          (:`9`
            (`MaterialInstanceDynamic.SetTextureParameterValue` _dynamicmaterial_2 "Tex10" _array_element)))))
    (:`then_2`
      (bind _output_get (set `self.MaterialFlipped` XFlip))
      (if _output_get
        (`MaterialInstanceDynamic.SetScalarParameterValue` _dynamicmaterial "XScale" -1.0)
        (else
          (`MaterialInstanceDynamic.SetScalarParameterValue` _dynamicmaterial "XScale" 1.0))))))

(fn `UpdateMaterialAngleStep`
  (params (DeltaTime :type "Float (double-precision)"))
  (locals (ResultAngle :type "Float (double-precision)" :default 0.0) (XFlip :type Boolean))
  (bind _returnvalue (`self.GetOwner`))
  (bind _resultangle (`local.ResultAngle`))
  (bind _skipdiagnonals (`self.SkipDiagnonals`))
  (bind _skipdiagnonals_2 (`self.SkipDiagnonals`))
  (bind _resultangle_2 (`local.ResultAngle`))
  (bind _yaw (.yaw (`KismetMathLibrary.NormalizedDeltaRotator` (`KismetMathLibrary.FindLookAtRotation` (`PlayerCameraManager.GetCameraLocation` (`self.CameraManager`)) (`Actor.K2_GetActorLocation` _returnvalue)) (`Actor.K2_GetActorRotation` _returnvalue))))
  (bind _returnvalue_2 (`KismetMathLibrary.Abs` _yaw))
  (`/Engine/EditorBlueprintResources/StandardMacros.IsValid` (`self.GetOwner`)
    (:`Is Valid`
      (if (`self.OrientToCamera`)
        (`/Engine/EditorBlueprintResources/StandardMacros.IsValid` (`self.CameraManager`)
          (:`Is Valid`
            _)
          (:`Is Not Valid`
            (set `self.CameraManager` (`GameplayStatics.GetPlayerCameraManager` 0))))
        (if (`self.OnlyOneSide`)
          (if (not (== (`self.CurrentAngle`) 180)) :!label _label
            (`self.UpdateMatByAngle` 180 (`self.0_Frames`) (`local.XFlip`)))
          (else
            (if (or (or (and (<= _returnvalue_2 22.5) (not (`self.SkipDiagnonals`))) (and (< _returnvalue_2 44.0) (`self.SkipDiagnonals`))) (or (and (> _returnvalue_2 157.5) (not (`self.SkipDiagnonals`))) (and (> _returnvalue_2 136.0) (`self.SkipDiagnonals`))))
              (set `local.XFlip` false)
              (else
                (set `local.XFlip` (xor (< (`KismetMathLibrary.SignOfFloat` _yaw) 0.0) (`self.FlipSideSprites`)))))
            (set `local.ResultAngle` (`KismetMathLibrary.Abs` _yaw))
            (if (or (and (> _resultangle_2 157.5) (not _skipdiagnonals_2)) (and (> _resultangle_2 136.0) _skipdiagnonals_2))
              (goto _label)
              (elif (and (> (`local.ResultAngle`) 112.0) (not (`self.SkipDiagnonals`)))
                (if (not (and (== (`self.CurrentAngle`) 135) (== (`self.MaterialFlipped`) (`local.XFlip`))))
                  (`self.UpdateMatByAngle` 135 (`self.45_Frames`) (`local.XFlip`)))
                (elif (or (and (> _resultangle 44.0) _skipdiagnonals) (and (> _resultangle 67.5) (not _skipdiagnonals)))
                  (if (not (and (== (`self.CurrentAngle`) 90) (== (`self.MaterialFlipped`) (`local.XFlip`))))
                    (`self.UpdateMatByAngle` 90 (`self.90_Frames`) (`local.XFlip`)))
                  (elif (and (> (`local.ResultAngle`) 22.5) (not (`self.SkipDiagnonals`)))
                    (if (not (and (== (`self.CurrentAngle`) 45) (== (`self.MaterialFlipped`) (`local.XFlip`))))
                      (`self.UpdateMatByAngle` 45 (`self.135_Frames`) (`local.XFlip`)))
                    (elif (not (== (`self.CurrentAngle`) 0))
                      (`self.UpdateMatByAngle` 0 (`self.180_Frames`) (`local.XFlip`)))))))))))))