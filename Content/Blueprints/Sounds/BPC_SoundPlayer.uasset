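; BPC_SoundPlayer is a component that plays a fall sound for a BP_2DGameCharacter.
; On BeginPlay it casts its owner to that character and takes its BPCStatTracking component.
; It binds PlayFallSound to that component's OnTakeDefeatingFall event, which plays the sound at the owner's location.
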(event `self.ReceiveBeginPlay`
  (bind _returnvalue (`self.GetOwner`))
  (`/Engine/EditorBlueprintResources/StandardMacros.IsValid` _returnvalue
    (:`Is Valid`
      (bind _asbp_2dgame_character (cast `/Game/Characters/CharacterBlueprints/BP_2DGameCharacter` _returnvalue))
      (bind _output_get (set `self.Owner` _asbp_2dgame_character))
      (bind _output_get_2 (set `self.StatTracking` (`/Game/Characters/CharacterBlueprints/BP_2DGameCharacter.BPC_StatTracking` _output_get)))
      (add `/Game/Blueprints/StatTracking/BPC_StatTracking.OnTakeDefeatingFall` _output_get_2 (delegate `PlayFallSound`)))))

(event `PlayFallSound`
  (`GameplayStatics.PlaySoundAtLocation` (`self.FallSound`) (`Actor.K2_GetActorLocation` (`self.Owner`)) (struct) 1.0 1.0 0.0 null null null null))