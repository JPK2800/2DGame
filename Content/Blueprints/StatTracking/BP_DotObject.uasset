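; Component that applies damage over time or healing over time to its Owner through the owner's BPCStatTracking.
; A looping timer started on BeginPlay calls HitDot every TimeToTick, sending non-negative Damage to TakeDamage and negative Damage, unnegated, to TakeHealing.
; Each successful tick subtracts TimeToTick from Duration, and the component clears its timer and destroys itself once Duration runs out.
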(event `self.ReceiveBeginPlay`
  (set `self.Duration` (`self.InitialDuration`))
  (bind _returnvalue (`KismetSystemLibrary.K2_SetTimer` null "HitDot" (`self.TimeToTick`) true))
  (set `self.Timer` _returnvalue))

(fn `HitDot`
  (bind _owner (`self.Owner`))
  (bind _damage (`self.Damage`))
  (bind _returnvalue (`KismetMathLibrary.Conv_IntToDouble` _damage))
  (bind _bpc_stattracking (`/Game/Characters/CharacterBlueprints/BP_2DGameCharacter.BPC_StatTracking` _owner))
  (`|ExecutionSequence`
    (:`then_0`
      (`/Engine/EditorBlueprintResources/StandardMacros.IsValid` _owner
        (:`Is Valid`
          (`/Engine/EditorBlueprintResources/StandardMacros.IsValid` _bpc_stattracking
            (:`Is Valid`
              (if (>= _damage 0)
                (`/Game/Blueprints/StatTracking/BPC_StatTracking.TakeDamage` _bpc_stattracking _returnvalue null true)
                (else
                  (`/Game/Blueprints/StatTracking/BPC_StatTracking.TakeHealing` _bpc_stattracking _returnvalue null true)))
              (set `self.Duration` (- (`self.Duration`) (`self.TimeToTick`))))))))
    (:`then_1`
      (if (<= (`self.Duration`) 0.0)
        (`KismetSystemLibrary.K2_ClearAndInvalidateTimerHandle` (`self.Timer`))
        (`self.K2_DestroyComponent`)))))