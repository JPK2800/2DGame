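; Health component for BP_2DGameCharacter that tracks current and max HP and handles damage, healing and defeat.
; Capsule overlaps with other-team projectiles route immediate damage by sign to TakeDamage or TakeHealing, and add BP_DotObject for damage over time.
; Clamped health changes fire dispatchers, driving placeholder printed numbers and optional owner destruction on defeat.
; Incapacitation is relayed through dispatchers, with a binding to the attacker's defeat event.
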(event `self.ReceiveBeginPlay`
  (bind _healthbase (`self.HealthBase`))
  (set `self.HealthMaxCurrent` _healthbase)
  (set `self.HealthCurrent` _healthbase)
  (bind _asbp_2dgame_character (cast `/Game/Characters/CharacterBlueprints/BP_2DGameCharacter` (`self.GetOwner`)))
  (set `self.OwnerCharacter` _asbp_2dgame_character)
  (add `PrimitiveComponent.OnComponentBeginOverlap` (`Character.CapsuleComponent` _asbp_2dgame_character) (delegate `OnBeginOverlap`))
  (add `self.OnTakeHit` (delegate `OnTakeHitDamageNumber`))
  (add `self.OnTakeHeal` (delegate `OnTakeHealHealingNumber`))
  (add `self.OnDefeatingHit` (delegate `OnTakeDefeatingHit`)))

(event `OnTakeHitDamageNumber` :!signature `self.OnTakeHit`
  (params (Damage :type "Float (double-precision)") (DotTick :type Boolean) (Attacker :type "/Game/Characters/CharacterBlueprints/BP_2DGameCharacter Object Reference"))
  (`self.SpawnDamageNumber` Damage))

(event `OnTakeHealHealingNumber` :!signature `self.OnTakeHeal`
  (params (Heal :type "Float (double-precision)") (HotTick :type Boolean))
  (`self.SpawnHealNumber` Heal))

(event `OnTakeDefeatingHit`
  (`self.CheckDestroyOwnerOnDefeat`))

(event `OnBeginOverlap`
  (params (OverlappedComponent :type "PrimitiveComponent Object Reference") (OtherActor :type "Actor Object Reference") (OtherComp :type "PrimitiveComponent Object Reference") (OtherBodyIndex :type Integer) (bFromSweep :type Boolean) (SweepResult :type "HitResult Structure (by ref)"))
  (bind _ownercharacter (`self.OwnerCharacter`))
  (bind _asbp_projectile (cast `/Game/ProjectilesAndSlashes/BP_Projectile` OtherActor))
  (`/Engine/EditorBlueprintResources/StandardMacros.IsValid` _ownercharacter
    (:`Is Valid`
      (bind _projectiledata (`/Game/ProjectilesAndSlashes/BP_Projectile.ProjectileData` _asbp_projectile))
      (if (!= (`.TeamID` (break `GenericTeamId` (`/Game/Characters/CharacterBlueprints/BP_2DGameCharacter.TeamId` _ownercharacter))) (`.TeamID` (break `GenericTeamId` (`.OriginTeamId_32_58FA1B63464A4B986646449B52B75D45` (break `/Game/ProjectilesAndSlashes/Struct_ProjectileDamageData` _projectiledata)))))
        (bind _asbp_2dgame_character (cast `/Game/Characters/CharacterBlueprints/BP_2DGameCharacter` (`Actor.GetOwner` _asbp_projectile)))
        (`self.TakeProjectileContact` _projectiledata _asbp_2dgame_character _asbp_projectile)))))

(fn `BeginDamageDot`
  (params (Data :type "/Game/ProjectilesAndSlashes/Struct_ProjectileDamageData Structure") (Attacker :type "/Game/Characters/CharacterBlueprints/BP_2DGameCharacter Object Reference"))
  (bind _ownercharacter (`self.OwnerCharacter`))
  (`/Engine/EditorBlueprintResources/StandardMacros.IsValid` _ownercharacter
    (:`Is Valid`
      (`|AddComponentByClass` _ownercharacter "/Game/Blueprints/StatTracking/BP_DotObject.BP_DotObject_C" Data_DamagePerTick_11_D680DDE24146E1A65A3E71A3926CA67E Data_TimeBetweenDotTicks_18_7322B4FB4D86989F21BA1FA92788F896 Data_DotDuration_16_C75169C14BC551769E48DE91C9A2E120 _ownercharacter Attacker))))

(fn `CheckDestroyOwnerOnDefeat`
  (bind _ownercharacter (`self.OwnerCharacter`))
  (if (`self.DestroyOwnerOnDefeat`)
    (if (`KismetSystemLibrary.IsValid` _ownercharacter)
      (`/Game/Characters/CharacterBlueprints/BP_2DGameCharacter.OwnerDestroyActor` _ownercharacter))))

(fn `EndIncapacitationByDefeatedAttacker`
  (`self.OnEndIncapacitation`))

(fn `GetBaseHP`
  (returns (BaseHealth :type "Float (double-precision)"))
  (return (`self.HealthBase`)))

(fn `GetCurrentHP`
  (returns (Health :type "Float (double-precision)"))
  (return (`self.HealthCurrent`)))

(fn `GetCurrentMaxHP`
  (returns (MaxHealth :type "Float (double-precision)"))
  (return (`self.HealthMaxCurrent`)))

(fn `ReceiveIncapacitation`
  (params (Attacker :type "/Game/Characters/CharacterBlueprints/BP_2DGameCharacter Object Reference") (Type :type Name) (HideAndAttachAttacker :type Boolean))
  (`self.OnReceiveIncapacitation` Type Attacker HideAndAttachAttacker)
  (add `self.OnDefeatingHit` (`/Game/Characters/CharacterBlueprints/BP_2DGameCharacter.BPC_StatTracking` Attacker) (`|CreateDelegate` :!event `EndIncapacitationByDefeatedAttacker`)))

(fn `SpawnDamageNumber`
  (params (Amount :type "Float (double-precision)") (Dot :type Boolean))
  (`KismetSystemLibrary.PrintString` (`KismetStringLibrary.Concat_StrStr` (`KismetSystemLibrary.GetDisplayName` (`self.GetOwner`)) " Damage: " (`KismetStringLibrary.Conv_DoubleToString` Amount))))

(fn `SpawnHealNumber`
  (params (Amount :type "Float (double-precision)") (Hot :type Boolean))
  (`KismetSystemLibrary.PrintString` (`KismetStringLibrary.Concat_StrStr` (`KismetSystemLibrary.GetDisplayName` (`self.GetOwner`)) " Healing: " (`KismetStringLibrary.Conv_DoubleToString` Amount))))

(fn `TakeDamage`
  (params (Damage :type "Float (double-precision)") (Attacker :type "/Game/Characters/CharacterBlueprints/BP_2DGameCharacter Object Reference") (Dot :type Boolean))
  (if (not (<= (`self.HealthCurrent`) 0.0))
    (bind _output_get (set `self.HealthCurrent` (`KismetMathLibrary.FClamp` (- (`self.HealthCurrent`) Damage) 0.0 (`self.HealthMaxCurrent`))))
    (`self.OnTakeHit` Damage Dot Attacker)
    (if (<= _output_get 0.0)
      (`self.OnDefeatingHit`))))

(fn `TakeHealing`
  (params (Heal :type "Float (double-precision)") (Attacker :type "/Game/Characters/CharacterBlueprints/BP_2DGameCharacter Object Reference") (Hot :type Boolean))
  (if (not (== (`self.HealthCurrent`) (`self.HealthMaxCurrent`)))
    (bind _output_get (set `self.HealthCurrent` (`KismetMathLibrary.FClamp` (+ (`self.HealthCurrent`) Heal) 0.0 (`self.HealthMaxCurrent`))))
    (`self.OnTakeHeal` Heal Hot)
    (if (>= _output_get (`self.HealthMaxCurrent`))
      (`self.OnFullHealth`))))

(fn `TakeProjectileContact`
  (params (Data :type "/Game/ProjectilesAndSlashes/Struct_ProjectileDamageData Structure") (Attacker :type "/Game/Characters/CharacterBlueprints/BP_2DGameCharacter Object Reference") (Projectile :type "/Game/ProjectilesAndSlashes/BP_Projectile Object Reference"))
  (bind (_dealsdamage _immediatedamage _dealsdamageinticks) (break `/Game/ProjectilesAndSlashes/Struct_ProjectileDamageData` Data))
  (bind _returnvalue (`KismetMathLibrary.Conv_IntToDouble` _immediatedamage))
  (`|ExecutionSequence`
    (:`then_0`
      (if _dealsdamage
        (if (>= _returnvalue 0.0)
          (`self.TakeDamage` _returnvalue Attacker)
          (else
            (`self.TakeHealing` _returnvalue Attacker)))))
    (:`then_1`
      (if _dealsdamageinticks
        (`self.BeginDamageDot` Data Attacker)))))