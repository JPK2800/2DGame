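; BP_Gate is an interactable gate actor that opens when its linked puzzle is completed.
; On BeginPlay it binds to the completion event of RelevantPuzzle, if one is set, and completion triggers BeginOpening.
; Tick then eases the static mesh toward an open relative location with VInterpTo, until a timer clears the opening flag after a fixed duration.
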(event `self.ReceiveBeginPlay`
  (bind _relevantpuzzle (`self.RelevantPuzzle`))
  (`/Engine/EditorBlueprintResources/StandardMacros.IsValid` _relevantpuzzle
    (:`Is Valid`
      (add `/Game/Interactables/PuzzleObjects/BP_PuzzleManagementActor.OnPuzzleComplete` _relevantpuzzle (delegate `OnPuzzleComplete`)))))

(event `OnPuzzleComplete`
  (`self.BeginOpening`))

(event `self.ReceiveTick`
  (params (DeltaSeconds :type "Float (single-precision)"))
  (`self.InterpWhenOpened` DeltaSeconds))

(fn `BeginOpening`
  (`KismetSystemLibrary.K2_SetTimer` null "StopOpening" 8.0)
  (set `self.IsOpening` true))

(fn `InterpWhenOpened`
  (params (Delta :type "Float (double-precision)"))
  (bind _staticmesh (`self.StaticMesh`))
  (if (`self.IsOpening`)
    (`SceneComponent.K2_SetRelativeLocation` _staticmesh (`KismetMathLibrary.VInterpTo` (`SceneComponent.RelativeLocation` _staticmesh) (`self.OpenRelativeLoc`) Delta 3.0) false false)))

(fn `StopOpening`
  (set `self.IsOpening` false))

(fn `UserConstructionScript`)