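; BPC_InteractListenerComponent is an actor component that links an interaction actor to the puzzle logic on its owner.
; On BeginPlay it binds to the interaction actor's player interaction event and, if the owner is a BP_PuzzleManagementActor, to its puzzle completion event.
; Interactions route through a server event to the OnInteract dispatcher.
; Completion likewise passes through a server event to mark the interaction actor's puzzle completed.
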(event `self.ReceiveBeginPlay`
  (`self.InitInteractActor` (`self.InteractionActor`))
  (`self.InitOwnerCompletionEvent`))

(event `ServerInteraction`
  (params (InteractData :type String))
  (`self.InteractionFunction` InteractData))

(event `ServerPuzzleComplete`
  (`self.CompleteFunction`))

(fn `CompleteFunction`
  (`/Game/Interactables/BP_InteractableActor.UpdatePuzzleCompleted` (`self.InteractionActor`) true))

(fn `InitInteractActor`
  (params (Actor :type "/Game/Interactables/BP_InteractableActor Object Reference"))
  (`/Engine/EditorBlueprintResources/StandardMacros.IsValid` Actor
    (:`Is Valid`
      (add `/Game/Interactables/BP_InteractableActor.OnPlayerInteraction` Actor (`|CreateDelegate` :!event `InteractOnServer`)))))

(fn `InitOwnerCompletionEvent`
  (bind _asbp_puzzle_management_actor (cast `/Game/Interactables/PuzzleObjects/BP_PuzzleManagementActor` (`self.GetOwner`)))
  (add `/Game/Interactables/PuzzleObjects/BP_PuzzleManagementActor.OnPuzzleComplete` _asbp_puzzle_management_actor (`|CreateDelegate` :!event `OnPuzzleComplete`)))

(fn `InteractionFunction`
  (params (InteractData :type String))
  (`self.OnInteract` InteractData))

(fn `InteractOnServer`
  (params (InteractData :type String))
  (`self.ServerInteraction` InteractData))

(fn `OnPuzzleComplete`
  (`self.ServerPuzzleComplete`))