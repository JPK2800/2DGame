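; Multiplayer puzzle manager in which interactions toggle four skulls (A to D), and the puzzle completes when all are active.
; Four interact listener components forward a data string to a server event, where each letter it contains flips that skull, so one interaction can toggle several.
; RepNotify states swap each skull between green and grey materials.
; Completion checking and handling override parent puzzle functions, with completion adding only a debug print.
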(event `self.ReceiveBeginPlay`
  (`parent.ReceiveBeginPlay`)
  (`self.SetSkullActive` (`self.A_Active`) (`self.SkullA`))
  (`self.SetSkullActive` (`self.B_Active`) (`self.SkullB`))
  (`self.SetSkullActive` (`self.C_Active`) (`self.SkullC`))
  (`self.SetSkullActive` (`self.D_Active`) (`self.SkullD`)))

(event `self.BPC_InteractListenerComponentB.OnInteract`
  (params (InteractData :type String))
  (`self.ServerUpdateData` InteractData))

(event `self.BPC_InteractListenerComponentC.OnInteract`
  (params (InteractData :type String))
  (`self.ServerUpdateData` InteractData))

(event `self.BPC_InteractListenerComponentD.OnInteract`
  (params (InteractData :type String))
  (`self.ServerUpdateData` InteractData))

(event `self.BPC_InteractListenerComponentA.OnInteract`
  (params (InteractData :type String))
  (`self.ServerUpdateData` InteractData))

(event `ServerUpdateData`
  (params (Data :type String))
  (`self.UpdateData` Data))

(fn `CheckIfPuzzleIsComplete`
  (returns (Complete :type Boolean))
  (`parent.CheckIfPuzzleIsComplete`)
  (return (and (`self.A_Active`) (`self.B_Active`) (`self.C_Active`) (`self.D_Active`))))

(fn `OnRep_A_Active`
  (`self.SetSkullActive` (`self.A_Active`) (`self.SkullA`)))

(fn `OnRep_B_Active`
  (`self.SetSkullActive` (`self.B_Active`) (`self.SkullB`)))

(fn `OnRep_C_Active`
  (`self.SetSkullActive` (`self.C_Active`) (`self.SkullC`)))

(fn `OnRep_D_Active`
  (`self.SetSkullActive` (`self.D_Active`) (`self.SkullD`)))

(fn `PuzzleComplete`
  (`parent.PuzzleComplete`)
  (`KismetSystemLibrary.PrintString` "PuzzleComplete"))

(fn `SetSkullActive`
  (params (Activate :type Boolean) (Mesh :type "StaticMeshComponent Object Reference"))
  (if Activate
    (`PrimitiveComponent.SetMaterial` Mesh 0 "/Game/Interactables/PuzzleObjects/Green_puzzle_skull_1/MI_GreenPuzzleSkull.MI_GreenPuzzleSkull")
    (else
      (`PrimitiveComponent.SetMaterial` Mesh 0 "/Game/Interactables/PuzzleObjects/Grey_skull_puzzle/MI_GreySkull.MI_GreySkull"))))

(fn `UpdateData`
  (params (Data :type String))
  (`|ExecutionSequence`
    (:`then_0`
      (if (`KismetStringLibrary.Contains` Data "A")
        (bind _output_get (set `self.A_Active` (not (`self.A_Active`))))
        (`self.SetSkullActive` _output_get (`self.SkullA`))))
    (:`then_1`
      (if (`KismetStringLibrary.Contains` Data "B")
        (bind _output_get_2 (set `self.B_Active` (not (`self.B_Active`))))
        (`self.SetSkullActive` _output_get_2 (`self.SkullB`))))
    (:`then_2`
      (if (`KismetStringLibrary.Contains` Data "C")
        (bind _output_get_3 (set `self.C_Active` (not (`self.C_Active`))))
        (`self.SetSkullActive` _output_get_3 (`self.SkullC`))))
    (:`then_3`
      (if (`KismetStringLibrary.Contains` Data "D")
        (bind _output_get_4 (set `self.D_Active` (not (`self.D_Active`))))
        (`self.SetSkullActive` _output_get_4 (`self.SkullD`))))
    (:`then_4`
      (bind _complete (`self.CheckIfPuzzleIsComplete`))
      (if _complete
        (set `self.PuzzleCompleted` true)
        (`self.PuzzleComplete`)))))

(fn `UserConstructionScript`
  (`parent.UserConstructionScript`))