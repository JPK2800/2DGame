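; Puzzle management actor that provides the hooks for checking and announcing completion of a puzzle, apparently as a base for specific puzzles.
; CheckIfPuzzleIsComplete is a stub returning false, and PuzzleComplete only fires the OnPuzzleComplete dispatcher.
; The PuzzleCompleted RepNotify spawns an optional dialogue actor at this actor's transform, owned by player 0's character, and plays an optional 2D completion sound.
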(fn `CheckIfPuzzleIsComplete`
  (returns (Complete :type Boolean))
  (return false))

(fn `OnRep_PuzzleCompleted`
  (bind _returnvalue (`GameplayStatics.GetPlayerCharacter` 0))
  (bind _spawndialogueoncompletion (`self.SpawnDialogueOnCompletion`))
  (bind _completesound (`self.CompleteSound`))
  (`|ExecutionSequence`
    (:`then_0`
      (if (`KismetSystemLibrary.IsValidClass` _spawndialogueoncompletion)
        (`|SpawnActorFromClass` _spawndialogueoncompletion (`self.GetTransform`) "Undefined" "MultiplyWithRoot" _returnvalue _returnvalue)))
    (:`then_1`
      (`/Engine/EditorBlueprintResources/StandardMacros.IsValid` _completesound
        (:`Is Valid`
          (`GameplayStatics.PlaySound2D` _completesound 1.0 1.0 0.0 null null))))))

(fn `PuzzleComplete`
  (`self.OnPuzzleComplete`))

(fn `UserConstructionScript`)