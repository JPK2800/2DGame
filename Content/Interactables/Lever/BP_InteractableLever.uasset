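; Interactable lever Blueprint that animates between its on and off states, built as a child of a parent interactable class.
; Its active and inactive mode overrides call the parent, then play the matching one-shot toggle animation on the skeletal mesh.
; Player interaction and construction pass straight through to the parent, and the event graph holds no active logic.
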(fn `PlayerInteracted`
  (`parent.PlayerInteracted`))

(fn `Set Mode Active`
  (`parent.Set Mode Active`)
  (`SkeletalMeshComponent.PlayAnimation` (`self.SkeletalMesh`) "/Game/Interactables/Lever/dungeon1_lever1_Anim_Armature_ToggleOn.dungeon1_lever1_Anim_Armature_ToggleOn" false))

(fn `SetModeInactive`
  (`parent.SetModeInactive`)
  (`SkeletalMeshComponent.PlayAnimation` (`self.SkeletalMesh`) "/Game/Interactables/Lever/dungeon1_lever1_Anim_Armature_ToggleOff.dungeon1_lever1_Anim_Armature_ToggleOff" false))

(fn `UserConstructionScript`
  (`parent.UserConstructionScript`))