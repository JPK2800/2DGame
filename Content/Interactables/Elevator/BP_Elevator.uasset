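; Elevator actor that moves its static mesh back and forth between two positions, PositionA and PositionB.
; On BeginPlay the server spawns a pressure plate, attaches it to the mesh and binds its interaction event.
; Authority-only SetNewDestination ignores calls during travel, otherwise toggles the target and calls MoveElevator.
; A timeline eases from the mesh's current location toward the target, then clears the travel flag and signals readiness for interaction.
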(event `self.ReceiveBeginPlay`
  (if (`self.HasAuthority`)
    (bind _returnvalue (`|SpawnActorFromClass` "/Game/Interactables/PressurePlate/BP_PressurePlate.BP_PressurePlate_C" (`KismetMathLibrary.MakeTransform` (0.0 0.0 20.0) (struct) (1.5 1.5 1.5)) "Undefined" "MultiplyWithRoot" self "" false "/Game/Sounds/lever/leverpull.leverpull" null))
    (`self.K2_AttachToComponent` _returnvalue (`self.StaticMesh`) "None" "KeepRelative" "KeepRelative" "KeepWorld" true)
    (add `/Game/Interactables/BP_InteractableActor.OnPlayerInteraction` _returnvalue (`|CreateDelegate` :!event `SetNewDestination`))
    (add `self.OnReadyForNewInteract` (`|CreateDelegate` _returnvalue :!event `ReenableInteractFromTimer`))))

(event `self.ReceiveTick`
  (params (DeltaSeconds :type "Float (single-precision)")))

(event `MoveElevator`
  (if (`self.IsTraveling`)
    (bind (_direction _newtrack_1) (`Timeline|MoveTimeline` :!via `PlayFromStart`)
      (:`Update`
        (`SceneComponent.K2_SetRelativeLocation` (`self.StaticMesh`) (`|EaseFunction` "EaseInOut" _newtrack_1 (`SceneComponent.RelativeLocation` (`self.StaticMesh`)) (`self.DestPos`) 1.0) false false))
      (:`Finished`
        (set `self.IsTraveling` false)
        (`self.OnReadyForNewInteract`)))))

(fn `SetNewDestination`
  (params (InteractData :type String))
  (if (`self.HasAuthority`)
    (if (not (`self.IsTraveling`))
      (set `self.IsTraveling` true)
      (if (`self.AtPosA`)
        (set `self.DestPos` (`SceneComponent.RelativeLocation` (`self.Position_B`)))
        (set `self.AtPosA` false)
        (else
          (set `self.DestPos` (`SceneComponent.RelativeLocation` (`self.Position_A`)))
          (set `self.AtPosA` true)))
      (`self.MoveElevator`))))

(fn `UserConstructionScript`)