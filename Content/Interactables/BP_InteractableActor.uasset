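; Base interactable actor for a networked 2D puzzle game that players toggle between active and inactive.
; Its box overlap shows an interact widget and binds the local player's interact event until the puzzle is completed.
; Interaction fires a dispatcher and flips IsActive, whose RepNotify calls empty mode hooks and briefly locks input on a timer.
; Server-section events set the active and completed states; completion hides the widget.
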(event `self.ReceiveBeginPlay`
  (if (`self.IsActive`)
    (`self.Set Mode Active`)
    (else
      (`self.SetModeInactive`))))

(event `self.InteractionBox.OnComponentBeginOverlap`
  (params (OverlappedComponent :type "PrimitiveComponent Object Reference") (OtherActor :type "Actor Object Reference") (OtherComp :type "PrimitiveComponent Object Reference") (OtherBodyIndex :type Integer) (bFromSweep :type Boolean) (SweepResult :type "HitResult Structure (by ref)"))
  (bind _asbp_2dgame_character (cast `/Game/Characters/CharacterBlueprints/BP_2DGameCharacter` OtherActor))
  (if (and (`Pawn.IsLocallyControlled` _asbp_2dgame_character) (`Pawn.IsPlayerControlled` _asbp_2dgame_character))
    (`self.BeginOverlapPlayer` _asbp_2dgame_character)
    (`self.OnBeginOverlapPlayer` _asbp_2dgame_character)))

(event `self.InteractionBox.OnComponentEndOverlap`
  (params (OverlappedComponent :type "PrimitiveComponent Object Reference") (OtherActor :type "Actor Object Reference") (OtherComp :type "PrimitiveComponent Object Reference") (OtherBodyIndex :type Integer))
  (bind _asbp_2dgame_character (cast `/Game/Characters/CharacterBlueprints/BP_2DGameCharacter` OtherActor))
  (if (and (`Pawn.IsLocallyControlled` _asbp_2dgame_character) (`Pawn.IsPlayerControlled` _asbp_2dgame_character))
    (`self.EndOverlapPlayer` _asbp_2dgame_character)
    (`self.OnEndOverlapPlayer` _asbp_2dgame_character)))

(event `UpdateInteractableMode`
  (params (Active :type Boolean))
  (set `self.IsActive` Active))

(event `UpdatePuzzleCompleted`
  (params (Complete :type Boolean))
  (set `self.CompletedPuzzle` Complete))

(fn `OnBeginOverlapPlayer`
  (params (Player :type "/Game/Characters/CharacterBlueprints/BP_2DGameCharacter Object Reference"))
  (if (not (`self.CompletedPuzzle`))
    (`SceneComponent.SetHiddenInGame` (`self.InteractWidget`) false false)
    (add `/Game/Characters/CharacterBlueprints/BP_2DGameCharacter.OnInteract` Player (`|CreateDelegate` :!event `PlayerInteracted`))))

(fn `OnEndOverlapPlayer`
  (params (Player :type "/Game/Characters/CharacterBlueprints/BP_2DGameCharacter Object Reference"))
  (`SceneComponent.SetHiddenInGame` (`self.InteractWidget`) true false)
  (clear `/Game/Characters/CharacterBlueprints/BP_2DGameCharacter.OnInteract` Player))

(fn `OnRep_CompletedPuzzle`
  (if (`self.CompletedPuzzle`)
    (`SceneComponent.SetHiddenInGame` (`self.InteractWidget`) true false)))

(fn `OnRep_IsActive`
  (if (`self.IsActive`)
    (`self.Set Mode Active`)
    (else
      (`self.SetModeInactive`)))
  (set `self.AllowInput` false)
  (`KismetSystemLibrary.K2_SetTimer` null "ReenableInteractFromTimer" (`self.InteractAbilityInterval`)))

(fn `PlayerInteracted`
  (if (and (`self.AllowInput`) (not (`self.CompletedPuzzle`)))
    (`self.OnPlayerInteraction` (`self.InteractData`))
    (set `self.IsActive` (not (`self.IsActive`)))))

(fn `ReenableInteractFromTimer`
  (set `self.AllowInput` true))

(fn `Set Mode Active`)

(fn `SetModeInactive`)

(fn `UserConstructionScript`)