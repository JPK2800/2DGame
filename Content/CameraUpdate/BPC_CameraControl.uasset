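; Camera control component for BP_2DGameCharacter that smoothly changes field of view and spring arm length.
; On BeginPlay it caches the owner's Camera and SpringArm.
; SetTargetFov and SetTargetArmLen store targets and raise flags.
; Tick eases each flagged value toward its target with FInterpTo, then snaps and clears the flag once within a small tolerance.
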(event `self.ReceiveBeginPlay`
  (`self.Init`))

(event `self.ReceiveTick`
  (params (DeltaSeconds :type "Float (single-precision)"))
  (`self.InterpFov` DeltaSeconds)
  (`self.InterpArmLen` DeltaSeconds))

(fn `Init`
  (bind _asbp_2dgame_character (cast `/Game/Characters/CharacterBlueprints/BP_2DGameCharacter` (`self.GetOwner`)))
  (set `self.OwnerCam` (`/Game/Characters/CharacterBlueprints/BP_2DGameCharacter.Camera` _asbp_2dgame_character))
  (set `self.OwnerSpringArm` (`/Game/Characters/CharacterBlueprints/BP_2DGameCharacter.SpringArm` _asbp_2dgame_character)))

(fn `InterpArmLen`
  (params (Delta :type "Float (double-precision)"))
  (bind _targetarmlen (`self.TargetArmLen`))
  (bind _ownerspringarm (`self.OwnerSpringArm`))
  (bind _targetarmlength (`SpringArmComponent.TargetArmLength` (`self.OwnerSpringArm`)))
  (if (`self.IsChangingSprintArmLen`)
    (if (<= (`KismetMathLibrary.Abs` (- _targetarmlength _targetarmlen)) 1.0)
      (set `SpringArmComponent.TargetArmLength` _targetarmlen _ownerspringarm)
      (set `self.IsChangingSprintArmLen` false)
      (else
        (set `SpringArmComponent.TargetArmLength` (`KismetMathLibrary.FInterpTo` _targetarmlength _targetarmlen Delta 1.0) _ownerspringarm)))))

(fn `InterpFov`
  (params (Delta :type "Float (double-precision)"))
  (bind _ownercam (`self.OwnerCam`))
  (bind _targetfov (`self.TargetFov`))
  (bind _fieldofview (`CameraComponent.FieldOfView` _ownercam))
  (if (`self.IsChangingFov`)
    (if (<= (`KismetMathLibrary.Abs` (- _fieldofview _targetfov)) 1.0)
      (`CameraComponent.SetFieldOfView` _ownercam _targetfov)
      (set `self.IsChangingFov` false)
      (else
        (`CameraComponent.SetFieldOfView` _ownercam (`KismetMathLibrary.FInterpTo` _fieldofview _targetfov Delta 1.0))))))

(fn `SetTargetArmLen`
  (params (Len :type "Float (double-precision)"))
  (set `self.TargetArmLen` Len)
  (set `self.IsChangingSprintArmLen` true))

(fn `SetTargetFov`
  (params (Fov :type "Float (double-precision)"))
  (set `self.IsChangingFov` true)
  (set `self.TargetFov` Fov))