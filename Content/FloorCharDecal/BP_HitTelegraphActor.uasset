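; Ground telegraph actor that warns of an incoming team-based hit, then damages overlapping enemy characters when its timer expires.
; A flipbook decal is tinted enemy or ally relative to the local player, shifting toward a trigger color over the countdown.
; Mesh overlaps track and notify opposing characters; only locally controlled victims apply the hit.
; It self-destroys after triggering or on owner defeat, spawning optional FX and clearing overlap notifications.
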(event `self.ReceiveBeginPlay`
  (`self.InitDestroyOnOwnerDefeat`)
  (`self.InitDecalTextures`)
  (`self.TraceOnCreate`)
  (`KismetSystemLibrary.K2_SetTimer` null "TriggerHit" (`self.TimeToTriggerHit`))
  (add `self.OnDestroyed` (delegate `OnDestroy`)))

(event `OnDestroy` :!signature `self.OnDestroyed`
  (params (DestroyedActor :type "Actor Object Reference"))
  (`self.SpawnFxOnDestroy`)
  (for _array_element (`self.OverlappingEnemyActors`)
    (`/Game/Characters/CharacterBlueprints/BP_2DGameCharacter.Overlapped Telegraph` _array_element self false)))

(event `self.StaticMesh.OnComponentBeginOverlap`
  (params (OverlappedComponent :type "PrimitiveComponent Object Reference") (OtherActor :type "Actor Object Reference") (OtherComp :type "PrimitiveComponent Object Reference") (OtherBodyIndex :type Integer) (bFromSweep :type Boolean) (SweepResult :type "HitResult Structure (by ref)"))
  (bind _teamid_teamid (break `GenericTeamId` (`self.TeamId`)))
  (bind _asbp_2dgame_character (cast `/Game/Characters/CharacterBlueprints/BP_2DGameCharacter` OtherActor))
  (bind _teamid_teamid_2 (break `GenericTeamId` (`/Game/Characters/CharacterBlueprints/BP_2DGameCharacter.TeamId` _asbp_2dgame_character)))
  (if (!= _teamid_teamid_2 _teamid_teamid)
    (`KismetArrayLibrary.Array_AddUnique` (`self.OverlappingEnemyActors`) _asbp_2dgame_character)
    (`/Game/Characters/CharacterBlueprints/BP_2DGameCharacter.Overlapped Telegraph` _asbp_2dgame_character self true)))

(event `self.StaticMesh.OnComponentEndOverlap`
  (params (OverlappedComponent :type "PrimitiveComponent Object Reference") (OtherActor :type "Actor Object Reference") (OtherComp :type "PrimitiveComponent Object Reference") (OtherBodyIndex :type Integer))
  (bind _overlappingenemyactors (`self.OverlappingEnemyActors`))
  (bind _asbp_2dgame_character (cast `/Game/Characters/CharacterBlueprints/BP_2DGameCharacter` OtherActor))
  (if (`KismetArrayLibrary.Array_Contains` _overlappingenemyactors _asbp_2dgame_character)
    (`KismetArrayLibrary.Array_RemoveItem` _overlappingenemyactors _asbp_2dgame_character)
    (`/Game/Characters/CharacterBlueprints/BP_2DGameCharacter.Overlapped Telegraph` _asbp_2dgame_character self false)))

(fn `InitDecalTextures`
  (bind _decaltextures (`self.DecalTextures`))
  (bind _returnvalue (`KismetMaterialLibrary.CreateDynamicMaterialInstance` "/Game/Mat_FlipbookDecal.Mat_FlipbookDecal"))
  (bind _output_get (set `self.DynamicMaterial` _returnvalue))
  (`DecalComponent.SetDecalMaterial` (`self.Decal`) _output_get)
  (`|ExecutionSequence`
    (:`then_0`
      ;[1 0.2622 0.6378] Init Params
      (for (_array_element _array_index) _decaltextures
        (switch `int` _array_index
          (:`0`
            (`MaterialInstanceDynamic.SetTextureParameterValue` _output_get "Tex1" _array_element))
          (:`1`
            (`MaterialInstanceDynamic.SetTextureParameterValue` _output_get "Tex2" _array_element))
          (:`2`
            (`MaterialInstanceDynamic.SetTextureParameterValue` _output_get "Tex3" _array_element))
          (:`3`
            (`MaterialInstanceDynamic.SetTextureParameterValue` _output_get "Tex4" _array_element))))
      (`MaterialInstanceDynamic.SetScalarParameterValue` _output_get "TexCount" (`KismetMathLibrary.Conv_IntToDouble` (`KismetArrayLibrary.Array_Length` _decaltextures))))
    (:`then_1`
      (`self.InitTelegraphColors`))))

(fn `InitDestroyOnOwnerDefeat`
  (bind _ownerchar (`self.OwnerChar`))
  (`/Engine/EditorBlueprintResources/StandardMacros.IsValid` _ownerchar
    (:`Is Valid`
      (add `/Game/Blueprints/StatTracking/BPC_StatTracking.OnDefeatingHit` (`/Game/Characters/CharacterBlueprints/BP_2DGameCharacter.BPC_StatTracking` _ownerchar) (`|CreateDelegate` :!event `OnOwnerDefeat`)))))

(fn `InitTelegraphColors`
  (bind _teamid_teamid (break `GenericTeamId` (`self.TeamId`)))
  (bind _dynamicmaterial (`self.DynamicMaterial`))
  (bind _asbp_2dgame_character (cast `/Game/Characters/CharacterBlueprints/BP_2DGameCharacter` (`GameplayStatics.GetPlayerCharacter` 0)))
  (bind _teamid_teamid_2 (break `GenericTeamId` (`/Game/Characters/CharacterBlueprints/BP_2DGameCharacter.TeamId` _asbp_2dgame_character)))
  (if (!= _teamid_teamid_2 _teamid_teamid)
    (set `self.IsEnemyDamage` true)
    (`MaterialInstanceDynamic.SetVectorParameterValue` _dynamicmaterial "ColorParameter" (`self.EnemyDamageColorStart`))
    (set `self.CurrentColorStart` (`self.EnemyDamageColorStart`))
    (set `self.CurrentColorTrigger` (`self.EnemyDamageColorTrigger`))
    (else
      (set `self.IsAllyDamage` true)
      (`MaterialInstanceDynamic.SetVectorParameterValue` _dynamicmaterial "ColorParameter" (`self.AllyDamageColorStart`))
      (set `self.CurrentColorStart` (`self.AllyDamageColorStart`))
      (set `self.CurrentColorTrigger` (`self.AllyDamageColorTrigger`))))
  (`KismetSystemLibrary.K2_SetTimer` null "UpdateColor" (`self.ColorShiftTickRate`) true))

(fn `OnOwnerDefeat`
  (`self.K2_DestroyActor`))

(fn `SpawnFxOnDestroy`
  (bind (_returnvalue_location _returnvalue_rotation) (`KismetMathLibrary.BreakTransform` (`self.GetTransform`)))
  (bind _fpfxactor (`self.FpFxActor`))
  (if (`KismetSystemLibrary.IsValidClass` _fpfxactor)
    (`|SpawnActorFromClass` _fpfxactor (`KismetMathLibrary.MakeTransform` _returnvalue_location _returnvalue_rotation) "Undefined" "MultiplyWithRoot" self null)))

(fn `TraceOnCreate`
  (bind _teamid_teamid (break `GenericTeamId` (`self.TeamId`)))
  (for _array_element (`PrimitiveComponent.GetOverlappingActors` (`self.StaticMesh`) null)
    (bind _asbp_2dgame_character (cast `/Game/Characters/CharacterBlueprints/BP_2DGameCharacter` _array_element))
    (bind _teamid_teamid_2 (break `GenericTeamId` (`/Game/Characters/CharacterBlueprints/BP_2DGameCharacter.TeamId` _asbp_2dgame_character)))
    (if (!= _teamid_teamid_2 _teamid_teamid)
      (`KismetArrayLibrary.Array_AddUnique` (`self.OverlappingEnemyActors`) _asbp_2dgame_character))))

(fn `TriggerHit`
  (`|ExecutionSequence`
    (:`then_0`
      (for _array_element (`self.OverlappingEnemyActors`)
        (if (`Pawn.IsLocallyControlled` _array_element)
          (bind _asbp_2dgame_character (cast `/Game/Characters/CharacterBlueprints/BP_2DGameCharacter` (`self.GetOwner`)))
          (`/Game/Blueprints/StatTracking/BPC_StatTracking.TakeContact` (`/Game/Characters/CharacterBlueprints/BP_2DGameCharacter.BPC_StatTracking` _array_element) (`self.DamageData`) _asbp_2dgame_character null))))
    (:`then_1`
      (`self.K2_DestroyActor`))))

(fn `UpdateColor`
  (bind _dynamicmaterial (`self.DynamicMaterial`))
  (bind _output_get (set `self.ProgressTIme` (+ (`self.ProgressTIme`) (`self.ColorShiftTickRate`))))
  (`/Engine/EditorBlueprintResources/StandardMacros.IsValid` _dynamicmaterial
    (:`Is Valid`
      (`MaterialInstanceDynamic.SetVectorParameterValue` _dynamicmaterial "ColorParameter" (`KismetMathLibrary.LinearColorLerp` (`self.CurrentColorStart`) (`self.CurrentColorTrigger`) (`KismetMathLibrary.MultiplyMultiply_FloatFloat` (/ _output_get (`self.TimeToTriggerHit`)) 0.5))))))

(fn `UserConstructionScript`)