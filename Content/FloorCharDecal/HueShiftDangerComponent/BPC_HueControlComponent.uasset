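; Character component that tints a BP_2DGameCharacter's billboard sprite with the color of a telegraph overlapping it.
; Owner overlap events maintain enemy and ally telegraph lists by team ID, and the fallback selection favors enemies over allies.
; The chosen color drives hue-shift parameters on the dynamic material, switching off when no telegraph is selected.
; A looping timer with a randomized interval prunes the lists and refreshes the tint.
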(event `self.ReceiveBeginPlay`
  (bind _asbp_2dgame_character (cast `/Game/Characters/CharacterBlueprints/BP_2DGameCharacter` (`self.GetOwner`)))
  (`self.Init` (`/Game/Blueprints/Billboard_Limbs/BPC_BillboardLimb.DynamicMaterial` (`/Game/Characters/CharacterBlueprints/BP_2DGameCharacter.BPC_BillboardCharacter` _asbp_2dgame_character)) _asbp_2dgame_character))

(fn `ChangeCurrentColor`
  (params (UseColor :type Boolean) (Color :type "LinearColor Structure"))
  (bind _dynamicmaterial (`self.DynamicMaterial`))
  (`/Engine/EditorBlueprintResources/StandardMacros.IsValid` _dynamicmaterial
    (:`Is Valid`
      (if UseColor
        (`MaterialInstanceDynamic.SetScalarParameterValue` _dynamicmaterial "UseColorShiftForTelegraph" 1.0)
        (`MaterialInstanceDynamic.SetVectorParameterValue` _dynamicmaterial "ColorShiftTelegraph" (make `LinearColor` Color_R Color_G Color_B 1.0))
        (else
          (`MaterialInstanceDynamic.SetScalarParameterValue` _dynamicmaterial "UseColorShiftForTelegraph" 0.0))))))

(fn `Init`
  (params (DynamicMaterial :type "MaterialInstanceDynamic Object Reference") (Owner :type "/Game/Characters/CharacterBlueprints/BP_2DGameCharacter Object Reference"))
  (set `self.DynamicMaterial` DynamicMaterial)
  (bind _output_get (set `self.Owner` Owner))
  (add `/Game/Characters/CharacterBlueprints/BP_2DGameCharacter.OnTelegraphOverlap` _output_get (`|CreateDelegate` :!event `OverlappedByTelegraph`))
  (add `/Game/Characters/CharacterBlueprints/BP_2DGameCharacter.OnTelegraphOverlapEnd` _output_get (`|CreateDelegate` :!event `OverlapEndByTelegraph`))
  (`KismetSystemLibrary.K2_SetTimer` null "TelegraphHouseKeeping" (`KismetMathLibrary.RandomFloatInRange` 18.0 25.0) true))

(fn `OverlapEndByTelegraph`
  (params (Telegraph :type "/Game/FloorCharDecal/BP_HitTelegraphActor Object Reference"))
  (`KismetArrayLibrary.Array_RemoveItem` (`self.Telegraphs_Enemy`) Telegraph)
  (`KismetArrayLibrary.Array_RemoveItem` (`self.Telegraphs_Ally`) Telegraph)
  (`self.UpdateOverlapHue` null))

(fn `OverlappedByTelegraph`
  (params (Telegraph :type "/Game/FloorCharDecal/BP_HitTelegraphActor Object Reference"))
  (bind _telegraphs_enemy (`self.Telegraphs_Enemy`))
  (bind _teamid_teamid (break `GenericTeamId` (`/Game/FloorCharDecal/BP_HitTelegraphActor.TeamId` Telegraph)))
  (bind _teamid_teamid_2 (break `GenericTeamId` (`/Game/Characters/CharacterBlueprints/BP_2DGameCharacter.TeamId` (`self.Owner`))))
  (if (`KismetSystemLibrary.IsValid` (`self.Owner`))
    (if (and (not (`KismetArrayLibrary.Array_Contains` _telegraphs_enemy Telegraph)) (not (`KismetArrayLibrary.Array_Contains` _telegraphs_enemy)))
      (if (!= _teamid_teamid _teamid_teamid_2)
        (`KismetArrayLibrary.Array_AddUnique` (`self.Telegraphs_Enemy`) Telegraph)
        (else
          (`KismetArrayLibrary.Array_AddUnique` (`self.Telegraphs_Ally`) Telegraph)))
      (`self.UpdateOverlapHue` Telegraph))))

(fn `TelegraphHouseKeeping`
  (locals (TelegraphsToRemove :type "Array of Integer"))
  (for (_array_element _array_index) (`self.Telegraphs_Enemy`)
    (`/Engine/EditorBlueprintResources/StandardMacros.IsValid` _array_element
      (:`Is Valid`
        (`KismetArrayLibrary.Array_Add` (`local.TelegraphsToRemove`) _array_index))))
  (bind (_arrayindex _arrayelement) (`/Engine/EditorBlueprintResources/StandardMacros.ReverseForEachLoop` (`local.TelegraphsToRemove`))
    (:`LoopBody`
      (`KismetArrayLibrary.Array_Remove` (`self.Telegraphs_Enemy`) _arrayelement))
    (:`Completed`
      (`KismetArrayLibrary.Array_Clear` (`local.TelegraphsToRemove`))
      (for (_array_element_2 _array_index_2) (`self.Telegraphs_Enemy`)
        (`/Engine/EditorBlueprintResources/StandardMacros.IsValid` _array_element_2
          (:`Is Valid`
            (`KismetArrayLibrary.Array_Add` (`local.TelegraphsToRemove`) _array_index_2))))
      (bind (_arrayindex_2 _arrayelement_2) (`/Engine/EditorBlueprintResources/StandardMacros.ReverseForEachLoop` (`local.TelegraphsToRemove`))
        (:`LoopBody`
          (`KismetArrayLibrary.Array_Remove` (`self.Telegraphs_Ally`) _arrayelement_2))
        (:`Completed`
          (`self.UpdateOverlapHue` null))))))

(fn `UpdateOverlapHue`
  (params (NewTelegraph :type "/Game/FloorCharDecal/BP_HitTelegraphActor Object Reference"))
  (bind _currentcolortrigger (`/Game/FloorCharDecal/BP_HitTelegraphActor.CurrentColorTrigger` NewTelegraph))
  (bind _telegraphs_enemy (`self.Telegraphs_Enemy`))
  (bind _telegraphs_ally (`self.Telegraphs_Ally`))
  (bind _teamid_teamid (break `GenericTeamId` (`/Game/FloorCharDecal/BP_HitTelegraphActor.TeamId` NewTelegraph)))
  (bind _returnvalue (not (`self.CurrentTelegraphEnemy`)))
  (bind _output (`|GetArrayItem` _telegraphs_enemy))
  (bind _output_2 (`|GetArrayItem` _telegraphs_ally))
  (bind _teamid_teamid_2 (break `GenericTeamId` (`/Game/Characters/CharacterBlueprints/BP_2DGameCharacter.TeamId` (`self.Owner`))))
  (`|ExecutionSequence`
    (:`then_0`
      (`/Engine/EditorBlueprintResources/StandardMacros.IsValid` NewTelegraph
        (:`Is Valid`
          (if (== _teamid_teamid _teamid_teamid_2)
            (if (and _returnvalue (not (`self.CurrentTelegraphAlly`)))
              (set `self.CurrentTelegraphEnemy` false)
              (set `self.CurrentTelegraphAlly` true)
              (set `self.CurrentTelegraphColor` _currentcolortrigger))
            (elif _returnvalue
              (set `self.CurrentTelegraphEnemy` false)
              (set `self.CurrentTelegraphAlly` true)
              (set `self.CurrentTelegraphColor` _currentcolortrigger))))
        (:`Is Not Valid`
          (if (`KismetArrayLibrary.Array_IsNotEmpty` _telegraphs_enemy)
            (`/Engine/EditorBlueprintResources/StandardMacros.IsValid` _output
              (:`Is Valid`
                (set `self.CurrentTelegraphEnemy` true)
                (set `self.CurrentTelegraphAlly` false)
                (set `self.CurrentTelegraphColor` (`/Game/FloorCharDecal/BP_HitTelegraphActor.CurrentColorTrigger` _output)))
              (:`Is Not Valid`
                (set `self.CurrentTelegraphColor` (struct :`R` 1.0 :`G` 1.0 :`B` 1.0 :`A` 1.0) :!label _label)
                (set `self.CurrentTelegraphEnemy` false)
                (set `self.CurrentTelegraphAlly` false)))
            (elif (`KismetArrayLibrary.Array_IsNotEmpty` _telegraphs_ally)
              (`/Engine/EditorBlueprintResources/StandardMacros.IsValid` _output_2
                (:`Is Valid`
                  (set `self.CurrentTelegraphEnemy` false)
                  (set `self.CurrentTelegraphAlly` true)
                  (set `self.CurrentTelegraphColor` (`/Game/FloorCharDecal/BP_HitTelegraphActor.CurrentColorTrigger` _output_2)))
                (:`Is Not Valid`
                  (goto _label)))
              (else
                (goto _label)))))))
    (:`then_1`
      (`self.ChangeCurrentColor` (or (`self.CurrentTelegraphEnemy`) (`self.CurrentTelegraphAlly`)) (`self.CurrentTelegraphColor`)))))