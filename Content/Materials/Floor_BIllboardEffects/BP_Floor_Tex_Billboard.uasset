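; Floor effect billboard actor that turns a textured plane to face the player camera around the yaw axis.
; Each tick it compares the camera location to PrevCamLoc, which is never written in these graphs, and updates rotation when they differ.
; Within a set camera distance, TexPlane and Scene take the look-at yaw with a fixed pitch and zero roll.
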(event `self.ReceiveTick`
  (params (DeltaSeconds :type "Float (single-precision)"))
  (bind _update (`self.CheckIfUpdateRot`))
  (if _update
    (`self.UpdateRot`)))

(fn `CheckIfUpdateRot`
  (returns (Update :type Boolean))
  (bind _loc (`self.GetCamLoc`))
  (return (!= (`self.PrevCamLoc`) _loc :`ErrorTolerance` 0.1)))

(fn `GetCamLoc`
  (returns (Loc :type "Vector Structure"))
  (return (`PlayerCameraManager.GetCameraLocation` (`GameplayStatics.GetPlayerCameraManager` 0))))

(fn `UpdateRot`
  (bind _texplane (`self.TexPlane`))
  (bind _returnvalue (`SceneComponent.K2_GetComponentLocation` _texplane))
  (bind _returnvalue_2 (`PlayerCameraManager.GetCameraLocation` (`GameplayStatics.GetPlayerCameraManager` 0)))
  (bind (_returnvalue_roll _returnvalue_pitch _returnvalue_yaw) (`KismetMathLibrary.BreakRotator` (`KismetMathLibrary.FindLookAtRotation` _returnvalue _returnvalue_2)))
  (if (< (`KismetMathLibrary.Vector_Distance` _returnvalue _returnvalue_2) 6500.0)
    (`SceneComponent.K2_SetWorldRotation` _texplane (`KismetMathLibrary.MakeRotator` 0.0 135.0 _returnvalue_yaw) false false)
    (`SceneComponent.K2_SetWorldRotation` (`self.Scene`) (`KismetMathLibrary.MakeRotator` 0.0 135.0 _returnvalue_yaw) false false)))

(fn `UserConstructionScript`)