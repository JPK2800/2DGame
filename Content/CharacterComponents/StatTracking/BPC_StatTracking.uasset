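; Actor component that tracks health and mana for 2D game characters and breakable objects, including timed mana regeneration.
; Character projectile overlaps pass a team check into TakeContact, which resolves dodges, damage, healing, damage-over-time and poise stun.
; Server events relay results by multicast to dispatchers, which drive floating numbers and optional owner destruction on defeat.
; Hits also return name-encoded on-hit effects, such as mana gain, to the attacker's component.
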(event `self.ReceiveBeginPlay`
  (bind _returnvalue (`self.GetOwner`))
  (bind _healthbase (`self.HealthBase`))
  (bind _manabase (`self.ManaBase`))
  (set `self.HealthMaxCurrent` _healthbase)
  (set `self.HealthCurrent` _healthbase)
  (set `self.ManaMaxCurrent` _manabase)
  (set `self.ManaCurrent` _manabase)
  (bind _asbp_2dgame_character (cast `/Game/Characters/CharacterBlueprints/BP_2DGameCharacter` _returnvalue)
    (:`then`
      (`|ExecutionSequence`
        (:`then_0`
          (`self.ServerSetOwnerCharacter` _asbp_2dgame_character)
          (add `PrimitiveComponent.OnComponentBeginOverlap` (`Character.CapsuleComponent` _asbp_2dgame_character) (delegate `OnBeginOverlap`)))
        (:`then_1`
          (add `self.OnTakeHit` (delegate `OnTakeHitDamageNumber`) :!label _label)
          (add `self.OnTakeHeal` (delegate `OnTakeHealHealingNumber`))
          (add `self.OnTakeDodge` (delegate `OnDodge`))
          (add `self.OnDefeatingHit` (delegate `OnTakeDefeatingHit`))
          (add `self.OnTakeDefeatingFall` (delegate `OnTakeDefeatingFallHit`))
          (bind _returnvalue_2 (`KismetSystemLibrary.K2_SetTimer` null "GainManaFiveSec" 1.0 true))
          (set `self.ManaRegenTimer` _returnvalue_2))))
    (:`CastFailed`
      (bind _asbp_breakable_3d (cast `/Game/Blueprints/Breakable3D/BP_Breakable3D` _returnvalue))
      (set `self.OwnerObject` _asbp_breakable_3d)
      (add `PrimitiveComponent.OnComponentBeginOverlap` (`/Game/Blueprints/Breakable3D/BP_Breakable3D.StaticMesh` _asbp_breakable_3d) (delegate `OnBeginOverlap`))
      (goto _label))))

(event `OnTakeHitDamageNumber` :!signature `self.OnTakeHit`
  (params (Damage :type "Float (double-precision)") (DotTick :type Boolean) (Attacker :type "/Game/Characters/CharacterBlueprints/BP_2DGameCharacter Object Reference") (DmgNumColor :type "LinearColor Structure") (OnHitEffects :type "Array of Name (by ref)") (PoiseDamage :type "Float (double-precision)"))
  (`self.SpawnDamageNumber` Damage DotTick Attacker DmgNumColor)
  (`self.PerformOnHitEventsForAttacker` OnHitEffects Attacker))

(event `OnTakeHealHealingNumber` :!signature `self.OnTakeHeal`
  (params (Heal :type "Float (double-precision)") (HotTick :type Boolean) (Healer :type "/Game/Characters/CharacterBlueprints/BP_2DGameCharacter Object Reference") (DmgNumColor :type "LinearColor Structure"))
  (`self.SpawnHealNumber` Heal HotTick Healer DmgNumColor))

(event `OnDodge`
  (`self.SpawnDodgeText`))

(event `OnTakeDefeatingHit` :!signature `self.OnDefeatingHit`
  (params (ChangeDefeatAnim :type Name))
  (`self.CheckDestroyOwnerOnDefeat`))

(event `OnTakeDefeatingFallHit`
  (`self.CheckDestroyOwnerOnDefeat`))

(event `OnBeginOverlap`
  (params (OverlappedComponent :type "PrimitiveComponent Object Reference") (OtherActor :type "Actor Object Reference") (OtherComp :type "PrimitiveComponent Object Reference") (OtherBodyIndex :type Integer) (bFromSweep :type Boolean) (SweepResult :type "HitResult Structure (by ref)"))
  (bind _ownercharacter (`self.OwnerCharacter`))
  (bind _asbp_projectile (cast `/Game/ProjectilesAndSlashes/BP_Projectile` OtherActor))
  (`/Engine/EditorBlueprintResources/StandardMacros.IsValid` _ownercharacter
    (:`Is Valid`
      (bind _projectiledata (`/Game/ProjectilesAndSlashes/BP_Projectile.ProjectileData` _asbp_projectile))
      (if (!= (`.TeamID` (break `GenericTeamId` (`/Game/Characters/CharacterBlueprints/BP_2DGameCharacter.TeamId` _ownercharacter))) (`.TeamID` (break `GenericTeamId` (`.OriginTeamId_32_58FA1B63464A4B986646449B52B75D45` (break `/Game/ProjectilesAndSlashes/Struct_ProjectileDamageData` _projectiledata)))))
        (bind _asbp_2dgame_character (cast `/Game/Characters/CharacterBlueprints/BP_2DGameCharacter` (`Actor.GetOwner` _asbp_projectile)))
        (`self.TakeContact` _projectiledata _asbp_2dgame_character _asbp_projectile "None" (`|MakeArray` "None" :!type "Name"))))))

(event `ServerSignalOnDefeatingHit`
  (params (ChangeDefeatAnim :type Name))
  (`self.OnDefeatingHit` ChangeDefeatAnim)
  (`self.MulticastSignalOnDefeatingHit` ChangeDefeatAnim))

(event `MulticastSignalOnDefeatingHit`
  (params (ChangeDefeatAnim :type Name))
  (`/Engine/EditorBlueprintResources/ActorComponentMacros.Switch Has Authority`
    (:`Remote`
      (`self.OnDefeatingHit` ChangeDefeatAnim))))

(event `ServerSignalOnFullHealth`
  (`self.OnFullHealth`)
  (`self.MulticastSignalOnFullHealth`))

(event `MulticastSignalOnFullHealth`
  (`/Engine/EditorBlueprintResources/ActorComponentMacros.Switch Has Authority`
    (:`Remote`
      (`self.OnFullHealth`))))

(event `ServerSignalOnTakeHit`
  (params (Damage :type "Float (double-precision)") (DotTick :type Boolean) (Attacker :type "/Game/Characters/CharacterBlueprints/BP_2DGameCharacter Object Reference") (DmgNumColor :type "LinearColor Structure") (OnHitEffects :type "Array of Name") (PoiseDamage :type "Float (double-precision)"))
  (`self.OnTakeHit` Damage DotTick Attacker DmgNumColor OnHitEffects PoiseDamage)
  (`self.MulticastSignalOnTakeHit` Damage DotTick Attacker DmgNumColor OnHitEffects PoiseDamage))

(event `MulticastSignalOnTakeHit`
  (params (Damage :type "Float (double-precision)") (DotTIck :type Boolean) (Attacker :type "/Game/Characters/CharacterBlueprints/BP_2DGameCharacter Object Reference") (DmgNumColor :type "LinearColor Structure") (OnHitEffects :type "Array of Name") (PoiseDamage :type "Float (double-precision)"))
  (`/Engine/EditorBlueprintResources/ActorComponentMacros.Switch Has Authority`
    (:`Remote`
      (`self.OnTakeHit` Damage DotTIck Attacker DmgNumColor OnHitEffects PoiseDamage))))

(event `ServerSignalOnTakeHeal`
  (params (Heal :type "Float (double-precision)") (HotTick :type Boolean) (Healer :type "/Game/Characters/CharacterBlueprints/BP_2DGameCharacter Object Reference") (DmgNumColor :type "LinearColor Structure"))
  (`self.OnTakeHeal` Heal HotTick Healer DmgNumColor)
  (`self.MulticastSignalOnTakeHeal` Heal HotTick Healer DmgNumColor))

(event `MulticastSignalOnTakeHeal`
  (params (Heal :type "Float (double-precision)") (HotTick :type Boolean) (Healer :type "/Game/Characters/CharacterBlueprints/BP_2DGameCharacter Object Reference") (DmgNumColor :type "LinearColor Structure"))
  (`/Engine/EditorBlueprintResources/ActorComponentMacros.Switch Has Authority`
    (:`Remote`
      (`self.OnTakeHeal` Heal HotTick Healer DmgNumColor))))

(event `ServerSignalOnTakeDodge`
  (`self.OnTakeDodge`)
  (`self.MulticastSignalOnTakeDodge`))

(event `MulticastSignalOnTakeDodge`
  (`/Engine/EditorBlueprintResources/ActorComponentMacros.Switch Has Authority`
    (:`Remote`
      (`self.OnTakeDodge`))))

(event `ServerSignalOnTakeDefeatingFall`
  (`self.OnTakeDefeatingFall`)
  (`self.MulticastSignalOnTakeDefeatingFall`))

(event `MulticastSignalOnTakeDefeatingFall`
  (`/Engine/EditorBlueprintResources/ActorComponentMacros.Switch Has Authority`
    (:`Remote`
      (`self.OnTakeDefeatingFall`))))

(event `ServerSignalOnHealthUpdate`
  (params (HP :type Integer))
  (`self.OnHealthUpdate` HP)
  (`self.MulticastSignalOnHealthUpdate` HP))

(event `MulticastSignalOnHealthUpdate`
  (params (HP :type Integer))
  (`/Engine/EditorBlueprintResources/ActorComponentMacros.Switch Has Authority`
    (:`Remote`
      (`self.OnHealthUpdate` HP))))

(event `ServerSetOwnerCharacter`
  (params (Character :type "/Game/Characters/CharacterBlueprints/BP_2DGameCharacter Object Reference"))
  (set `self.OwnerCharacter` Character))

(event `ServerTriggerHitEvents`
  (params (Events :type "Array of Name"))
  (for _array_element Events
    (`self.HandleOnHitEvent` _array_element))
  (`self.MulticastTriggerHitEvents` Events))

(event `MulticastTriggerHitEvents`
  (params (Events :type "Array of Name"))
  (for _array_element Events
    (`self.HandleOnHitEvent` _array_element)))

(event `ServerPoiseHitStun`
  (`self.MulticastPoiseHitStun`)
  (`self.OnTakeHitStun`))

(event `MulticastPoiseHitStun`
  (`self.OnTakeHitStun`))

(fn `BeginDamageDot`
  (params (Data :type "/Game/ProjectilesAndSlashes/Struct_ProjectileDamageData Structure") (Attacker :type "/Game/Characters/CharacterBlueprints/BP_2DGameCharacter Object Reference") (DmgNumColor :type "LinearColor Structure"))
  (bind _ownercharacter (`self.OwnerCharacter`))
  (`/Engine/EditorBlueprintResources/StandardMacros.IsValid` _ownercharacter
    (:`Is Valid`
      (`|AddComponentByClass` _ownercharacter "/Game/CharacterComponents/StatTracking/BP_DotObject.BP_DotObject_C" Data_DamagePerTick_11_D680DDE24146E1A65A3E71A3926CA67E Data_TimeBetweenDotTicks_18_7322B4FB4D86989F21BA1FA92788F896 Data_DotDuration_16_C75169C14BC551769E48DE91C9A2E120 _ownercharacter Attacker DmgNumColor))))

(fn `CheckDestroyOwnerOnDefeat`
  (bind _ownercharacter (`self.OwnerCharacter`))
  (bind _ownerobject (`self.OwnerObject`))
  (if (`self.DestroyOwnerOnDefeat`)
    (if (`KismetSystemLibrary.IsValid` _ownercharacter)
      (`/Game/Characters/CharacterBlueprints/BP_2DGameCharacter.OwnerDestroyActor` _ownercharacter)
      (elif (`KismetSystemLibrary.IsValid` _ownerobject)
        (`/Game/Blueprints/Breakable3D/BP_Breakable3D.ServerDestroyActor` _ownerobject)))))

(fn `GainManaFiveSec`
  (`self.UpdateMana` (`self.ManaRegenPerSecBase`)))

(fn `GetBaseHP`
  (returns (BaseHealth :type "Float (double-precision)"))
  (return (`self.HealthBase`)))

(fn `GetBaseMP`
  (returns (BaseHealth :type "Float (double-precision)"))
  (return (`self.ManaBase`)))

(fn `GetCurrentHP`
  (returns (Health :type "Float (double-precision)"))
  (return (`self.HealthCurrent`)))

(fn `GetCurrentMaxHP`
  (returns (MaxHealth :type "Float (double-precision)"))
  (return (`self.HealthMaxCurrent`)))

(fn `GetCurrentMaxMP`
  (returns (CurrentMP :type "Float (double-precision)"))
  (return (`self.ManaMaxCurrent`)))

(fn `GetCurrentMP`
  (returns (CurrentMP :type "Float (double-precision)"))
  (return (`self.ManaCurrent`)))

(fn `HandleOnHitEvent`
  (params (Event :type Name))
  (locals (EventName :type String))
  (bind _returnvalue (`KismetStringLibrary.Conv_NameToString` Event))
  (bind (_lefts _rights _returnvalue_2) (`KismetStringLibrary.Split` _returnvalue "|"))
  (if (`Pawn.IsLocallyControlled` (`self.OwnerCharacter`))
    (if _returnvalue_2
      (set `local.EventName` _lefts)
      (else
        (set `local.EventName` _returnvalue)))
    (switch `string` (`local.EventName`)
      (:`ManaGain`
        (`self.UpdateMana` (`KismetStringLibrary.Conv_StringToDouble` _rights))))))

(fn `PerformOnHitEventsForAttacker`
  (params (OnHitEffects :type "Array of Name") (Attacker :type "/Game/Characters/CharacterBlueprints/BP_2DGameCharacter Object Reference"))
  (`/Engine/EditorBlueprintResources/StandardMacros.IsValid` Attacker
    (:`Is Valid`
      (if (`Pawn.IsLocallyControlled` Attacker)
        (`self.ServerTriggerHitEvents` (`/Game/Characters/CharacterBlueprints/BP_2DGameCharacter.BPC_StatTracking` Attacker) OnHitEffects)))))

(fn `ReceiveFallDefeat`
  (bind _ownercharacter (`self.OwnerCharacter`))
  (bind _springarm (`/Game/Characters/CharacterBlueprints/BP_2DGameCharacter.SpringArm` _ownercharacter))
  (bind (_returnvalue_roll _returnvalue_pitch _returnvalue_yaw) (`KismetMathLibrary.BreakRotator` (`SpringArmComponent.GetTargetRotation` _springarm)))
  (`self.OnTakeDefeatingFall`)
  (`/Game/Characters/CharacterBlueprints/BP_2DGameCharacter.ToggleGravityAndMovement` _ownercharacter true true true)
  (`SceneComponent.K2_SetWorldRotation` _springarm (`KismetMathLibrary.MakeRotator` _returnvalue_roll -89.0 _returnvalue_yaw) false false))

(fn `SetVulnerability`
  (params (Invulnerable :type Boolean))
  (set `self.DodgeInvulnerable` Invulnerable))

(fn `SpawnDamageNumber`
  (params (Amount :type "Float (double-precision)") (Dot :type Boolean) (Attacker :type "/Game/Characters/CharacterBlueprints/BP_2DGameCharacter Object Reference") (DmgNumColor :type "LinearColor Structure"))
  (bind _ownercharacter (`self.OwnerCharacter`))
  (bind _returnvalue (`Pawn.IsPlayerControlled` _ownercharacter))
  (bind _returnvalue_2 (`Actor.K2_GetActorLocation` (`self.OwnerObject`)))
  (bind _returnvalue_3 (`PlayerCameraManager.GetCameraLocation` (`GameplayStatics.GetPlayerCameraManager` 0)))
  (bind _returnvalue_4 (`Actor.K2_GetActorLocation` _ownercharacter))
  (bind _returnvalue_5 (and (`Pawn.IsLocallyControlled` _ownercharacter) _returnvalue))
  (if (`KismetSystemLibrary.IsValid` (`self.OwnerCharacter`))
    (bind _returnvalue_6 (`|SpawnActorFromClass` "/Game/DamageNumbers/BP_DamageNumberSpawn.BP_DamageNumberSpawn_C" (`KismetMathLibrary.MakeTransform` _returnvalue_4 (`KismetMathLibrary.FindLookAtRotation` (`PlayerCameraManager.GetCameraLocation` (`GameplayStatics.GetPlayerCameraManager` 0)) _returnvalue_4)) "Undefined" "MultiplyWithRoot" _ownercharacter DmgNumColor Attacker))
    (`/Game/DamageNumbers/BP_DamageNumberSpawn.InitWidget` _returnvalue_6 false false _returnvalue_5 _returnvalue false (`KismetMathLibrary.Conv_IntToDouble` (`KismetMathLibrary.Round` Amount)) (or _returnvalue_5 (and (`Pawn.IsLocallyControlled` Attacker) (`Pawn.IsPlayerControlled` Attacker))))
    (else
      (`/Engine/EditorBlueprintResources/StandardMacros.IsValid` (`self.OwnerObject`)
        (:`Is Valid`
          (bind _returnvalue_7 (`|SpawnActorFromClass` "/Game/DamageNumbers/BP_DamageNumberSpawn.BP_DamageNumberSpawn_C" (`KismetMathLibrary.MakeTransform` (/ (+ _returnvalue_2 _returnvalue_3) 2.0) (`KismetMathLibrary.FindLookAtRotation` _returnvalue_3 _returnvalue_2)) "Undefined" "MultiplyWithRoot" null DmgNumColor null))
          (`/Game/DamageNumbers/BP_DamageNumberSpawn.InitWidget` _returnvalue_7 false false false true false (`KismetMathLibrary.Conv_IntToDouble` (`KismetMathLibrary.Round` Amount)) false))))))

(fn `SpawnDodgeText`
  (bind _ownercharacter (`self.OwnerCharacter`))
  (bind _returnvalue (`Actor.K2_GetActorLocation` _ownercharacter))
  (bind _returnvalue_2 (`|SpawnActorFromClass` "/Game/DamageNumbers/BP_DamageNumberSpawn.BP_DamageNumberSpawn_C" (`KismetMathLibrary.MakeTransform` _returnvalue (`KismetMathLibrary.FindLookAtRotation` (`PlayerCameraManager.GetCameraLocation` (`GameplayStatics.GetPlayerCameraManager` 0)) _returnvalue)) "Undefined" "MultiplyWithRoot" _ownercharacter (struct :`R` 1.0 :`G` 1.0 :`B` 1.0 :`A` 1.0) null))
  (`/Game/DamageNumbers/BP_DamageNumberSpawn.InitWidget` _returnvalue_2 true false false false false 0.0 (and (`Pawn.IsLocallyControlled` _ownercharacter) (`Pawn.IsPlayerControlled` _ownercharacter))))

(fn `SpawnHealNumber`
  (params (Amount :type "Float (double-precision)") (Hot :type Boolean) (Healer :type "/Game/Characters/CharacterBlueprints/BP_2DGameCharacter Object Reference") (DmgNumColor :type "LinearColor Structure"))
  (bind _returnvalue (`self.GetOwner`))
  (bind _ownercharacter (`self.OwnerCharacter`))
  (bind _returnvalue_2 (`|SpawnActorFromClass` "/Game/DamageNumbers/BP_DamageNumberSpawn.BP_DamageNumberSpawn_C" (`KismetMathLibrary.MakeTransform` (`Actor.K2_GetActorLocation` _returnvalue)) "Undefined" "MultiplyWithRoot" _returnvalue DmgNumColor null))
  (`/Game/DamageNumbers/BP_DamageNumberSpawn.InitWidget` _returnvalue_2 false false false false true Amount (or (and (`Pawn.IsLocallyControlled` _ownercharacter) (`Pawn.IsPlayerControlled` _ownercharacter)) (and (`Pawn.IsLocallyControlled` Healer) (`Pawn.IsPlayerControlled` Healer)))))

(fn `TakeContact`
  (params (Data :type "/Game/ProjectilesAndSlashes/Struct_ProjectileDamageData Structure") (Attacker :type "/Game/Characters/CharacterBlueprints/BP_2DGameCharacter Object Reference") (Projectile :type "/Game/ProjectilesAndSlashes/BP_Projectile Object Reference") (ChangeDefeatAnim :type Name) (OnHitEffects :type "Array of Name"))
  (returns (MadeHit :type Boolean))
  (locals (WasTargetHit :type Boolean))
  (bind (_dealsdamage _immediatedamage _dealsdamageinticks _damagepertick _timebetweendotticks _dotduration _originteamid _dmgnumbercolor _poisedamage) (break `/Game/ProjectilesAndSlashes/Struct_ProjectileDamageData` Data))
  (bind _returnvalue (`KismetMathLibrary.Conv_IntToDouble` _immediatedamage))
  (if (`self.DodgeInvulnerable`)
    (`self.TakeDodge`)
    (set `local.WasTargetHit` false)
    (else
      (`|ExecutionSequence`
        (:`then_0`
          (if _dealsdamage
            (if (>= _returnvalue 0.0)
              (`self.TakeDamage` _returnvalue Attacker false ChangeDefeatAnim _dmgnumbercolor OnHitEffects (`KismetMathLibrary.Conv_IntToDouble` _poisedamage))
              (else
                (`self.TakeHealing` _returnvalue Attacker false _dmgnumbercolor))))
          (set `local.WasTargetHit` true))
        (:`then_1`
          (if _dealsdamageinticks
            (`self.BeginDamageDot` Data Attacker _dmgnumbercolor)
            (set `local.WasTargetHit` true)))
        (:`then_2`
          (return (`local.WasTargetHit`)))))))

(fn `TakeDamage`
  (params (Damage :type "Float (double-precision)") (Attacker :type "/Game/Characters/CharacterBlueprints/BP_2DGameCharacter Object Reference") (Dot :type Boolean) (ChangeDefeatAnim :type Name) (DmgNumColor :type "LinearColor Structure") (OnHitEffects :type "Array of Name") (PoiseDamage :type "Float (double-precision)"))
  (if (`self.Invulnerable`)
    (`self.ServerSignalOnTakeHit` Damage Dot Attacker DmgNumColor OnHitEffects)
    (elif (not (<= (`self.HealthCurrent`) 0.0))
      (bind _output_get (set `self.HealthCurrent` (`KismetMathLibrary.FClamp` (- (`self.HealthCurrent`) Damage) 0.0 (`self.HealthMaxCurrent`))))
      (`self.ServerSignalOnTakeHit` Damage Dot Attacker DmgNumColor OnHitEffects)
      (`self.ServerSignalOnHealthUpdate` (`KismetMathLibrary.FTrunc` _output_get))
      (if (<= _output_get 0.0)
        (`self.ServerSignalOnDefeatingHit` ChangeDefeatAnim)
        (elif (> PoiseDamage (`self.Poise`))
          (`self.ServerPoiseHitStun`))))))

(fn `TakeDodge`
  (`self.ServerSignalOnTakeDodge`))

(fn `TakeHealing`
  (params (Heal :type "Float (double-precision)") (Attacker :type "/Game/Characters/CharacterBlueprints/BP_2DGameCharacter Object Reference") (Hot :type Boolean) (DmgNumColor :type "LinearColor Structure"))
  (if (not (== (`self.HealthCurrent`) (`self.HealthMaxCurrent`)))
    (bind _output_get (set `self.HealthCurrent` (`KismetMathLibrary.FClamp` (+ (`self.HealthCurrent`) Heal) 0.0 (`self.HealthMaxCurrent`))))
    (`self.ServerSignalOnTakeHeal` Heal Hot Attacker DmgNumColor)
    (`self.ServerSignalOnHealthUpdate` (`KismetMathLibrary.FTrunc` _output_get))
    (if (>= _output_get (`self.HealthMaxCurrent`))
      (`self.ServerSignalOnFullHealth`))))

(fn `UpdateMana`
  (params (Mana :type "Float (double-precision)"))
  (bind _output_get (set `self.ManaCurrent` (`KismetMathLibrary.FClamp` (+ (`self.ManaCurrent`) Mana) 0.0 (`self.ManaMaxCurrent`))))
  (`self.OnManaUpdate` (`KismetMathLibrary.FFloor` _output_get)))

(fn `UpdateMaxHP`
  (params (NewHealthMax :type "Float (double-precision)"))
  (bind _output_get (set `self.HealthMaxCurrent` NewHealthMax))
  (`self.OnMaxHealthUpdate` (`KismetMathLibrary.FTrunc` _output_get)))

(fn `UpdateMaxMP`
  (params (NewManaMax :type "Float (double-precision)"))
  (bind _output_get (set `self.ManaMaxCurrent` NewManaMax))
  (`self.OnMaxManaUpdate` (`KismetMathLibrary.FTrunc` _output_get)))