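; Actor component that switches the billboard limbs of a BP_SimpleBillboardActor between idle and moving data.
; On BeginPlay it binds to the owner's start and stop movement events and caches its BPC_BillboardLimb components.
; Each event records the current movement state and pushes MovingData or IdleData to every cached limb through UpdateData, starting in idle.
; It is event-driven, with no Tick logic.
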(event `self.ReceiveBeginPlay`
  (bind _asbp_simple_billboard_actor (cast `/Game/Objects/BP_SimpleBillboardActor` (`self.GetOwner`)))
  (add `/Game/Objects/BP_SimpleBillboardActor.StartMovement` _asbp_simple_billboard_actor (delegate `BeginSetMoving`))
  (add `/Game/Objects/BP_SimpleBillboardActor.StopMovement` _asbp_simple_billboard_actor (delegate `BeginSetIdle`))
  (set `self.RelevantBillboards` (`Actor.K2_GetComponentsByClass` _asbp_simple_billboard_actor "/Game/CharacterComponents/Billboard_Limbs/BPC_BillboardLimb.BPC_BillboardLimb_C"))
  (`self.SetIdle`))

(event `BeginSetMoving`
  (`self.SetMoving`))

(event `BeginSetIdle`
  (`self.SetIdle`))

(fn `SetIdle`
  (set `self.CurrentMovementState` "Idle")
  (for _array_element (`self.RelevantBillboards`)
    (`/Game/CharacterComponents/Billboard_Limbs/BPC_BillboardLimb.UpdateData` _array_element (`self.IdleData`))))

(fn `SetMoving`
  (set `self.CurrentMovementState` "Moving")
  (for _array_element (`self.RelevantBillboards`)
    (`/Game/CharacterComponents/Billboard_Limbs/BPC_BillboardLimb.UpdateData` _array_element (`self.MovingData`))))