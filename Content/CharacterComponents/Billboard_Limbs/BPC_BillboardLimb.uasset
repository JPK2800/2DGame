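; Billboard component for a character limb that shows an animated directional sprite facing the player camera.
; Each tick it rotates toward the camera, then buckets the owner-to-camera yaw into five angles, optionally skipping diagonals or using one side.
; Angle changes swap texture and frame count on a dynamic flipbook material; XFlip is computed but both branches use identical textures.
; UpdateData loads new frame sets and settings, while helper functions reset or resync playback time.
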(event `self.ReceiveBeginPlay`
  (`self.InitDynamicMat`))

(event `self.ReceiveTick`
  (params (DeltaSeconds :type "Float (single-precision)"))
  (`self.OrientLimbStep` DeltaSeconds)
  (`self.UpdateMaterialAngleStep` DeltaSeconds))

(fn `InitDynamicMat`
  (bind _returnvalue (`self.CreateDynamicMaterialInstance` 0 "/Game/Characters/Mat_CharacterFlipbookMaterial.Mat_CharacterFlipbookMaterial"))
  (bind _output_get (set `self.DynamicMaterial` _returnvalue))
  (`self.SetMaterial` 0 _output_get))

(fn `OrientLimbStep`
  (params (DeltaTime :type "Float (double-precision)"))
  (bind _returnvalue (`self.GetOwner`))
  (bind _returnvalue_2 (`KismetMathLibrary.FindLookAtRotation` (`PlayerCameraManager.GetCameraLocation` (`self.CameraManager`)) (`Actor.K2_GetActorLocation` _returnvalue)))
  (`/Engine/EditorBlueprintResources/StandardMacros.IsValid` _returnvalue
    (:`Is Valid`
      (if (`self.OrientToCamera`)
        (`/Engine/EditorBlueprintResources/StandardMacros.IsValid` (`self.CameraManager`)
          (:`Is Valid`
            _)
          (:`Is Not Valid`
            (set `self.CameraManager` (`GameplayStatics.GetPlayerCameraManager` 0))))
        (if (`self.OrientUseZAxis`)
          (`self.K2_SetWorldRotation` (`KismetMathLibrary.MakeRotator` (+ (.roll _returnvalue_2) 180.0) (+ (* (.pitch _returnvalue_2) 1.0) -90.0) (.yaw _returnvalue_2)))
          (else
            (`self.K2_SetWorldRotation` (`KismetMathLibrary.MakeRotator` (+ (.roll _returnvalue_2) 90.0) -90.0 (+ (.yaw _returnvalue_2) 90.0)))))))))

(fn `ResyncFlipbooks`
  (`MaterialInstanceDynamic.SetScalarParameterValue` (`self.DynamicMaterial`) "ResetTime" 0.0))

(fn `StartFlipbookFromStart`
  (`MaterialInstanceDynamic.SetScalarParameterValue` (`self.DynamicMaterial`) "ResetTime" (`KismetSystemLibrary.GetGameTimeInSeconds`)))

(fn `UpdateData`
  (params (Data :type "/Game/CharacterComponents/Billboard_Limbs/Struct_BillboardData Structure"))
  (`|ExecutionSequence`
    (:`then_0`
      (set `self.0_Frames` Data_0_Frames_38_028B00B844E292C899EAA3A562E33BC7)
      (set `self.45_Frames` Data_45_Frames_39_D43F149A41B15205A3BD69BFAC2626BD)
      (set `self.90_Frames` Data_90_Frames_40_2C10A25D46B000AF50AF9380333B5691)
      (set `self.135_Frames` Data_135_Frames_41_EAE025994E0F982539F0B0B0258B70D2)
      (set `self.180_Frames` Data_180_Frames_42_4361621A4E3E796D0B313991F5BE7024))
    (:`then_1`
      (set `self.-45_Frames` `Data_-45_Frames_43_47607E2C4583212D3429C5BEBF9CFF3E`)
      (set `self.-90_Frames` `Data_-90_Frames_44_13FD55394E6D04DD40DFF4A9236FF428`)
      (set `self.-135_Frames` `Data_-135_Frames_45_A081635E41B6D7F80F483CA85319E615`)
      (set `self.FlipSideSprites` false)
      (set `self.OrientToCamera` Data_OrientToCam_26_E6EC66584897E752B1333CB8CEA23B08)
      (set `self.OrientUseZAxis` Data_UseZ_28_B9A6E912426A7685F0A97BA2E089B545)
      (bind _output_get (set `self.PlayRate` Data_PlayRate_31_5653BD6F41767AC25D56449EE85EFC95))
      (set `self.SkipDiagnonals` Data_SkipDiags_35_E3CFCE73445F8EC35DC49DA96E907E5E)
      (set `self.OnlyOneSide` Data_OneSide_37_DFB7FADD4B2856697C8D78A3DF659838)
      (`MaterialInstanceDynamic.SetScalarParameterValue` (`self.DynamicMaterial`) "Rate" _output_get))
    (:`then_2`
      (set `self.0_Frames_Count` Data_0_FrameCount_48_CD2FDB674457081ACEFA1C847D6FC37B)
      (set `self.45_Frames_Count` Data_45_FrameCount_50_05D3290D4D986843E00CAD8E41469130)
      (set `self.90_Frames_Count` Data_90_FrameCount_52_D799231E4E5643179E3F26964C6D5632)
      (set `self.135_Frames_Count` Data_135_FrameCount_54_16ADA28942B289FE5AAF1BB4C8DA19C3)
      (set `self.180_Frames_Count` Data_180_FrameCount_56_8E6AAB3E41382556FA0CEA803239B34E))
    (:`then_3`
      (set `self.CurrentAngle` -1)
      (`self.UpdateMaterialAngleStep` (`GameplayStatics.GetWorldDeltaSeconds`)))))

(fn `UpdateMatByAngle`
  (params (NewAngle :type Integer) (Textures :type "Texture2D Object Reference") (FramesCount :type Integer))
  (`|ExecutionSequence`
    (:`then_0`
      (`MaterialInstanceDynamic.SetScalarParameterValue` (`self.DynamicMaterial`) "TexCount" (`KismetMathLibrary.Conv_IntToDouble` FramesCount)))
    (:`then_1`
      (set `self.CurrentAngle` NewAngle)
      (`MaterialInstanceDynamic.SetTextureParameterValue` (`self.DynamicMaterial`) "TexParam" Textures))))

(fn `UpdateMaterialAngleStep`
  (params (DeltaTime :type "Float (double-precision)"))
  (locals (ResultAngle :type "Float (double-precision)" :default 0.0) (XFlip :type Boolean))
  (bind _returnvalue (`self.GetOwner`))
  (bind _45_frames_count (`self.45_Frames_Count`))
  (bind _90_frames_count (`self.90_Frames_Count`))
  (bind _135_frames_count (`self.135_Frames_Count`))
  (bind _resultangle (`local.ResultAngle`))
  (bind _skipdiagnonals (`self.SkipDiagnonals`))
  (bind _skipdiagnonals_2 (`self.SkipDiagnonals`))
  (bind _resultangle_2 (`local.ResultAngle`))
  (bind _yaw (.yaw (`KismetMathLibrary.NormalizedDeltaRotator` (`KismetMathLibrary.FindLookAtRotation` (`PlayerCameraManager.GetCameraLocation` (`self.CameraManager`)) (`Actor.K2_GetActorLocation` _returnvalue)) (`Actor.K2_GetActorRotation` _returnvalue))))
  (bind _returnvalue_2 (`KismetMathLibrary.Abs` _yaw))
  (`/Engine/EditorBlueprintResources/StandardMacros.IsValid` (`self.GetOwner`)
    (:`Is Valid`
      (if (`self.OrientToCamera`)
        (`/Engine/EditorBlueprintResources/StandardMacros.IsValid` (`self.CameraManager`)
          (:`Is Valid`
            _)
          (:`Is Not Valid`
            (set `self.CameraManager` (`GameplayStatics.GetPlayerCameraManager` 0))))
        (if (`self.OnlyOneSide`)
          (if (not (== (`self.CurrentAngle`) 180)) :!label _label
            (`self.UpdateMatByAngle` 180 (`self.0_Frames`) (`self.0_Frames_Count`)))
          (else
            (if (or (or (and (<= _returnvalue_2 22.5) (not (`self.SkipDiagnonals`))) (and (< _returnvalue_2 44.0) (`self.SkipDiagnonals`))) (or (and (> _returnvalue_2 157.5) (not (`self.SkipDiagnonals`))) (and (> _returnvalue_2 136.0) (`self.SkipDiagnonals`))))
              (set `local.XFlip` false)
              (else
                (set `local.XFlip` (xor (< (`KismetMathLibrary.SignOfFloat` _yaw) 0.0) (`self.FlipSideSprites`)))))
            (set `local.ResultAngle` (`KismetMathLibrary.Abs` _yaw))
            (if (or (and (> _resultangle_2 157.5) (not _skipdiagnonals_2)) (and (> _resultangle_2 136.0) _skipdiagnonals_2))
              (goto _label)
              (elif (and (> (`local.ResultAngle`) 112.0) (not (`self.SkipDiagnonals`)))
                (if (== (`self.CurrentAngle`) 135)
                  _
                  (elif (`local.XFlip`)
                    (`self.UpdateMatByAngle` 135 (`self.-45_Frames`) _45_frames_count)
                    (else
                      (`self.UpdateMatByAngle` 135 (`self.45_Frames`) _45_frames_count))))
                (elif (or (and (> _resultangle 44.0) _skipdiagnonals) (and (> _resultangle 67.5) (not _skipdiagnonals)))
                  (if (== (`self.CurrentAngle`) 90)
                    _
                    (elif (`local.XFlip`)
                      (`self.UpdateMatByAngle` 90 (`self.-90_Frames`) _90_frames_count)
                      (else
                        (`self.UpdateMatByAngle` 90 (`self.90_Frames`) _90_frames_count))))
                  (elif (and (> (`local.ResultAngle`) 22.5) (not (`self.SkipDiagnonals`)))
                    (if (== (`self.CurrentAngle`) 45)
                      _
                      (elif (`local.XFlip`)
                        (`self.UpdateMatByAngle` 45 (`self.-135_Frames`) _135_frames_count)
                        (else
                          (`self.UpdateMatByAngle` 45 (`self.135_Frames`) _135_frames_count))))
                    (elif (not (== (`self.CurrentAngle`) 0))
                      (`self.UpdateMatByAngle` 0 (`self.180_Frames`) (`self.180_Frames_Count`)))))))))))))