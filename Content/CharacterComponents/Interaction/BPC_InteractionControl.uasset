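; BPC_InteractionControl is a component that tracks interactable actors and triggers player interaction with them.
; AddInteractable and RemoveInteractable maintain the Interactables list, adding entries uniquely.
; TriggerInteract passes the list to the ServerTriggerInteract event, which calls ServerPlayerInteracted on every entry, so all listed interactables respond at once.
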(event `ServerTriggerInteract`
  (params (Interactables :type "Array of /Game/Interactables/BP_InteractableActor Object Reference"))
  (for _array_element Interactables
    (`/Game/Interactables/BP_InteractableActor.ServerPlayerInteracted` _array_element)))

(fn `AddInteractable`
  (params (Actor :type "/Game/Interactables/BP_InteractableActor Object Reference"))
  (`KismetArrayLibrary.Array_AddUnique` (`self.Interactables`) Actor))

(fn `RemoveInteractable`
  (params (Interactable :type "/Game/Interactables/BP_InteractableActor Object Reference"))
  (`KismetArrayLibrary.Array_RemoveItem` (`self.Interactables`) Interactable))

(fn `TriggerInteract`
  (`self.ServerTriggerInteract` (`self.Interactables`)))