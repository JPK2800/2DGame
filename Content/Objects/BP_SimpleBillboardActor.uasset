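; BP_SimpleBillboardActor is an actor that detects when it starts and stops moving.
; Every Tick, TrackMovementEventsStep compares the velocity magnitude against a small threshold and uses an IsMoving flag to catch transitions.
; It calls StartMovement or StopMovement once per change of state, with no response to either defined in this Blueprint.
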(event `self.ReceiveTick`
  (params (DeltaSeconds :type "Float (single-precision)"))
  (`self.TrackMovementEventsStep` DeltaSeconds))

(fn `TrackMovementEventsStep`
  (params (DeltaTime :type "Float (double-precision)"))
  (bind _returnvalue (`KismetMathLibrary.VSize` (`self.GetVelocity`)))
  (if (and (> _returnvalue 10.0) (not (`self.IsMoving`)))
    (set `self.IsMoving` true)
    (`self.StartMovement`)
    (elif (and (<= _returnvalue 10.0) (`self.IsMoving`))
      (set `self.IsMoving` false)
      (`self.StopMovement`))))

(fn `UserConstructionScript`)