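; Coin spawner actor that creates a batch of BP_Coin actors at its own location when play begins.
; A BeginPlay loop spawns coins until the CoinsSpawned counter reaches CoinsToSpawn, all at once with no delay.
; Each coin's X axis is aimed upward with a slight random tilt via MakeRotFromX, and the coin inherits the spawner's owner and instigator.
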(event `self.ReceiveBeginPlay`
  (bind _returnvalue_location (`KismetMathLibrary.BreakTransform` (`self.GetTransform`)))
  (`parent.ReceiveBeginPlay`)
  (while (< (`self.CoinsSpawned`) (`self.CoinsToSpawn`))
    (`|SpawnActorFromClass` "/Game/Objects/BP_Coin.BP_Coin_C" (`KismetMathLibrary.MakeTransform` _returnvalue_location (`KismetMathLibrary.MakeRotFromX` (`KismetMathLibrary.MakeVector` (`KismetMathLibrary.RandomFloatInRange` -10.0 10.0) (`KismetMathLibrary.RandomFloatInRange` -10.0 10.0) 90.0))) "Undefined" "MultiplyWithRoot" (`self.GetOwner`) (`self.GetInstigator`))
    (`/Engine/EditorBlueprintResources/StandardMacros.IncrementInt` (`self.CoinsSpawned`))))

(fn `UserConstructionScript`
  (`parent.UserConstructionScript`))