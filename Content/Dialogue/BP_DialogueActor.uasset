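; BP_DialogueActor plays a linear dialogue script on screen, one node at a time, then destroys itself.
; BeginPlay calls InitDialogue, an empty function here.
; StartScript registers the actor with BP_DialogueManager, creates a WBP_DialogueWidget showing the current node, and binds its ReadyForNextNode event.
; SetNextNode feeds successive DialogueScript entries to the widget, calling EndScript to remove widget and actor when none remain.
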(event `self.ReceiveBeginPlay`
  (`self.InitDialogue`))

(fn `EndScript`
  (`Widget.RemoveFromParent` (`self.DialogueWidget`))
  (`self.K2_DestroyActor`))

(fn `InitDialogue`)

(fn `SetNextNode`
  (bind _dialoguewidget (`self.DialogueWidget`))
  (bind _currentdialoguenode (`self.CurrentDialogueNode`))
  (bind _dialoguescript (`self.DialogueScript`))
  (`/Engine/EditorBlueprintResources/StandardMacros.IsValid` _dialoguewidget
    (:`Is Valid`
      (if (`KismetArrayLibrary.Array_IsValidIndex` _dialoguescript _currentdialoguenode)
        (`/Game/Dialogue/WBP_DialogueWidget.StartText` _dialoguewidget (`|GetArrayItem` _dialoguescript _currentdialoguenode))
        (`/Engine/EditorBlueprintResources/StandardMacros.IncrementInt` _currentdialoguenode)
        (else
          (`self.EndScript`))))))

(fn `StartScript`
  (bind _currentdialoguenode (`self.CurrentDialogueNode`))
  (`|ExecutionSequence`
    (:`then_0`
      (bind _returnvalue (`GameplayStatics.GetActorOfClass` "/Game/Dialogue/DialogueManager/BP_DialogueManager.BP_DialogueManager_C"))
      (`/Engine/EditorBlueprintResources/StandardMacros.IsValid` _returnvalue
        (:`Is Valid`
          (`/Game/Dialogue/DialogueManager/BP_DialogueManager.Start New Dialogue Actor` _returnvalue self))))
    (:`then_1`
      (bind _returnvalue_2 (`|CreateWidget` "/Game/Dialogue/WBP_DialogueWidget.WBP_DialogueWidget_C"))
      (set `self.DialogueWidget` _returnvalue_2)
      (`/Game/Dialogue/WBP_DialogueWidget.StartText` _returnvalue_2 (`|GetArrayItem` (`self.DialogueScript`) _currentdialoguenode))
      (`/Engine/EditorBlueprintResources/StandardMacros.IncrementInt` _currentdialoguenode
        (:`  `
          (add `/Game/Dialogue/WBP_DialogueWidget.ReadyForNextNode` _returnvalue_2 (`|CreateDelegate` :!event `SetNextNode`))
          (`UserWidget.AddToPlayerScreen` _returnvalue_2 0))))))

(fn `UserConstructionScript`)