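; Character component that runs data-driven basic attack and dodge actions for a BP_2DGameCharacter.
; The owning client triggers actions immediately, relaying them through server and multicast events to non-local copies.
; Each action plays on tag-matched billboard components and queues timed events, checked on Tick, for projectiles, telegraphs, movement, invulnerability and incap collision.
; A timer based on frame count and play rate ends the action and resets character state.
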(event `self.ReceiveTick`
  (params (DeltaSeconds :type "Float (single-precision)"))
  (`self.Action Event Check Step` DeltaSeconds))

(event `ServerTriggerBasicAttack`
  (params (InputRotation :type "Rotator Structure"))
  (`self.MulticastTriggerBasicAttack` InputRotation))

(event `MulticastTriggerBasicAttack`
  (params (InputRotation :type "Rotator Structure"))
  (bind _ascharacter (cast `Character` (`self.GetOwner`)))
  (if (not (`Pawn.IsLocallyControlled` _ascharacter))
    (`self.TriggerBasicAttack` InputRotation)))

(event `ServerTriggerDodge`
  (params (InputRotation :type "Rotator Structure"))
  (`self.MulticastTriggerDodge` InputRotation))

(event `MulticastTriggerDodge`
  (params (InputRotation :type "Rotator Structure"))
  (bind _ascharacter (cast `Character` (`self.GetOwner`)))
  (if (not (`Pawn.IsLocallyControlled` _ascharacter))
    (`self.TriggerDodge` InputRotation)))

(fn `Action Event Check Step`
  (params (Step :type "Float (double-precision)"))
  (locals (EventsToRemove :type "Array of Integer"))
  (for (_array_element _array_index) (`self.Events`)
    (if (< (`.StartTime_5_DF9352264112217122070BB31F281322` (break `/Game/ActionData/Struct_ActionEvent` _array_element)) (- (`GameplayStatics.GetRealTimeSeconds`) (`self.EventQueueStartTime`)))
      (`KismetArrayLibrary.Array_Add` (`local.EventsToRemove`) _array_index)
      (`self.Trigger Action Event` _array_element)))
  (bind (_arrayindex _arrayelement) (`/Engine/EditorBlueprintResources/StandardMacros.ReverseForEachLoop` (`local.EventsToRemove`))
    (:`LoopBody`
      (if (`KismetArrayLibrary.Array_IsValidIndex` (`self.Events`) _arrayelement)
        (`KismetArrayLibrary.Array_Remove` (`self.Events`) _arrayelement)))))

(fn `AutoEndAction`
  (`self.ClearActionState`))

(fn `ClearActionState`
  (bind _gamecharacter (`self.GameCharacter`))
  (`|ExecutionSequence`
    (:`then_0`
      (bind _asbp_2dgame_character (cast `/Game/Characters/CharacterBlueprints/BP_2DGameCharacter` (`self.GetOwner`)))
      (bind _output_get (set `self.GameCharacter` _asbp_2dgame_character))
      (for _array_element (`Actor.K2_GetComponentsByClass` _output_get "/Game/Blueprints/Billboard_Limbs/BPC_BillboardDataControl.BPC_BillboardDataControl_C")
        (if (== (`/Game/Blueprints/Billboard_Limbs/BPC_BillboardDataControl.TagName` _array_element) (`self.CurrentActionSpriteTag`))
          (`/Game/Blueprints/Billboard_Limbs/BPC_BillboardDataControl.Clear Action` _array_element))))
    (:`then_1`
      (set `self.CurrentActionData` (make `/Game/ActionData/Struct_Action1` "None"))
      (set `self.ReadyForNewAction` true))
    (:`then_2`
      (`KismetArrayLibrary.Array_Clear` (`self.Events`)))
    (:`then_3`
      (`/Engine/EditorBlueprintResources/StandardMacros.IsValid` _gamecharacter
        (:`Is Valid`
          (`|ExecutionSequence`
            (:`then_0`
              (if (`Pawn.IsLocallyControlled` _gamecharacter)
                (bind _asbp_game_player_controller (cast `/Game/PlayerController/BP_GamePlayerController` (`Pawn.GetController` _gamecharacter)))
                (`/Game/PlayerController/BP_GamePlayerController.ToggleMovementControlForAction` _asbp_game_player_controller false)))
            (:`then_1`
              (`/Game/Characters/CharacterBlueprints/BP_2DGameCharacter.UpdateMovementSpeed` _gamecharacter 0.0 true))
            (:`then_2`
              (`/Game/Characters/CharacterBlueprints/BP_2DGameCharacter.SetForceForwardState` :`self` _gamecharacter))
            (:`then_3`
              (`/Game/Blueprints/StatTracking/BPC_StatTracking.SetVulnerability` (`/Game/Characters/CharacterBlueprints/BP_2DGameCharacter.BPC_StatTracking` _gamecharacter) false))))))))

(fn `IncapCollisionDestroyed`
  (params (DestroyedActor :type "Actor Object Reference"))
  (set `self.CurrentIncapCollision` null))

(fn `Owner Action Is Local and Ready`
  (returns (Ready :type Boolean))
  (bind _gamecharacter (`self.GameCharacter`))
  (bind _gamecharacter_2 (`self.GameCharacter`))
  (bind _gamecharacter_3 (`self.GameCharacter`))
  (`/Engine/EditorBlueprintResources/StandardMacros.IsValid` _gamecharacter
    (:`Is Valid`
      (if (not (`/Game/Characters/CharacterBlueprints/BP_2DGameCharacter.IsDefeated` _gamecharacter)) :!label _label
        _
        (else
          (return false))))
    (:`Is Not Valid`
      (bind _asbp_2dgame_character (cast `/Game/Characters/CharacterBlueprints/BP_2DGameCharacter` (`self.GetOwner`)))
      (set `self.GameCharacter` _asbp_2dgame_character)
      (`/Engine/EditorBlueprintResources/StandardMacros.IsValid` _gamecharacter
        (:`Is Valid`
          (goto _label))
        (:`Is Not Valid`
          (return false)))))
  (if (`self.ReadyForNewAction`)
    (`/Engine/EditorBlueprintResources/StandardMacros.IsValid` _gamecharacter_2
      (:`Is Valid`
        (if (and (`Pawn.IsLocallyControlled` _gamecharacter_2) (`/Game/Characters/CharacterBlueprints/BP_2DGameCharacter.In No Action State` _gamecharacter_2))
          (`/Engine/EditorBlueprintResources/StandardMacros.IsValid` (`/Game/Characters/CharacterBlueprints/BP_2DGameCharacter.IncapTarget` _gamecharacter_3)
            (:`Is Valid`
              _)
            (:`Is Not Valid`
              (if (not (`/Game/Characters/CharacterBlueprints/BP_2DGameCharacter.IsIncapacitated` _gamecharacter_3))
                (return true)
                (else
                  _)))))
        (return false)))
    (else
      (return false))))

(fn `OwnerActivateBasicAttack`
  (params (InputRotation :type "Rotator Structure"))
  (bind (_basicattackdata_actionname _basicattackdata_billboarddata _basicattackdata_actionevents _basicattackdata_isdefined) (break `/Game/ActionData/Struct_Action1` (`self.BasicAttackData`)))
  (bind _ready (`self.Owner Action Is Local and Ready`))
  (if _ready
    (if _basicattackdata_isdefined
      (`self.ServerTriggerBasicAttack` InputRotation)
      (`self.TriggerBasicAttack` InputRotation))))

(fn `OwnerActivateDodge`
  (params (InputRotation :type "Rotator Structure"))
  (bind (_dodgeactiondata_actionname _dodgeactiondata_billboarddata _dodgeactiondata_actionevents _dodgeactiondata_isdefined) (break `/Game/ActionData/Struct_Action1` (`self.DodgeActionData`)))
  (bind _ready (`self.Owner Action Is Local and Ready`))
  (if _ready
    (if _dodgeactiondata_isdefined
      (`self.ServerTriggerDodge` InputRotation)
      (`self.TriggerDodge` InputRotation))))

(fn `Queue Action Events`
  (params (Events :type "Array of /Game/ActionData/Struct_ActionEvent Structure"))
  (set `self.Events` Events)
  (set `self.EventQueueStartTime` (`GameplayStatics.GetRealTimeSeconds`)))

(fn `Trigger Action Event`
  (params (Event :type "/Game/ActionData/Struct_ActionEvent Structure (by ref)"))
  (bind (_eventname _starttime _lifespan _spawnprojectile _relativespawntf _disablesmovement _enablesmovement _enablesactiontransition _changemovementspeed _setmovementspeed _resetspeed _forcemovementforward _endforcemovementforward _incap _incapdata _telegraphspawn _telegraohrelativespawntf _disablestakingdamage _enablestakingdamage) (break `/Game/ActionData/Struct_ActionEvent` Event))
  (bind _returnvalue (`self.GetOwner`))
  (bind _returnvalue_2 (`self.GetOwner`))
  (bind _gamecharacter (`self.GameCharacter`))
  (bind _gamecharacter_2 (`self.GameCharacter`))
  (bind _gamecharacter_3 (`self.GameCharacter`))
  (bind _gamecharacter_4 (`self.GameCharacter`))
  (bind _gamecharacter_5 (`self.GameCharacter`))
  (bind _gamecharacter_6 (`self.GameCharacter`))
  (bind _gamecharacter_7 (`self.GameCharacter`))
  (bind _gamecharacter_8 (`self.GameCharacter`))
  (bind (_incapname _hideactorandattach _damagepertick _tickrate _ticks _lifetime _collisionradius _collisionoffset) (break `/Game/ActionData/Struct_IncapData` _incapdata))
  (bind _returnvalue_3 (`Actor.K2_GetActorRotation` _returnvalue_2))
  (bind _returnvalue_4 (`Actor.K2_GetActorRotation` _returnvalue))
  (bind _bpc_stattracking (`/Game/Characters/CharacterBlueprints/BP_2DGameCharacter.BPC_StatTracking` (`self.GameCharacter`)))
  (`|ExecutionSequence`
    (:`then_0`
      ;[1 0.1344 0.7061] SpawnActor
      (`|ExecutionSequence`
        (:`then_0`
          (if (`KismetSystemLibrary.IsValidClass` _spawnprojectile)
            (bind _returnvalue_5 (`|SpawnActorFromClass` _spawnprojectile (`KismetMathLibrary.MakeTransform` (+ (`Actor.K2_GetActorLocation` _returnvalue_2) (`KismetMathLibrary.GreaterGreater_VectorRotator` (.location _relativespawntf) _returnvalue_3)) (`KismetMathLibrary.ComposeRotators` _returnvalue_3 (.rotation _relativespawntf)) (.scale _relativespawntf)) "Undefined" "MultiplyWithRoot" _gamecharacter (`/Game/Characters/CharacterBlueprints/BP_2DGameCharacter.TeamId` _gamecharacter) _gamecharacter))
            (`Actor.SetLifeSpan` _returnvalue_5 _lifespan)))))
    (:`then_1`
      ;[1 0.3116 0.2118] EnableAndDisableMovementControl
      (if _disablesmovement
        (`/Engine/EditorBlueprintResources/StandardMacros.IsValid` _gamecharacter_5
          (:`Is Valid`
            (if (`Pawn.IsLocallyControlled` _gamecharacter_5)
              (`/Game/Characters/CharacterBlueprints/BP_2DGameCharacter.SignalAllowMovement` _gamecharacter_5 false)
              (bind _asbp_game_player_controller (cast `/Game/PlayerController/BP_GamePlayerController` (`Pawn.GetController` _gamecharacter_5)))
              (`/Game/PlayerController/BP_GamePlayerController.ToggleMovementControlForAction` _asbp_game_player_controller true))))))
    (:`then_2`
      (if _enablesmovement
        (`/Engine/EditorBlueprintResources/StandardMacros.IsValid` _gamecharacter_6
          (:`Is Valid`
            (if (`Pawn.IsLocallyControlled` _gamecharacter_6)
              (`/Game/Characters/CharacterBlueprints/BP_2DGameCharacter.SignalAllowMovement` _gamecharacter_6 true)
              (bind _asbp_game_player_controller_2 (cast `/Game/PlayerController/BP_GamePlayerController` (`Pawn.GetController` _gamecharacter_6)))
              (`/Game/PlayerController/BP_GamePlayerController.ToggleMovementControlForAction` _asbp_game_player_controller_2 false))))))
    (:`then_3`
      ;[0.4896 0.4943 1] SpeedControl
      (if _changemovementspeed
        (`/Engine/EditorBlueprintResources/StandardMacros.IsValid` _gamecharacter_7
          (:`Is Valid`
            (bind _ascharacter_movement_component (cast `CharacterMovementComponent` (`Pawn.GetMovementComponent` _gamecharacter_7)))
            (set `CharacterMovementComponent.MaxWalkSpeed` _setmovementspeed _ascharacter_movement_component)))))
    (:`then_4`
      (if _resetspeed
        (`/Engine/EditorBlueprintResources/StandardMacros.IsValid` _gamecharacter_8
          (:`Is Valid`
            (bind _ascharacter_movement_component_2 (cast `CharacterMovementComponent` (`Pawn.GetMovementComponent` _gamecharacter_8)))
            (set `CharacterMovementComponent.MaxWalkSpeed` (`/Game/Characters/CharacterBlueprints/BP_2DGameCharacter.DefaultSpeed` _gamecharacter_8) _ascharacter_movement_component_2)))))
    (:`then_5`
      ;[1 0.1828 0.415] ForceMovementForward
      (if _forcemovementforward
        (`/Game/Characters/CharacterBlueprints/BP_2DGameCharacter.SetForceForwardState` _gamecharacter_2 true (`self.SnapshotActionRotation`))
        (elif _endforcemovementforward
          (`/Game/Characters/CharacterBlueprints/BP_2DGameCharacter.SetForceForwardState` :`self` _gamecharacter_2))))
    (:`then_6`
      ;[1 1 1] Incap
      (if _incap
        (bind _returnvalue_6 (`|SpawnActorFromClass` "/Game/ActionData/CombatCollisionComponent/BPC_SphereCollisionComponent.BPC_SphereCollisionComponent_C" (`SceneComponent.K2_GetComponentToWorld` (`Character.Mesh` _gamecharacter_3)) "AlwaysSpawn" "MultiplyWithRoot" _gamecharacter_3 (`/Game/Characters/CharacterBlueprints/BP_2DGameCharacter.TeamId` _gamecharacter_3) (`Pawn.IsLocallyControlled` _gamecharacter_3) (make `/Game/ProjectilesAndSlashes/Struct_ProjectileDamageData` false) true _incapname _hideactorandattach _ticks _tickrate _damagepertick _lifetime _collisionradius _collisionoffset _gamecharacter_3))
        (`Actor.K2_AttachToComponent` _returnvalue_6 (`Character.Mesh` (`self.GameCharacter`)) "None" "KeepRelative" "KeepRelative" "KeepWorld" true)
        (bind _output_get (set `self.CurrentIncapCollision` _returnvalue_6))
        (add `Actor.OnDestroyed` _output_get (`|CreateDelegate` :!event `IncapCollisionDestroyed`))))
    (:`then_7`
      ;[1 0.04843 0.1281] Telegraph Spawn
      (if (`KismetSystemLibrary.IsValidClass` _telegraphspawn)
        (`|SpawnActorFromClass` _telegraphspawn (`KismetMathLibrary.MakeTransform` (+ (`Actor.K2_GetActorLocation` _returnvalue) (`KismetMathLibrary.GreaterGreater_VectorRotator` (.location _telegraohrelativespawntf) _returnvalue_4)) (`KismetMathLibrary.ComposeRotators` _returnvalue_4 (.rotation _telegraohrelativespawntf))) "Undefined" "MultiplyWithRoot" _gamecharacter_4 (`/Game/Characters/CharacterBlueprints/BP_2DGameCharacter.TeamId` _gamecharacter_4) _gamecharacter_4 _gamecharacter_4)))
    (:`then_8`
      ;[1 0.8166 0.1821] Invulnerability
      (if _disablestakingdamage
        (`/Game/Blueprints/StatTracking/BPC_StatTracking.SetVulnerability` _bpc_stattracking true)
        (elif _enablestakingdamage
          (`/Game/Blueprints/StatTracking/BPC_StatTracking.SetVulnerability` _bpc_stattracking false))))))

(fn `TriggerAction`
  (params (Action :type "/Game/ActionData/Struct_Action1 Structure (by ref)") (SnapshotWorldRotation :type "Rotator Structure"))
  (bind _gamecharacter (`self.GameCharacter`))
  (bind _output_get (set `self.CurrentActionData` Action))
  (set `self.SnapshotActionRotation` SnapshotWorldRotation)
  (bind (_actionname _billboarddata _actionevents _isdefined _spritetag) (break `/Game/ActionData/Struct_Action1` _output_get))
  (`self.Queue Action Events` _actionevents)
  (set `self.ReadyForNewAction` false)
  (bind _returnvalue (`KismetSystemLibrary.K2_SetTimer` null "AutoEndAction" (/ (`KismetMathLibrary.Conv_IntToDouble` (`KismetArrayLibrary.Array_Length` (break `/Game/Blueprints/Billboard_Limbs/Struct_BillboardData` _billboarddata))) (`.PlayRate_31_5653BD6F41767AC25D56449EE85EFC95` (break `/Game/Blueprints/Billboard_Limbs/Struct_BillboardData` _billboarddata)))))
  (set `self.ActionTimer` _returnvalue)
  (`/Engine/EditorBlueprintResources/StandardMacros.IsValid` _gamecharacter
    (:`Is Valid`
      _)
    (:`Is Not Valid`
      (bind _asbp_2dgame_character (cast `/Game/Characters/CharacterBlueprints/BP_2DGameCharacter` (`self.GetOwner`)))
      (set `self.GameCharacter` _asbp_2dgame_character)))
  (for _array_element (`Actor.K2_GetComponentsByClass` _gamecharacter "/Game/Blueprints/Billboard_Limbs/BPC_BillboardDataControl.BPC_BillboardDataControl_C")
    (if (== (`/Game/Blueprints/Billboard_Limbs/BPC_BillboardDataControl.TagName` _array_element) _spritetag)
      (`/Game/Blueprints/Billboard_Limbs/BPC_BillboardDataControl.SetAction` (`/Game/Characters/CharacterBlueprints/BP_2DGameCharacter.BPC_BillboardDataControl` _gamecharacter) (`.BillboardData_8_C125C66048CC4E054D524F996060D22E` (break `/Game/ActionData/Struct_Action1` (`self.CurrentActionData`))))
      (`/Game/Blueprints/Billboard_Limbs/BPC_BillboardDataControl.SetAction` _array_element (`.BillboardData_8_C125C66048CC4E054D524F996060D22E` (break `/Game/ActionData/Struct_Action1` (`self.CurrentActionData`))))))
  (set `self.CurrentActionSpriteTag` _spritetag))

(fn `TriggerBasicAttack`
  (params (InputRotation :type "Rotator Structure"))
  (`self.TriggerAction` (`self.BasicAttackData`) InputRotation))

(fn `TriggerDodge`
  (params (InputRotation :type "Rotator Structure"))
  (bind _ascharacter (cast `Character` (`self.GetOwner`)))
  (`Actor.K2_SetActorRotation` _ascharacter InputRotation true)
  (`self.TriggerAction` (`self.DodgeActionData`) InputRotation))