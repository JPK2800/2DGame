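; A short-lived spherical combat hitbox actor that applies damage and incapacitation to enemy 2D game characters.
; On spawn it sizes itself from Radius and catches characters via an initial overlap check and later begin-overlap events.
; Hits process only for locally controlled players or when IsLocalControlledChar is set, once per actor and skipping same-team targets.
; Damage goes through the target's stat tracking component; an incapacitation also notifies the attacker and shuts the hitbox down.
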(event `self.ReceiveBeginPlay`
  (`self.TraceOnSpawn`)
  (`self.SetLifeSpan` (`self.Lifetime`))
  (`SceneComponent.K2_SetRelativeTransform` (`self.CollisionComponent`) (`KismetMathLibrary.MakeTransform` (`self.SpawnOffsetFromFloor`) (struct) (`KismetMathLibrary.Conv_DoubleToVector` (/ (`self.Radius`) 80.0))) false false))

(event `self.CollisionComponent.OnComponentBeginOverlap`
  (params (OverlappedComponent :type "PrimitiveComponent Object Reference") (OtherActor :type "Actor Object Reference") (OtherComp :type "PrimitiveComponent Object Reference") (OtherBodyIndex :type Integer) (bFromSweep :type Boolean) (SweepResult :type "HitResult Structure (by ref)"))
  (bind _asbp_2dgame_character (cast `/Game/Characters/CharacterBlueprints/BP_2DGameCharacter` OtherActor))
  (`self.OnOverlap` _asbp_2dgame_character))

(fn `HitTarget`
  (params (Target :type "/Game/Characters/CharacterBlueprints/BP_2DGameCharacter Object Reference") (StatTrackingTarget :type "/Game/CharacterComponents/StatTracking/BPC_StatTracking Object Reference") (Attacker :type "/Game/Characters/CharacterBlueprints/BP_2DGameCharacter Object Reference"))
  (bind (_damagedata_dealsdamage _damagedata_immediatedamage _damagedata_dealsdamageinticks) (break `/Game/ProjectilesAndSlashes/Struct_ProjectileDamageData` (`self.DamageData`)))
  (if (not (`self.IncapStarted`))
    (`/Engine/EditorBlueprintResources/StandardMacros.IsValid` StatTrackingTarget
      (:`Is Valid`
        (`/Engine/EditorBlueprintResources/StandardMacros.IsValid` Target
          (:`Is Valid`
            (`|ExecutionSequence`
              (:`then_0`
                (if (or _damagedata_dealsdamage _damagedata_dealsdamageinticks)
                  (bind _asbp_2dgame_character (cast `/Game/Characters/CharacterBlueprints/BP_2DGameCharacter` (`self.GetOwner`)))
                  (`/Game/CharacterComponents/StatTracking/BPC_StatTracking.TakeContact` StatTrackingTarget (`self.DamageData`) _asbp_2dgame_character null "None" (`|MakeArray`))))
              (:`then_1`
                (`/Engine/EditorBlueprintResources/StandardMacros.IsValid` Attacker
                  (:`Is Valid`
                    (if (`self.IsIncap`)
                      (`/Game/CharacterComponents/StatTracking/BPC_StatTracking.ReceiveIncapacitation` StatTrackingTarget Attacker (`self.IncapName`) (`self.IncapAttachAndHideActor`))
                      (`/Game/Characters/CharacterBlueprints/BP_2DGameCharacter.HideActorWhenIncapacitating` Attacker (`self.IncapAttachAndHideActor`) Target)
                      (set `self.IncapStarted` true)
                      (`PrimitiveComponent.SetCollisionEnabled` (`self.CollisionComponent`) "NoCollision")
                      (`self.SetLifeSpan` 0.05))))))))))))

(fn `OnOverlap`
  (params (OverlappedActor :type "/Game/Characters/CharacterBlueprints/BP_2DGameCharacter Object Reference"))
  (bind _bpc_stattracking (`/Game/Characters/CharacterBlueprints/BP_2DGameCharacter.BPC_StatTracking` OverlappedActor))
  (bind _teamid_teamid (break `GenericTeamId` (`/Game/Characters/CharacterBlueprints/BP_2DGameCharacter.TeamId` OverlappedActor)))
  (if (or (and (`Pawn.IsPlayerControlled` OverlappedActor) (`Pawn.IsLocallyControlled` OverlappedActor)) (`self.IsLocalControlledChar`))
    (if (not (`KismetArrayLibrary.Array_Contains` (`self.HitActors`) OverlappedActor))
      (`|ExecutionSequence`
        (:`then_0`
          (`/Engine/EditorBlueprintResources/StandardMacros.IsValid` _bpc_stattracking
            (:`Is Valid`
              (if (!= _teamid_teamid (`.TeamID` (break `GenericTeamId` (`self.TeamId`))))
                (bind _asbp_2dgame_character (cast `/Game/Characters/CharacterBlueprints/BP_2DGameCharacter` (`self.GetOwner`)))
                (`self.HitTarget` OverlappedActor _bpc_stattracking _asbp_2dgame_character)))))
        (:`then_1`
          (`KismetArrayLibrary.Array_Add` (`self.HitActors`) OverlappedActor))))))

(fn `TraceOnSpawn`
  (for _array_element (`PrimitiveComponent.GetOverlappingActors` (`self.CollisionComponent`) null)
    (bind _asbp_2dgame_character (cast `/Game/Characters/CharacterBlueprints/BP_2DGameCharacter` _array_element))
    (`self.OnOverlap` _asbp_2dgame_character)))

(fn `UserConstructionScript`)