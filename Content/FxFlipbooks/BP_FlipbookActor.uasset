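; Flipbook effect actor that plays a Paper2D flipbook once and can destroy itself when playback finishes.
; Looping is turned off on BeginPlay, and the finished event destroys the actor if DestroyAfterSinglePlay is set.
; Each tick it can billboard the flipbook using a look-at rotation from the cached player 0 camera, with a 90-degree yaw offset.
; UseZAxisOrient selects full rotation; otherwise only yaw follows the camera.
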(event `self.ReceiveBeginPlay`
  (`PaperFlipbookComponent.SetLooping` (`self.FP`) false))

(event `self.ReceiveTick`
  (params (DeltaSeconds :type "Float (single-precision)"))
  (`self.OrientToCameraStep`))

(event `self.FP.OnFinishedPlaying`
  (if (`self.DestroyAfterSinglePlay`)
    (`self.K2_DestroyActor`)))

(fn `OrientToCameraStep`
  (bind _fp (`self.FP`))
  (bind _returnvalue (`KismetMathLibrary.FindLookAtRotation` (`PlayerCameraManager.GetCameraLocation` (`self.CameraManager`)) (`self.K2_GetActorLocation`)))
  (if (`self.OrientToPlayerCamera`)
    (`/Engine/EditorBlueprintResources/StandardMacros.IsValid` (`self.CameraManager`)
      (:`Is Valid`
        _)
      (:`Is Not Valid`
        (set `self.CameraManager` (`GameplayStatics.GetPlayerCameraManager` 0))))
    (if (`self.UseZAxisOrient`)
      (`SceneComponent.K2_SetWorldRotation` _fp (`KismetMathLibrary.MakeRotator` (.roll _returnvalue) (.pitch _returnvalue) (+ (.yaw _returnvalue) 90.0)) false false)
      (else
        (`SceneComponent.K2_SetWorldRotation` _fp (`KismetMathLibrary.MakeRotator` 0.0 0.0 (+ (.yaw _returnvalue) 90.0)) false false)))))

(fn `UserConstructionScript`)