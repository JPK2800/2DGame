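; BP_WizardWhack is an effect actor that swaps between two visual components, FP and FP20, based on the player camera's viewing angle.
; A looping timer, started on BeginPlay and cleared on Destroyed, runs UpdateByCamAngle instead of using Tick.
; That function converts the camera-to-actor direction into local yaw, showing FP20 when the view is near the actor's forward/back axis and FP otherwise.
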(event `self.ReceiveBeginPlay`
  (`parent.ReceiveBeginPlay`)
  (bind _returnvalue (`KismetSystemLibrary.K2_SetTimer` null "UpdateByCamAngle" 0.1 true))
  (set `self.CamAngleTimer` _returnvalue)
  (`self.UpdateByCamAngle`))

(event `self.ReceiveDestroyed`
  (`KismetSystemLibrary.K2_ClearAndInvalidateTimerHandle` (`self.CamAngleTimer`))
  (`parent.ReceiveDestroyed`))

(fn `UpdateByCamAngle`
  (bind _showfrontfp (`self.ShowFrontFP`))
  (bind (_returnvalue_roll _returnvalue_pitch _returnvalue_yaw) (`KismetMathLibrary.BreakRotator` (`KismetMathLibrary.MakeRotationFromAxes` (`KismetMathLibrary.LessLess_VectorRotator` (`KismetMathLibrary.GetForwardVector` (`KismetMathLibrary.FindLookAtRotation` (`PlayerCameraManager.GetCameraLocation` (`GameplayStatics.GetPlayerCameraManager` 0)) (`self.K2_GetActorLocation`))) (`self.K2_GetActorRotation`)))))
  (bind _returnvalue (`KismetMathLibrary.Abs` _returnvalue_yaw))
  (if (or (< _returnvalue 20.0) (> _returnvalue 160.0))
    (set `self.ShowFrontFP` true)
    (else
      (set `self.ShowFrontFP` false)))
  (`SceneComponent.SetVisibility` (`self.FP`) (not _showfrontfp) true)
  (`SceneComponent.SetVisibility` (`self.FP_<20`) _showfrontfp true))

(fn `UserConstructionScript`
  (`parent.UserConstructionScript`))