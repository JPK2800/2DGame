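; Player controller for BP_2DGameCharacter that handles camera-relative movement, spring-arm look, interaction, debug states and a controls-screen toggle.
; Attack and dodge presses become timestamped objects in an input buffer, which Tick drains into BPCCharacterActionData when ready, discarding expired entries and aiming by move input.
; Stat-tracking incapacitation events are bound to block movement and attack input.
; An optional debug widget supports character selection, with ServerSpawnActor spawning and possessing at a PlayerStart.
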(event `self.ReceiveBeginPlay`
  (bind _returnvalue (subsystem `EnhancedInputLocalPlayerSubsystem`))
  (`self.InitDebugSpawner`)
  (`/Engine/EditorBlueprintResources/StandardMacros.IsValid` _returnvalue
    (:`Is Valid`
      (`EnhancedInputSubsystemInterface.AddMappingContext` _returnvalue "/Game/PlayerController/Inputs/IMC_GameCharacter.IMC_GameCharacter" 0 (struct)))))

(event `self.ReceiveTick`
  (params (DeltaSeconds :type "Float (single-precision)"))
  (`self.UpdateControlRotation`)
  (`self.HandleQueuedActionsStep` DeltaSeconds))

(event `EnhancedInput|/Game/PlayerController/Inputs/IA_Move`
  (params (ActionValue :type "Vector2D Structure") (ElapsedSeconds :type "Float (double-precision)") (TriggeredSeconds :type "Float (double-precision)") (InputAction :type "InputAction Object Reference" :default "/Game/PlayerController/Inputs/IA_Move.IA_Move"))
  (bind (_x _y) (`KismetMathLibrary.BreakVector2D` ActionValue))
  (bind _gamecharacter (`self.GameCharacter`))
  (:`Triggered`
    (if (and (not (`self.MovementControlDisabled`)) (not (`self.Incap`)))
      (`/Engine/EditorBlueprintResources/StandardMacros.IsValid` _gamecharacter
        (:`Is Valid`
          _)
        (:`Is Not Valid`
          (`self.InitGameCharacter`)
          (`/Engine/EditorBlueprintResources/StandardMacros.IsValid` _gamecharacter
            (:`Is Valid`
              _))))
      (if (not (`/Game/Characters/CharacterBlueprints/BP_2DGameCharacter.IsDefeated` _gamecharacter))
        (`Pawn.AddMovementInput` _gamecharacter (`KismetMathLibrary.GreaterGreater_VectorRotator` (`KismetMathLibrary.MakeVector` _y _x) (`self.GetControlRotation`)) (`KismetMathLibrary.VSize2D` ActionValue) false)))))

(event `EnhancedInput|/Game/PlayerController/Inputs/IA_Look`
  (params (ActionValue :type "Vector2D Structure") (ElapsedSeconds :type "Float (double-precision)") (TriggeredSeconds :type "Float (double-precision)") (InputAction :type "InputAction Object Reference" :default "/Game/PlayerController/Inputs/IA_Look.IA_Look"))
  (bind _gamecharacter (`self.GameCharacter`))
  (bind _springarm (`/Game/Characters/CharacterBlueprints/BP_2DGameCharacter.SpringArm` _gamecharacter))
  (bind (_returnvalue_roll _returnvalue_pitch _returnvalue_yaw) (`KismetMathLibrary.BreakRotator` (`SceneComponent.K2_GetComponentRotation` _springarm)))
  (:`Triggered`
    (`/Engine/EditorBlueprintResources/StandardMacros.IsValid` _gamecharacter
      (:`Is Valid`
        _)
      (:`Is Not Valid`
        (`self.InitGameCharacter`)
        (`/Engine/EditorBlueprintResources/StandardMacros.IsValid` _gamecharacter
          (:`Is Valid`
            _))))
    (if (`/Game/Characters/CharacterBlueprints/BP_2DGameCharacter.AllowCamMovement` _gamecharacter)
      (`SceneComponent.K2_SetWorldRotation` _springarm (`KismetMathLibrary.MakeRotator` 0.0 (`KismetMathLibrary.FClamp` (+ _returnvalue_pitch ActionValue_Y) -30.0 0.0) (+ _returnvalue_yaw ActionValue_X)) false false))))

(event `EnhancedInput|/Game/PlayerController/Inputs/IA_BasicAttack`
  (params (ActionValue :type Boolean) (ElapsedSeconds :type "Float (double-precision)") (TriggeredSeconds :type "Float (double-precision)") (InputAction :type "InputAction Object Reference" :default "/Game/PlayerController/Inputs/IA_BasicAttack.IA_BasicAttack"))
  (:`Triggered`
    (if (not (`self.Incap`))
      (`self.QueueAction` "BasicAttack"))))

(event `EnhancedInput|/Game/PlayerController/Inputs/IA_Roll`
  (params (ActionValue :type Boolean) (ElapsedSeconds :type "Float (double-precision)") (TriggeredSeconds :type "Float (double-precision)") (InputAction :type "InputAction Object Reference" :default "/Game/PlayerController/Inputs/IA_Roll.IA_Roll"))
  (:`Triggered`
    (if ActionValue
      (`self.QueueAction` "Dodge"))))

(event `EnhancedInput|/Game/PlayerController/Inputs/IA_DebugButton7`
  (params (ActionValue :type Boolean) (ElapsedSeconds :type "Float (double-precision)") (TriggeredSeconds :type "Float (double-precision)") (InputAction :type "InputAction Object Reference" :default "/Game/PlayerController/Inputs/IA_DebugButton7.IA_DebugButton7"))
  (bind _gamecharacter (`self.GameCharacter`))
  (:`Triggered`
    (if ActionValue
      (`/Engine/EditorBlueprintResources/StandardMacros.IsValid` _gamecharacter
        (:`Is Valid`
          (`/Game/Characters/CharacterBlueprints/BP_2DGameCharacter.Owner Update State` _gamecharacter "None" true))))))

(event `EnhancedInput|/Game/PlayerController/Inputs/IA_DebugButton8`
  (params (ActionValue :type Boolean) (ElapsedSeconds :type "Float (double-precision)") (TriggeredSeconds :type "Float (double-precision)") (InputAction :type "InputAction Object Reference" :default "/Game/PlayerController/Inputs/IA_DebugButton8.IA_DebugButton8"))
  (bind _gamecharacter (`self.GameCharacter`))
  (:`Triggered`
    (if ActionValue
      (`/Engine/EditorBlueprintResources/StandardMacros.IsValid` _gamecharacter
        (:`Is Valid`
          (`/Game/Characters/CharacterBlueprints/BP_2DGameCharacter.Owner Update State` _gamecharacter "Defeated" false))))))

(event `EnhancedInput|/Game/PlayerController/Inputs/IA_DebugButton9`
  (params (ActionValue :type Boolean) (ElapsedSeconds :type "Float (double-precision)") (TriggeredSeconds :type "Float (double-precision)") (InputAction :type "InputAction Object Reference" :default "/Game/PlayerController/Inputs/IA_DebugButton9.IA_DebugButton9"))
  (bind _gamecharacter (`self.GameCharacter`))
  (:`Triggered`
    (if ActionValue
      (`/Engine/EditorBlueprintResources/StandardMacros.IsValid` _gamecharacter
        (:`Is Valid`
          (`/Game/Characters/CharacterBlueprints/BP_2DGameCharacter.Owner Update State` _gamecharacter "Stomped" false))))))

(event `EnhancedInput|/Game/PlayerController/Inputs/IA_DebugButton0`
  (params (ActionValue :type Boolean) (ElapsedSeconds :type "Float (double-precision)") (TriggeredSeconds :type "Float (double-precision)") (InputAction :type "InputAction Object Reference" :default "/Game/PlayerController/Inputs/IA_DebugButton0.IA_DebugButton0"))
  (:`Triggered`
    (if ActionValue
      (`/Engine/EditorBlueprintResources/StandardMacros.IsValid` (`self.GameCharacter`)))))

(event `EnhancedInput|/Game/PlayerController/Inputs/IA_Pause`
  (params (ActionValue :type Boolean) (ElapsedSeconds :type "Float (double-precision)") (TriggeredSeconds :type "Float (double-precision)") (InputAction :type "InputAction Object Reference" :default "/Game/PlayerController/Inputs/IA_Pause.IA_Pause"))
  (:`Started`
    (`self.TogglePause` (not (`self.Paused`)))))

(event `EnhancedInput|/Game/PlayerController/Inputs/IA_Interact`
  (params (ActionValue :type Boolean) (ElapsedSeconds :type "Float (double-precision)") (TriggeredSeconds :type "Float (double-precision)") (InputAction :type "InputAction Object Reference" :default "/Game/PlayerController/Inputs/IA_Interact.IA_Interact"))
  (bind _gamecharacter (`self.GameCharacter`))
  (:`Started`
    (`/Engine/EditorBlueprintResources/StandardMacros.IsValid` _gamecharacter
      (:`Is Valid`
        (`/Game/Characters/CharacterBlueprints/BP_2DGameCharacter.OnInteract` _gamecharacter)))))

(event `ServerSpawnActor`
  (params (Class :type "/Game/Characters/CharacterBlueprints/BP_2DGameCharacter Class Reference"))
  (bind _returnvalue (`GameplayStatics.GetActorOfClass` "/Script/Engine.PlayerStart"))
  (`/Engine/EditorBlueprintResources/StandardMacros.IsValid` _returnvalue
    (:`Is Valid`
      (bind _returnvalue_2 (`|SpawnActorFromClass` Class (`KismetMathLibrary.MakeTransform` (`self.K2_GetActorLocation` _returnvalue) (`self.K2_GetActorRotation` _returnvalue)) "AlwaysSpawn" "MultiplyWithRoot" self null null))
      (`self.Possess` _returnvalue_2))))

(fn `HandleQueuedActionIfReady`
  (params (QueuedData :type "/Game/PlayerController/BP_QueuedDataObject Object Reference"))
  (returns (Success :type Boolean) (Remove :type Boolean))
  (locals (InputRot :type "Rotator Structure" :default (struct)) (MovementInputMeetsThreshold :type Boolean))
  (bind (_returnvalue_x _returnvalue_y) (`KismetMathLibrary.BreakVector2D` (`|GetInputActionValue`)))
  (bind _gamecharacter (`self.GameCharacter`))
  (bind _gamecharacter_2 (`self.GameCharacter`))
  (bind _gamecharacter_3 (`self.GameCharacter`))
  (bind _gamecharacter_4 (`self.GameCharacter`))
  (bind _bpc_characteractiondata (`/Game/Characters/CharacterBlueprints/BP_2DGameCharacter.BPC_CharacterActionData` _gamecharacter_3))
  (bind (_x _y) (`KismetMathLibrary.BreakVector3f` (`KismetMathLibrary.GreaterGreater_VectorRotator` (`KismetMathLibrary.MakeVector` (* _returnvalue_y 1.0) (* _returnvalue_x 1.0)) (`self.GetControlRotation`))))
  (bind _expire (`/Game/PlayerController/BP_QueuedDataObject.IsExpired` QueuedData (`GameplayStatics.GetRealTimeSeconds`)))
  (if _expire
    (return false true)
    (else
      (set `local.MovementInputMeetsThreshold` (> (+ (`KismetMathLibrary.Abs` _returnvalue_x) (`KismetMathLibrary.Abs` _returnvalue_y)) 0.2))
      (set `local.InputRot` (`KismetMathLibrary.Conv_VectorToRotator` (`KismetMathLibrary.Normal` (`KismetMathLibrary.MakeVector` _x _y))))
      (`|ExecutionSequence`
        (:`then_0`
          (switch `name` (`/Game/PlayerController/BP_QueuedDataObject.EventName` QueuedData)
            (:`Dodge`
              ;[0.5736 0.3268 1] Dodge
              (if (`local.MovementInputMeetsThreshold`)
                (`/Engine/EditorBlueprintResources/StandardMacros.IsValid` _gamecharacter
                  (:`Is Valid`
                    _)
                  (:`Is Not Valid`
                    (`self.InitGameCharacter`)))
                (`/Engine/EditorBlueprintResources/StandardMacros.IsValid` _gamecharacter_2
                  (:`Is Valid`
                    (if (`.IsDefined_16_BF70770E4D3FBB2912EDCAA8619CD20A` (break `/Game/ActionData/Struct_Action1` (`/Game/ActionData/BPC_CharacterActionData.DodgeActionData` (`/Game/Characters/CharacterBlueprints/BP_2DGameCharacter.BPC_CharacterActionData` _gamecharacter_2))))
                      (`/Game/ActionData/BPC_CharacterActionData.OwnerActivateDodge` (`/Game/Characters/CharacterBlueprints/BP_2DGameCharacter.BPC_CharacterActionData` _gamecharacter) (`local.InputRot`)))))))
            (:`BasicAttack`
              ;[1 0.2417 0.4432] BasicAttack
              (`/Engine/EditorBlueprintResources/StandardMacros.IsValid` _gamecharacter_3
                (:`Is Valid`
                  _)
                (:`Is Not Valid`
                  (`self.InitGameCharacter`)))
              (`/Engine/EditorBlueprintResources/StandardMacros.IsValid` _gamecharacter_4
                (:`Is Valid`
                  (if (`local.MovementInputMeetsThreshold`)
                    (if (`.IsDefined_16_BF70770E4D3FBB2912EDCAA8619CD20A` (break `/Game/ActionData/Struct_Action1` (`/Game/ActionData/BPC_CharacterActionData.BasicAttackData` (`/Game/Characters/CharacterBlueprints/BP_2DGameCharacter.BPC_CharacterActionData` _gamecharacter_4))))
                      (`/Game/ActionData/BPC_CharacterActionData.OwnerActivateBasicAttack` _bpc_characteractiondata (`local.InputRot`)))
                    (else
                      (`/Game/ActionData/BPC_CharacterActionData.OwnerActivateBasicAttack` _bpc_characteractiondata (`KismetMathLibrary.MakeRotator` 0.0 0.0 (.yaw (`self.K2_GetActorRotation` _gamecharacter_3)))))))))))
        (:`then_1`
          (return true true))))))

(fn `HandleQueuedActionsStep`
  (params (Delta :type "Float (double-precision)"))
  (locals (FoundAction :type Boolean) (IndexToCheck :type Integer) (CountInputs :type Integer :default 0))
  (bind _gamecharacter (`self.GameCharacter`))
  (bind _queuedinputs (`self.QueuedInputs`))
  (bind _indextocheck (`local.IndexToCheck`))
  (bind _output (`|GetArrayItem` _queuedinputs _indextocheck))
  (bind _bpc_characteractiondata (`/Game/Characters/CharacterBlueprints/BP_2DGameCharacter.BPC_CharacterActionData` _gamecharacter))
  (`/Engine/EditorBlueprintResources/StandardMacros.IsValid` _gamecharacter
    (:`Is Valid`
      (`/Engine/EditorBlueprintResources/StandardMacros.IsValid` _bpc_characteractiondata
        (:`Is Valid`
          (bind _ready (`/Game/ActionData/BPC_CharacterActionData.Owner Action Is Local and Ready` _bpc_characteractiondata))
          (if _ready
            (bind _output_get (set `local.CountInputs` (`KismetArrayLibrary.Array_Length` _queuedinputs)))
            (while (<= _output_get (`KismetArrayLibrary.Array_Length` _queuedinputs))
              (if (`KismetArrayLibrary.Array_IsValidIndex` _queuedinputs _indextocheck)
                (`/Engine/EditorBlueprintResources/StandardMacros.IsValid` _output
                  (:`Is Valid`
                    (bind (_success _remove) (`self.HandleQueuedActionIfReady` _output))
                    (if _remove
                      (`KismetArrayLibrary.Array_RemoveItem` _queuedinputs _output))
                    (return))
                  (:`Is Not Valid`
                    (`KismetArrayLibrary.Array_Remove` _queuedinputs (`local.IndexToCheck`))))
                (else
                  (`/Engine/EditorBlueprintResources/StandardMacros.IncrementInt` (`local.CountInputs`)))))))))))

(fn `IncapBegin`
  (params (Type :type Name) (Attacker :type "/Game/Characters/CharacterBlueprints/BP_2DGameCharacter Object Reference") (HideAndAttachAttacker :type Boolean))
  (set `self.Incap` true))

(fn `IncapEnd`
  (set `self.Incap` false))

(fn `InitDebugSpawner`
  (if (and (`self.DebugSpawner`) (`self.IsLocalPlayerController`))
    (bind _returnvalue (`|CreateWidget` "/Game/PlayerController/WBP_DebugCharacterSelection.WBP_DebugCharacterSelection_C" self))
    (`UserWidget.AddToPlayerScreen` _returnvalue 0)
    (set `self.DebugSpawnerWidget` _returnvalue)))

(fn `InitGameCharacter`
  (bind _asbp_2dgame_character (cast `/Game/Characters/CharacterBlueprints/BP_2DGameCharacter` (`self.K2_GetPawn`)))
  (set `self.GameCharacter` _asbp_2dgame_character)
  (bind _bpc_stattracking (`/Game/Characters/CharacterBlueprints/BP_2DGameCharacter.BPC_StatTracking` _asbp_2dgame_character))
  (add `/Game/CharacterComponents/StatTracking/BPC_StatTracking.OnReceiveIncapacitation` _bpc_stattracking (`|CreateDelegate` :!event `IncapBegin`))
  (add `/Game/CharacterComponents/StatTracking/BPC_StatTracking.OnEndIncapacitation` _bpc_stattracking (`|CreateDelegate` :!event `IncapEnd`)))

(fn `QueueAction`
  (params (Action :type Name))
  (bind _returnvalue (`|GenericCreateObject` "/Game/PlayerController/BP_QueuedDataObject.BP_QueuedDataObject_C" Action (`GameplayStatics.GetRealTimeSeconds`)))
  (`KismetArrayLibrary.Array_Add` (`self.QueuedInputs`) _returnvalue))

(fn `SpawnCharacterOfClass`
  (params (Class :type "/Game/Characters/CharacterBlueprints/BP_2DGameCharacter Class Reference"))
  (if (and (`KismetSystemLibrary.IsValidClass` Class) (`self.IsLocalController` self))
    (`self.ServerSpawnActor` Class)))

(fn `ToggleMovementControlForAction`
  (params (Disable :type Boolean))
  (set `self.MovementControlDisabled` Disable))

(fn `TogglePause`
  (params (StartPause :type Boolean))
  (if StartPause
    (bind _returnvalue (`|CreateWidget` "/Game/Controls/WBP_Controls.WBP_Controls_C" self))
    (`UserWidget.AddToPlayerScreen` _returnvalue 0)
    (set `self.PauseControlsScreen` _returnvalue)
    (set `self.Paused` true)
    (else
      (`Widget.RemoveFromParent` (`self.PauseControlsScreen`))
      (set `self.Paused` false))))

(fn `UpdateControlRotation`
  (`self.SetControlRotation` (`PlayerCameraManager.GetCameraRotation` (`GameplayStatics.GetPlayerCameraManager` 0))))

(fn `UserConstructionScript`)