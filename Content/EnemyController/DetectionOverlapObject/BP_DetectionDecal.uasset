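; BP_DetectionDecal is a detection area that reports when an enemy character enters its mesh.
; On BeginPlay it sets the visibility of its mesh and decal from the ShowMesh and ShowDecal flags.
; Mesh overlaps with BP_2DGameCharacter actors trigger EnemyDetected, but only when the owner character is valid and locally controlled and the other character's team ID differs.
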(event `self.ReceiveBeginPlay`
  (`SceneComponent.SetVisibility` (`self.StaticMesh`) (`self.ShowMesh`) false)
  (`SceneComponent.SetVisibility` (`self.Decal`) (`self.ShowDecal`) false))

(event `self.StaticMesh.OnComponentBeginOverlap`
  (params (OverlappedComponent :type "PrimitiveComponent Object Reference") (OtherActor :type "Actor Object Reference") (OtherComp :type "PrimitiveComponent Object Reference") (OtherBodyIndex :type Integer) (bFromSweep :type Boolean) (SweepResult :type "HitResult Structure (by ref)"))
  (bind _asbp_2dgame_character (cast `/Game/Characters/CharacterBlueprints/BP_2DGameCharacter` OtherActor))
  (`self.EnemyOverlap` _asbp_2dgame_character))

(fn `EnemyOverlap`
  (params (Character :type "/Game/Characters/CharacterBlueprints/BP_2DGameCharacter Object Reference"))
  (bind _ownercharacter (`self.OwnerCharacter`))
  (`/Engine/EditorBlueprintResources/StandardMacros.IsValid` _ownercharacter
    (:`Is Valid`
      (if (`Pawn.IsLocallyControlled` _ownercharacter)
        (if (!= (`.TeamID` (break `GenericTeamId` (`/Game/Characters/CharacterBlueprints/BP_2DGameCharacter.TeamId` _ownercharacter))) (`.TeamID` (break `GenericTeamId` (`/Game/Characters/CharacterBlueprints/BP_2DGameCharacter.TeamId` Character))))
          (`self.EnemyDetected` Character))))))

(fn `UserConstructionScript`)