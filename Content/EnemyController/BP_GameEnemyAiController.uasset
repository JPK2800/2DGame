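; AI controller for enemy BP_2DGameCharacter pawns that chases detected targets and performs basic attacks.
; Character events for detection, hits, defeat and movement control maintain the target list and state, switching to an attacker if it is closer.
; Tick stops movement at a preferred distance and, when the action component is ready, attacks within a range band or resumes the chase.
; Per-action requirement checks are stubbed to always pass.
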(event `self.ReceiveBeginPlay`
  (`self.InitControlledCharacter`))

(event `self.ReceiveTick`
  (params (DeltaSeconds :type "Float (single-precision)"))
  (`self.CheckDistToCancelMovementStep`)
  (`self.CheckToStartActionStep`))

(fn `ActivateAction`
  (params (Action :type Name))
  (bind (_returnvalue_roll _returnvalue_pitch _returnvalue_yaw) (`KismetMathLibrary.BreakRotator` (`KismetMathLibrary.FindLookAtRotation` (`self.K2_GetActorLocation` (`self.GameCharacter`)) (`self.K2_GetActorLocation` (`self.CurrentTarget`)))))
  (`self.CancelMovement`)
  (switch `name` Action
    (:`BasicAttack`
      (`/Game/ActionData/BPC_CharacterActionData.OwnerActivateBasicAttack` (`/Game/Characters/CharacterBlueprints/BP_2DGameCharacter.BPC_CharacterActionData` (`self.GameCharacter`)) (`KismetMathLibrary.MakeRotator` 0.0 0.0 _returnvalue_yaw)))))

(fn `ActivateAi`
  (set `self.AiActive` true)
  (`self.SetActorTickEnabled` true))

(fn `CancelMovement`
  (`self.StopMovement`)
  (set `self.IsMoving` false))

(fn `CharacterMovementControlChanged`
  (params (Enabled :type Boolean))
  (bind _output_get (set `self.AiActive` Enabled))
  (if (not _output_get)
    (`self.StopMovement`)))

(fn `CheckDistToCancelMovementStep`
  (bind _currenttarget (`self.CurrentTarget`))
  (if (`self.IsMoving`)
    (`/Engine/EditorBlueprintResources/StandardMacros.IsValid` _currenttarget
      (:`Is Valid`
        (if (<= (`KismetMathLibrary.Vector_Distance` (`self.K2_GetActorLocation` _currenttarget) (`self.K2_GetActorLocation` (`self.GameCharacter`))) (`self.PreferredDistanceToTarget`))
          (`self.CancelMovement`))))))

(fn `CheckToStartActionStep`
  (bind _currenttarget (`self.CurrentTarget`))
  (bind _gamecharacter (`self.GameCharacter`))
  (`/Engine/EditorBlueprintResources/StandardMacros.IsValid` (`self.CurrentTarget`)
    (:`Is Valid`
      (`/Engine/EditorBlueprintResources/StandardMacros.IsValid` _gamecharacter
        (:`Is Valid`
          (if (and (not (`self.IsDefeated`)) (`/Game/ActionData/BPC_CharacterActionData.ReadyForNewAction` (`/Game/Characters/CharacterBlueprints/BP_2DGameCharacter.BPC_CharacterActionData` _gamecharacter)))
            (`|ExecutionSequence`
              (:`then_2`
                (bind _valid (`self.ConsiderAction` (`self.BasicAttackRequirementData`)))
                (if _valid
                  (`self.ActivateAction` "BasicAttack")
                  (return)))
              (:`then_3`
                (if (not (`self.IsMoving`))
                  (`/Engine/EditorBlueprintResources/StandardMacros.IsValid` _currenttarget
                    (:`Is Valid`
                      (`self.Move Towards Actor` _currenttarget))
                    (:`Is Not Valid`
                      (bind _newtarg (`self.ConsiderNewtarget`))
                      (`/Engine/EditorBlueprintResources/StandardMacros.IsValid` _newtarg
                        (:`Is Valid`
                          (`self.Move Towards Actor` _newtarg))))))))))))))

(fn `ConsiderAction`
  (params (Data :type "/Game/EnemyController/Struct_ActionConsiderData Structure (by ref)"))
  (returns (Valid :type Boolean))
  (bind (_mindistance _maxdistance _uniqueactionreqs) (break `/Game/EnemyController/Struct_ActionConsiderData` Data))
  (bind _currenttarget (`self.CurrentTarget`))
  (bind _returnvalue (`KismetMathLibrary.Vector_Distance` (`self.K2_GetActorLocation` (`self.GameCharacter`)) (`self.K2_GetActorLocation` _currenttarget)))
  (`/Engine/EditorBlueprintResources/StandardMacros.IsValid` _currenttarget
    (:`Is Valid`
      (for _array_element _uniqueactionreqs
        (bind _valid (`self.ConsiderActionRequirement` _array_element))
        (if (not _valid)
          (return false)))
      (return (and (< _returnvalue _maxdistance) (> _returnvalue _mindistance))))))

(fn `ConsiderActionRequirement`
  (params (Req :type Name))
  (returns (Valid :type Boolean))
  (return true))

(fn `ConsiderNewtarget`
  (returns (NewTarg :type "/Game/Characters/CharacterBlueprints/BP_2DGameCharacter Object Reference"))
  (locals (TargetsToRemove :type "Array of /Game/Characters/CharacterBlueprints/BP_2DGameCharacter Object Reference") (NearestValidTarget :type "/Game/Characters/CharacterBlueprints/BP_2DGameCharacter Object Reference") (NearestDist :type "Float (double-precision)" :default 9999.0))
  (bind _availabletargets (`self.AvailableTargets`))
  (bind _returnvalue (`KismetMathLibrary.Vector_Distance` (`self.K2_GetActorLocation` (`local.NearestValidTarget`)) (`self.K2_GetActorLocation` (`self.GameCharacter`))))
  (for _array_element _availabletargets
    (`/Engine/EditorBlueprintResources/StandardMacros.IsValid` _array_element
      (:`Is Valid`
        (if (< _returnvalue (`local.NearestDist`))
          (set `local.NearestValidTarget` _array_element)
          (set `local.NearestDist` _returnvalue)))
      (:`Is Not Valid`
        (`KismetArrayLibrary.Array_Add` (`local.TargetsToRemove`) _array_element))))
  (for _array_element_2 (`local.TargetsToRemove`)
    (`KismetArrayLibrary.Array_RemoveItem` _availabletargets _array_element_2))
  (bind _output_get (set `self.CurrentTarget` (`local.NearestValidTarget`)))
  (return _output_get))

(fn `ConsiderNewTargetOnTakeHit`
  (params (Attacker :type "/Game/Characters/CharacterBlueprints/BP_2DGameCharacter Object Reference"))
  (bind _currenttarget (`self.CurrentTarget`))
  (bind _returnvalue (`self.K2_GetActorLocation` (`self.GameCharacter`)))
  (`/Engine/EditorBlueprintResources/StandardMacros.IsValid` Attacker
    (:`Is Valid`
      (`self.EnemyDetected` Attacker)
      (if (!= _currenttarget Attacker)
        (if (< (`KismetMathLibrary.Vector_Distance` _returnvalue (`self.K2_GetActorLocation` Attacker)) (`KismetMathLibrary.Vector_Distance` _returnvalue (`self.K2_GetActorLocation` _currenttarget)))
          (set `self.CurrentTarget` Attacker))))))

(fn `Defeated`
  (set `self.IsDefeated` true))

(fn `EnemyDetected`
  (params (Enemy :type "/Game/Characters/CharacterBlueprints/BP_2DGameCharacter Object Reference"))
  (`|ExecutionSequence`
    (:`then_0`
      (if (not (`self.AiActive`))
        (`self.ActivateAi`)))
    (:`then_1`
      (`KismetArrayLibrary.Array_AddUnique` (`self.AvailableTargets`) Enemy)
      (`/Engine/EditorBlueprintResources/StandardMacros.IsValid` (`self.CurrentTarget`)
        (:`Is Not Valid`
          (`self.SetCharacterAsTarget` Enemy))))))

(fn `HitTaken`
  (params (Damage :type "Float (double-precision)") (DotTick :type Boolean) (Attacker :type "/Game/Characters/CharacterBlueprints/BP_2DGameCharacter Object Reference"))
  (`self.ConsiderNewTargetOnTakeHit` Attacker))

(fn `InitControlledCharacter`
  (bind _asbp_2dgame_character (cast `/Game/Characters/CharacterBlueprints/BP_2DGameCharacter` (`self.K2_GetPawn`)))
  (bind _output_get (set `self.GameCharacter` _asbp_2dgame_character))
  (add `/Game/Characters/CharacterBlueprints/BP_2DGameCharacter.InMovementControl` _output_get (`|CreateDelegate` :!event `CharacterMovementControlChanged`))
  (add `/Game/Characters/CharacterBlueprints/BP_2DGameCharacter.LocalEnemyDetected` _output_get (`|CreateDelegate` :!event `EnemyDetected`))
  (bind _bpc_stattracking (`/Game/Characters/CharacterBlueprints/BP_2DGameCharacter.BPC_StatTracking` _output_get))
  (add `/Game/Blueprints/StatTracking/BPC_StatTracking.OnTakeHit` _bpc_stattracking (`|CreateDelegate` :!event `HitTaken`))
  (add `/Game/Blueprints/StatTracking/BPC_StatTracking.OnDefeatingHit` _bpc_stattracking (`|CreateDelegate` :!event `Defeated`)))

(fn `InitDetectionComponent`
  (bind _gamecharacter (`self.GameCharacter`))
  (`/Engine/EditorBlueprintResources/StandardMacros.IsValid` _gamecharacter
    (:`Is Valid`
      (`/Game/Characters/CharacterBlueprints/BP_2DGameCharacter.SpawnDetectionComponent` _gamecharacter))))

(fn `Move Towards Actor`
  (params (Actor :type "Actor Object Reference"))
  (`self.MoveToActor` Actor 200.0 true true false null)
  (set `self.IsMoving` true))

(fn `SetCharacterAsTarget`
  (params (Character :type "/Game/Characters/CharacterBlueprints/BP_2DGameCharacter Object Reference"))
  (bind _output_get (set `self.CurrentTarget` Character))
  (if (> (`self.GetDistanceTo` _output_get (`self.GameCharacter`)) (`self.PreferredDistanceToTarget`))
    (`self.Move Towards Actor` _output_get)))

(fn `UserConstructionScript`)