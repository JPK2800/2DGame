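; Timed attack telegraph decal that warns of an incoming hit, then damages enemy-team characters and breakables inside its mesh.
; Overlap events track and notify targets, while a flipbook material shifts from an ally or enemy start color toward its trigger color.
; On expiry, it hits only locally controlled characters plus breakables, runs text-encoded on-hit effects, plays hit/miss sound and destroys itself.
; Owner defeat cancels it without destroy FX.
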(event `self.ReceiveBeginPlay`
  (`self.InitDestroyOnOwnerDefeat`)
  (`self.InitDecalTextures`)
  (`KismetSystemLibrary.K2_SetTimer` null "TriggerHit" (`self.TimeToTriggerHit`))
  (add `self.OnDestroyed` (delegate `OnDestroy`))
  (`self.TraceOnCreate`))

(event `OnDestroy` :!signature `self.OnDestroyed`
  (params (DestroyedActor :type "Actor Object Reference"))
  (`self.SpawnFxOnDestroy`)
  (for _array_element (`self.OverlappingEnemyActors`)
    (`/Game/Characters/CharacterBlueprints/BP_2DGameCharacter.Overlapped Telegraph` _array_element self false)))

(event `self.StaticMesh.OnComponentBeginOverlap`
  (params (OverlappedComponent :type "PrimitiveComponent Object Reference") (OtherActor :type "Actor Object Reference") (OtherComp :type "PrimitiveComponent Object Reference") (OtherBodyIndex :type Integer) (bFromSweep :type Boolean) (SweepResult :type "HitResult Structure (by ref)"))
  (bind _teamid_teamid (break `GenericTeamId` (`self.TeamId`)))
  (if (`self.Initialized`)
    (bind _asbp_2dgame_character (cast `/Game/Characters/CharacterBlueprints/BP_2DGameCharacter` OtherActor)
      (:`then`
        (bind _teamid_teamid_2 (break `GenericTeamId` (`/Game/Characters/CharacterBlueprints/BP_2DGameCharacter.TeamId` _asbp_2dgame_character)))
        (if (!= _teamid_teamid_2 _teamid_teamid)
          (`KismetArrayLibrary.Array_AddUnique` (`self.OverlappingEnemyActors`) _asbp_2dgame_character)
          (`/Game/Characters/CharacterBlueprints/BP_2DGameCharacter.Overlapped Telegraph` _asbp_2dgame_character self true)))
      (:`CastFailed`
        (bind _asbp_breakable_3d (cast `/Game/Blueprints/Breakable3D/BP_Breakable3D` OtherActor))
        (`KismetArrayLibrary.Array_Add` (`self.OverlappingBreakableObjects`) _asbp_breakable_3d)
        (`/Game/Blueprints/Breakable3D/BP_Breakable3D.Overlapped Telegraph` _asbp_breakable_3d self true)))))

(event `self.StaticMesh.OnComponentEndOverlap`
  (params (OverlappedComponent :type "PrimitiveComponent Object Reference") (OtherActor :type "Actor Object Reference") (OtherComp :type "PrimitiveComponent Object Reference") (OtherBodyIndex :type Integer))
  (bind _overlappingenemyactors (`self.OverlappingEnemyActors`))
  (bind _asbp_2dgame_character (cast `/Game/Characters/CharacterBlueprints/BP_2DGameCharacter` OtherActor)
    (:`then`
      (if (`KismetArrayLibrary.Array_Contains` _overlappingenemyactors _asbp_2dgame_character)
        (`KismetArrayLibrary.Array_RemoveItem` _overlappingenemyactors _asbp_2dgame_character)
        (`/Game/Characters/CharacterBlueprints/BP_2DGameCharacter.Overlapped Telegraph` _asbp_2dgame_character self false)))
    (:`CastFailed`
      (bind _asbp_breakable_3d (cast `/Game/Blueprints/Breakable3D/BP_Breakable3D` OtherActor))
      (`KismetArrayLibrary.Array_RemoveItem` (`self.OverlappingBreakableObjects`) _asbp_breakable_3d)
      (`/Game/Blueprints/Breakable3D/BP_Breakable3D.Overlapped Telegraph` _asbp_breakable_3d self false))))

(fn `ActivateOnHitEffect`
  (params (TargetActor :type "/Game/Characters/CharacterBlueprints/BP_2DGameCharacter Object Reference") (Effect :type Name))
  (locals (EventText :type String) (ParamsText :type String))
  (bind _returnvalue (`KismetStringLibrary.Conv_NameToString` Effect))
  (bind _ownerchar (`self.OwnerChar`))
  (bind (_lefts _rights _returnvalue_2) (`KismetStringLibrary.Split` _returnvalue "|"))
  (if _returnvalue_2
    (set `local.EventText` _lefts)
    (set `local.ParamsText` _rights)
    (else
      (set `local.EventText` _returnvalue)))
  (switch `string` (`local.EventText`)
    (:`ManaGain`
      (`/Engine/EditorBlueprintResources/StandardMacros.IsValid` _ownerchar
        (:`Is Valid`
          (if (`Pawn.IsLocallyControlled` _ownerchar)
            (`/Game/CharacterComponents/StatTracking/BPC_StatTracking.UpdateMana` (`/Game/Characters/CharacterBlueprints/BP_2DGameCharacter.BPC_StatTracking` _ownerchar) (`KismetMathLibrary.Conv_IntToDouble` (`KismetStringLibrary.Conv_StringToInt` (`local.ParamsText`))))))))))

(fn `ActivateOnHitEffects`
  (params (HitCharacters :type "Array of /Game/Characters/CharacterBlueprints/BP_2DGameCharacter Object Reference"))
  (bind _onhitflipbook (`self.OnHitFlipbook`))
  (bind _ownerchar (`self.OwnerChar`))
  (`|ExecutionSequence`
    (:`then_0`
      (for _array_element (`self.OnHitEffectsPerTarget`)
        (for _array_element_2 HitCharacters
          (`self.ActivateOnHitEffect` _array_element_2 _array_element))))
    (:`then_1`
      (if (`KismetSystemLibrary.IsValidClass` _onhitflipbook)
        (for _array_element_3 HitCharacters
          (`|SpawnActorFromClass` _onhitflipbook (`KismetMathLibrary.MakeTransform` (`self.K2_GetActorLocation` _array_element_3)) "Undefined" "MultiplyWithRoot" _ownerchar _ownerchar))))))

(fn `InitDecalTextures`
  (bind _decaltextures (`self.DecalTextures`))
  (bind _returnvalue (`KismetMaterialLibrary.CreateDynamicMaterialInstance` "/Game/AttackDecals/Mat_FlipbookDecal.Mat_FlipbookDecal"))
  (bind _output_get (set `self.DynamicMaterial` _returnvalue))
  (`DecalComponent.SetDecalMaterial` (`self.Decal`) _output_get)
  (`|ExecutionSequence`
    (:`then_0`
      ;[1 0.2622 0.6378] Init Params
      (for (_array_element _array_index) _decaltextures
        (switch `int` _array_index
          (:`0`
            (`MaterialInstanceDynamic.SetTextureParameterValue` _output_get "Tex1" _array_element))
          (:`1`
            (`MaterialInstanceDynamic.SetTextureParameterValue` _output_get "Tex2" _array_element))
          (:`2`
            (`MaterialInstanceDynamic.SetTextureParameterValue` _output_get "Tex3" _array_element))
          (:`3`
            (`MaterialInstanceDynamic.SetTextureParameterValue` _output_get "Tex4" _array_element))))
      (`MaterialInstanceDynamic.SetScalarParameterValue` _output_get "TexCount" (`KismetMathLibrary.Conv_IntToDouble` (`KismetArrayLibrary.Array_Length` _decaltextures))))
    (:`then_1`
      (`self.InitTelegraphColors`))))

(fn `InitDestroyOnOwnerDefeat`
  (bind _ownerchar (`self.OwnerChar`))
  (`/Engine/EditorBlueprintResources/StandardMacros.IsValid` _ownerchar
    (:`Is Valid`
      (add `/Game/CharacterComponents/StatTracking/BPC_StatTracking.OnDefeatingHit` (`/Game/Characters/CharacterBlueprints/BP_2DGameCharacter.BPC_StatTracking` _ownerchar) (`|CreateDelegate` :!event `OnOwnerDefeat`)))))

(fn `InitTelegraphColors`
  (bind _teamid_teamid (break `GenericTeamId` (`self.TeamId`)))
  (bind _dynamicmaterial (`self.DynamicMaterial`))
  (bind _asbp_2dgame_character (cast `/Game/Characters/CharacterBlueprints/BP_2DGameCharacter` (`GameplayStatics.GetPlayerCharacter` 0)))
  (bind _teamid_teamid_2 (break `GenericTeamId` (`/Game/Characters/CharacterBlueprints/BP_2DGameCharacter.TeamId` _asbp_2dgame_character)))
  (if (!= _teamid_teamid_2 _teamid_teamid)
    (set `self.IsEnemyDamage` true)
    (`MaterialInstanceDynamic.SetVectorParameterValue` _dynamicmaterial "ColorParameter" (`self.EnemyDamageColorStart`))
    (set `self.CurrentColorStart` (`self.EnemyDamageColorStart`))
    (set `self.CurrentColorTrigger` (`self.EnemyDamageColorTrigger`))
    (else
      (set `self.IsAllyDamage` true)
      (`MaterialInstanceDynamic.SetVectorParameterValue` _dynamicmaterial "ColorParameter" (`self.AllyDamageColorStart`))
      (set `self.CurrentColorStart` (`self.AllyDamageColorStart`))
      (set `self.CurrentColorTrigger` (`self.AllyDamageColorTrigger`))))
  (`KismetSystemLibrary.K2_SetTimer` null "UpdateColor" (`self.ColorShiftTickRate`) true))

(fn `OnOwnerDefeat`
  (set `self.ManuallyDestroyed` true)
  (`self.K2_DestroyActor`))

(fn `PlaySoundOnStrike`
  (params (HitSuccessful :type Boolean))
  (bind _returnvalue (`self.K2_GetActorLocation`))
  (if HitSuccessful
    (`GameplayStatics.PlaySoundAtLocation` (`self.HitTargetSound`) _returnvalue (struct) 1.0 1.0 0.0 null null null null)
    (else
      (`GameplayStatics.PlaySoundAtLocation` (`self.MissTargetSound`) _returnvalue (struct) 1.0 1.0 0.0 null null null null))))

(fn `SpawnFxOnDestroy`
  (bind (_returnvalue_location _returnvalue_rotation) (`KismetMathLibrary.BreakTransform` (`self.GetTransform`)))
  (bind _fpfxactor (`self.FpFxActor`))
  (if (not (`self.ManuallyDestroyed`))
    (if (`KismetSystemLibrary.IsValidClass` _fpfxactor)
      (`|SpawnActorFromClass` _fpfxactor (`KismetMathLibrary.MakeTransform` _returnvalue_location _returnvalue_rotation) "Undefined" "MultiplyWithRoot" self null))))

(fn `TraceOnCreate`
  (bind _teamid_teamid (break `GenericTeamId` (`self.TeamId`)))
  (`|ExecutionSequence`
    (:`then_0`
      (for _array_element (`PrimitiveComponent.GetOverlappingActors` (`self.StaticMesh`) null)
        (bind _asbp_2dgame_character (cast `/Game/Characters/CharacterBlueprints/BP_2DGameCharacter` _array_element)
          (:`then`
            (bind _teamid_teamid_2 (break `GenericTeamId` (`/Game/Characters/CharacterBlueprints/BP_2DGameCharacter.TeamId` _asbp_2dgame_character)))
            (if (!= _teamid_teamid_2 _teamid_teamid)
              (`KismetArrayLibrary.Array_AddUnique` (`self.OverlappingEnemyActors`) _asbp_2dgame_character)
              (`/Game/Characters/CharacterBlueprints/BP_2DGameCharacter.Overlapped Telegraph` _asbp_2dgame_character self true)))
          (:`CastFailed`
            (bind _asbp_breakable_3d (cast `/Game/Blueprints/Breakable3D/BP_Breakable3D` _array_element))
            (`KismetArrayLibrary.Array_AddUnique` (`self.OverlappingBreakableObjects`) _asbp_breakable_3d)
            (`/Game/Blueprints/Breakable3D/BP_Breakable3D.Overlapped Telegraph` _asbp_breakable_3d self true)))))
    (:`then_1`
      (set `self.Initialized` true))))

(fn `TriggerHit`
  (locals (MadeContact :type Boolean) (HitActors :type "Array of /Game/Characters/CharacterBlueprints/BP_2DGameCharacter Object Reference"))
  (`|ExecutionSequence`
    (:`then_0`
      (for _array_element (`self.OverlappingEnemyActors`)
        (if (`Pawn.IsLocallyControlled` _array_element)
          (bind _asbp_2dgame_character (cast `/Game/Characters/CharacterBlueprints/BP_2DGameCharacter` (`self.GetOwner`)))
          (bind _madehit (`/Game/CharacterComponents/StatTracking/BPC_StatTracking.TakeContact` (`/Game/Characters/CharacterBlueprints/BP_2DGameCharacter.BPC_StatTracking` _array_element) (`self.DamageData`) _asbp_2dgame_character null))
          (if _madehit
            (set `local.MadeContact` true)
            (`KismetArrayLibrary.Array_AddUnique` (`local.HitActors`) _array_element))
          (elif (not (`/Game/CharacterComponents/StatTracking/BPC_StatTracking.DodgeInvulnerable` (`/Game/Characters/CharacterBlueprints/BP_2DGameCharacter.BPC_StatTracking` _array_element)))
            (set `local.MadeContact` true)))))
    (:`then_1`
      (for _array_element_2 (`self.OverlappingBreakableObjects`)
        (bind _asbp_2dgame_character_2 (cast `/Game/Characters/CharacterBlueprints/BP_2DGameCharacter` (`self.GetOwner`)))
        (bind _madehit_2 (`/Game/CharacterComponents/StatTracking/BPC_StatTracking.TakeContact` (`/Game/Blueprints/Breakable3D/BP_Breakable3D.BPC_StatTracking` _array_element_2) (`self.DamageData`) _asbp_2dgame_character_2 null))
        (if _madehit_2
          (set `local.MadeContact` true))))
    (:`then_2`
      (`self.ActivateOnHitEffects` (`local.HitActors`)))
    (:`then_3`
      (`self.PlaySoundOnStrike` (`local.MadeContact`))
      (`self.K2_DestroyActor`))))

(fn `UpdateColor`
  (bind _dynamicmaterial (`self.DynamicMaterial`))
  (bind _output_get (set `self.ProgressTIme` (+ (`self.ProgressTIme`) (`self.ColorShiftTickRate`))))
  (bind _returnvalue (`KismetMathLibrary.MultiplyMultiply_FloatFloat` (/ _output_get (`self.TimeToTriggerHit`)) 0.5))
  (set `self.PercentComplete` _returnvalue)
  (`/Engine/EditorBlueprintResources/StandardMacros.IsValid` _dynamicmaterial
    (:`Is Valid`
      (`MaterialInstanceDynamic.SetVectorParameterValue` _dynamicmaterial "ColorParameter" (`KismetMathLibrary.LinearColorLerp` (`self.CurrentColorStart`) (`self.CurrentColorTrigger`) _returnvalue)))))

(fn `UserConstructionScript`)