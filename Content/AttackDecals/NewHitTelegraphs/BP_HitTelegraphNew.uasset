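; Ground hit telegraph actor that shows an incoming hit, colored as enemy or ally damage by comparing its team to the player's.
; BeginPlay snaps it to static floor with a short downward trace.
; InitDecalTextures creates dynamic materials for ring, fill and inner ring, then sets team colors.
; A looping UpdateColor timer shifts fill color, raises fill and inner-ring opacity, and grows the inner ring toward the outer by elapsed fraction of TimeToTriggerHit.
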(event `self.ReceiveBeginPlay`
  (`self.SnapToFloor`)
  (`parent.ReceiveBeginPlay`))

(fn `InitDecalTextures`
  (bind _hittelegraphring (`self.HitTelegraphRing`))
  (bind _hittelegraphfill (`self.HitTelegraphFill`))
  (bind _hittelegraphinnerring (`self.HitTelegraphInnerRing`))
  (`|ExecutionSequence`
    (:`then_0`
      (bind _returnvalue (`PrimitiveComponent.CreateDynamicMaterialInstance` _hittelegraphring 0 (`PrimitiveComponent.GetMaterial` _hittelegraphring 0) "None"))
      (bind _output_get (set `self.StaticRingMat` _returnvalue))
      (`PrimitiveComponent.SetMaterial` _hittelegraphring 0 _output_get))
    (:`then_1`
      (bind _returnvalue_2 (`PrimitiveComponent.CreateDynamicMaterialInstance` _hittelegraphfill 0 (`PrimitiveComponent.GetMaterial` _hittelegraphfill 0) "None"))
      (bind _output_get_2 (set `self.FillMat` _returnvalue_2))
      (`PrimitiveComponent.SetMaterial` _hittelegraphfill 0 _output_get_2))
    (:`then_2`
      (bind _returnvalue_3 (`PrimitiveComponent.CreateDynamicMaterialInstance` _hittelegraphinnerring 0 (`PrimitiveComponent.GetMaterial` _hittelegraphinnerring 0) "None"))
      (bind _output_get_3 (set `self.InnerRingMat` _returnvalue_3))
      (`PrimitiveComponent.SetMaterial` _hittelegraphinnerring 0 _output_get_3))
    (:`then_3`
      (`self.InitTelegraphColors`))))

(fn `InitTelegraphColors`
  (bind _teamid_teamid (break `GenericTeamId` (`self.TeamId`)))
  (bind (_currentcolorstart_r _currentcolorstart_g _currentcolorstart_b) (break `LinearColor` (`self.CurrentColorStart`)))
  (bind _fillmat (`self.FillMat`))
  (bind _percentcomplete (`self.PercentComplete`))
  (bind (_currentcolortrigger_r _currentcolortrigger_g _currentcolortrigger_b) (break `LinearColor` (`self.CurrentColorTrigger`)))
  (bind _innerringmat (`self.InnerRingMat`))
  (bind _asbp_2dgame_character (cast `/Game/Characters/CharacterBlueprints/BP_2DGameCharacter` (`GameplayStatics.GetPlayerCharacter` 0)))
  (bind _teamid_teamid_2 (break `GenericTeamId` (`/Game/Characters/CharacterBlueprints/BP_2DGameCharacter.TeamId` _asbp_2dgame_character)))
  (if (!= _teamid_teamid_2 _teamid_teamid)
    (set `self.IsEnemyDamage` true)
    (set `self.CurrentColorStart` (`self.EnemyDamageColorStart`))
    (set `self.CurrentColorTrigger` (`self.EnemyDamageColorTrigger`))
    (else
      (set `self.IsAllyDamage` true)
      (set `self.CurrentColorStart` (`self.AllyDamageColorStart`))
      (set `self.CurrentColorTrigger` (`self.AllyDamageColorTrigger`))))
  (`MaterialInstanceDynamic.SetVectorParameterValue` (`self.StaticRingMat`) "Color" (make `LinearColor` _currentcolortrigger_r _currentcolortrigger_g _currentcolortrigger_b 1.0))
  (`MaterialInstanceDynamic.SetVectorParameterValue` _fillmat "Color" (make `LinearColor` _currentcolorstart_r _currentcolorstart_g _currentcolorstart_b 1.0))
  (`MaterialInstanceDynamic.SetVectorParameterValue` _innerringmat "Color" (make `LinearColor` _currentcolortrigger_r _currentcolortrigger_g _currentcolortrigger_b 1.0))
  (`MaterialInstanceDynamic.SetScalarParameterValue` _fillmat "Opacity" _percentcomplete)
  (`MaterialInstanceDynamic.SetScalarParameterValue` _innerringmat "Opacity" _percentcomplete)
  (`SceneComponent.SetRelativeScale3D` (`self.HitTelegraphInnerRing`) (0.0 0.0 0.0))
  (`self.UpdateColor`)
  (`KismetSystemLibrary.K2_SetTimer` null "UpdateColor" (`self.ColorShiftTickRate`) true))

(fn `SnapToFloor`
  (bind _returnvalue (`self.K2_GetActorLocation`))
  (bind _outhit (`KismetSystemLibrary.LineTraceSingleForObjects` _returnvalue (- _returnvalue (0.0 0.0 100.0)) (`|MakeArray` "ObjectTypeQuery1" :!type "EObjectTypeQuery Enum")))
  (bind (_bblockinghit _binitialoverlap _time _distance _location _impactpoint _normal _impactnormal _physmat _hitactor) (`GameplayStatics.BreakHitResult` _outhit))
  (`/Engine/EditorBlueprintResources/StandardMacros.IsValid` _hitactor
    (:`Is Valid`
      (`self.K2_SetActorLocation` (- _impactpoint (0.0 0.0 -1.0)) false true))))

(fn `UpdateColor`
  (bind _percentcomplete (`self.PercentComplete`))
  (bind _output_get (set `self.ProgressTIme` (+ (`self.ProgressTIme`) (`self.ColorShiftTickRate`))))
  (bind _output_get_2 (set `self.PercentComplete` (/ _output_get (`self.TimeToTriggerHit`))))
  (`|ExecutionSequence`
    (:`then_0`
      (bind (_returnvalue_r _returnvalue_g _returnvalue_b) (break `LinearColor` (`KismetMathLibrary.LinearColorLerp` (`self.CurrentColorStart`) (`self.CurrentColorTrigger`) _output_get_2)))
      (`MaterialInstanceDynamic.SetVectorParameterValue` (`self.FillMat`) "Color" (make `LinearColor` _returnvalue_r _returnvalue_g _returnvalue_b 1.0)))
    (:`then_1`
      (`MaterialInstanceDynamic.SetScalarParameterValue` (`self.FillMat`) "Opacity" _percentcomplete)
      (`MaterialInstanceDynamic.SetScalarParameterValue` (`self.InnerRingMat`) "Opacity" _percentcomplete))
    (:`then_2`
      (`SceneComponent.SetRelativeScale3D` (`self.HitTelegraphInnerRing`) (* (`SceneComponent.RelativeScale3D` (`self.HitTelegraphRing`)) (`self.PercentComplete`))))))

(fn `UserConstructionScript`
  (`parent.UserConstructionScript`))