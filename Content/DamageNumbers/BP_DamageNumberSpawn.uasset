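; BP_DamageNumberSpawn is a short-lived actor that displays a floating combat number for damage, healing, dodges or crits.
; InitWidget copies the value, hit-type and relevance flags, plus a color, into its WBP_DamageNumberWidget, then initializes it.
; Each tick eases the widget component toward a target relative offset and rotates it to face player 0's camera.
; The actor expires after TotalDuration through its lifespan, set on BeginPlay.
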(event `self.ReceiveBeginPlay`
  (`self.SetLifeSpan` (`self.TotalDuration`)))

(event `self.ReceiveTick`
  (params (DeltaSeconds :type "Float (single-precision)"))
  (`self.InterpRelativeWidgetPositionStep` DeltaSeconds)
  (`self.FacePlayerControllerStep`))

(fn `FacePlayerControllerStep`
  (bind _widget (`self.Widget`))
  (`SceneComponent.K2_SetWorldRotation` _widget (`KismetMathLibrary.FindLookAtRotation` (`SceneComponent.K2_GetComponentLocation` _widget) (`self.K2_GetActorLocation` (`GameplayStatics.GetPlayerCameraManager` 0))) false false))

(fn `InitWidget`
  (params (IsDodge :type Boolean) (IsCrit :type Boolean) (IsEnemyDamage :type Boolean) (IsAllyDamage :type Boolean) (IsHealing :type Boolean) (Value :type "Float (double-precision)") (IsLocalRelevant :type Boolean))
  (bind _aswbp_damage_number_widget (cast `/Game/DamageNumbers/WBP_DamageNumberWidget` (`WidgetComponent.GetWidget` (`self.Widget`))))
  (set `/Game/DamageNumbers/WBP_DamageNumberWidget.IsDodge` IsDodge _aswbp_damage_number_widget)
  (set `/Game/DamageNumbers/WBP_DamageNumberWidget.IsCrit` IsCrit _aswbp_damage_number_widget)
  (set `/Game/DamageNumbers/WBP_DamageNumberWidget.IsEnemyDamage` IsEnemyDamage _aswbp_damage_number_widget)
  (set `/Game/DamageNumbers/WBP_DamageNumberWidget.IsAllyDamage` IsAllyDamage _aswbp_damage_number_widget)
  (set `/Game/DamageNumbers/WBP_DamageNumberWidget.IsHealing` IsHealing _aswbp_damage_number_widget)
  (set `/Game/DamageNumbers/WBP_DamageNumberWidget.DamageNumber` Value _aswbp_damage_number_widget)
  (set `/Game/DamageNumbers/WBP_DamageNumberWidget.IsLocalRelevant` IsLocalRelevant _aswbp_damage_number_widget)
  (set `/Game/DamageNumbers/WBP_DamageNumberWidget.UseCustomColor` (`self.DmgNumColor`) _aswbp_damage_number_widget)
  (`/Game/DamageNumbers/WBP_DamageNumberWidget.InitWidget` _aswbp_damage_number_widget))

(fn `InterpRelativeWidgetPositionStep`
  (params (DeltaTime :type "Float (double-precision)"))
  (bind _widget (`self.Widget`))
  (`SceneComponent.K2_SetRelativeLocation` _widget (`KismetMathLibrary.VInterpTo` (`SceneComponent.RelativeLocation` _widget) (`self.TargetRelativeTransform`) DeltaTime 2.0) false false))

(fn `UserConstructionScript`)