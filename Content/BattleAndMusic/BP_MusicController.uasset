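; Music controller on BP_BattleManager that switches between battle and calm 2D music as the local player enters and leaves combat.
; On BeginPlay it binds to the manager's combat events, filtered to player controllers, and calls EndBattleMusic.
; An InBattleMusic flag prevents retriggering the same state.
; Tracks are never stopped explicitly; both play under a shared SoundConcurrency setting, owned by the player character.
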(event `self.ReceiveBeginPlay`
  (bind _asbp_battle_manager (cast `/Game/BattleAndMusic/BP_BattleManager` (`self.GetOwner`)))
  (add `/Game/BattleAndMusic/BP_BattleManager.LocalPlayerInCombat` _asbp_battle_manager (delegate `OnPlayerInCombat`))
  (add `/Game/BattleAndMusic/BP_BattleManager.LocalPlayerOutOfCombat` _asbp_battle_manager (delegate `OnPlayerOutOfCombat`))
  (`self.EndBattleMusic`))

(event `OnPlayerInCombat`
  (params (Controller :type "/Game/PlayerController/BP_GamePlayerController Object Reference"))
  (if (`Controller.IsPlayerController` Controller)
    (`self.BeginBattleMusic`)))

(event `OnPlayerOutOfCombat`
  (params (Controller :type "/Game/PlayerController/BP_GamePlayerController Object Reference"))
  (if (`Controller.IsPlayerController` Controller)
    (`self.EndBattleMusic`)))

(fn `BeginBattleMusic`
  (if (not (`self.InBattleMusic`))
    (`GameplayStatics.PlaySound2D` (`self.BattleMusic`) 1.0 1.0 0.0 "/Game/BattleAndMusic/SoundConcurrency.SoundConcurrency" (`GameplayStatics.GetPlayerCharacter` 0))
    (set `self.InBattleMusic` true)))

(fn `EndBattleMusic`
  (if (`self.InBattleMusic`)
    (`GameplayStatics.PlaySound2D` (`self.CalmMusic`) 1.0 1.0 0.0 "/Game/BattleAndMusic/SoundConcurrency.SoundConcurrency" (`GameplayStatics.GetPlayerCharacter` 0))
    (set `self.InBattleMusic` false)))