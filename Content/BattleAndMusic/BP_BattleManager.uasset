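; Battle manager that tracks which enemy characters and player controllers are in combat and broadcasts combat state changes.
; An enemy landing at index 0 of the enemy list fires BeginCombat; emptying the list fires EndCombat and calls removal on the tracked players.
; Adding or removing a player fires LocalPlayerInCombat or LocalPlayerOutOfCombat only for locally controlled controllers.
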(fn `AddEnemyToBattle`
  (params (Character :type "/Game/Characters/CharacterBlueprints/BP_2DGameCharacter Object Reference"))
  (bind _returnvalue (`KismetArrayLibrary.Array_AddUnique` (`self.EnemyCharacters`) Character))
  (if (== _returnvalue 0)
    (`self.BeginCombat`)
    (set `self.EnemyInCombat` true)))

(fn `AddPlayerToBattle`
  (params (PlayerController :type "/Game/PlayerController/BP_GamePlayerController Object Reference"))
  (`/Engine/EditorBlueprintResources/StandardMacros.IsValid` PlayerController
    (:`Is Valid`
      (`KismetArrayLibrary.Array_AddUnique` (`self.PlayerControllers`) PlayerController)
      (if (`Controller.IsLocalController` PlayerController)
        (`self.LocalPlayerInCombat` PlayerController)))))

(fn `RemoveEnemyFromBattle`
  (params (Character :type "/Game/Characters/CharacterBlueprints/BP_2DGameCharacter Object Reference"))
  (bind _enemycharacters (`self.EnemyCharacters`))
  (`KismetArrayLibrary.Array_RemoveItem` _enemycharacters Character)
  (if (`KismetArrayLibrary.Array_IsEmpty` _enemycharacters)
    (`self.EndCombat`)
    (set `self.EnemyInCombat` false)
    (for _array_element (`self.PlayerControllers`)
      (`self.RemovePlayerFromBattle` _array_element))))

(fn `RemovePlayerFromBattle`
  (params (Controller :type "/Game/PlayerController/BP_GamePlayerController Object Reference"))
  (bind _playercontrollers (`self.PlayerControllers`))
  (if (`KismetArrayLibrary.Array_Contains` _playercontrollers Controller)
    (`KismetArrayLibrary.Array_RemoveItem` _playercontrollers Controller)
    (if (`Controller.IsLocalController` Controller)
      (`self.LocalPlayerOutOfCombat` Controller))))

(fn `UserConstructionScript`)